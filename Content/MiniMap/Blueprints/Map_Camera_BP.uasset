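; Minimap capture actor that, on BeginPlay in non-distribution builds when Active, exports an orthographic PNG of each map tile.
; The construction script computes tile centers from grid size and tile width, drawing numbered preview boxes.
; A delayed loop moves the SceneCapture to each tile, nudging it to refresh the per-resolution render target before saving.
; It can repeat tiles down to a minimum resolution, with optional per-resolution paths and gated 8K output.
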(event EventBeginPlay
  (bind _scenecapturecomponent2d (Variables|Default|GetSceneCaptureComponent2D))
  (bind _current_tile (Variables|Default|GetCurrent%20Tile))
  (bind _current_tile_2 (Variables|Default|GetCurrent%20Tile))
  (bind _scenecapturecomponent2d_2 (Variables|Default|GetSceneCaptureComponent2D))
  (bind _current_tile_3 (Variables|Default|GetCurrent%20Tile))
  (bind _grid_locations (Variables|Default|GetGrid%20Locations))
  (bind _current_tile_4 (Variables|Default|GetCurrent%20Tile))
  (bind _returnvalue (Utilities|String|ToString(Integer) _current_tile_2))
  (bind _output (Utilities|Array|Get(acopy) _grid_locations _current_tile))
  (bind _returnvalue_2 (Utilities|String|Append "000" _returnvalue))
  ;[1 1 1] Upon starting play, save a picture of each tile from the camera
  (if (not (Class|KismetSystemLibrary|IsPackagedforDistribution))
    (if (Variables|Default|GetActive) :!label _label
      (if (> (Variables|Default|GetCurrent%20Tile) (Utilities|Array|LastIndex (Variables|Default|GetGrid%20Locations)))
        (Development|PrintString "All Tiles Saved" true true "(R=1.000000,G=0.000000,B=0.023671,A=1.000000)" 3e+01)
        (else
          (if (Variables|SavedFiles|GetUse%20Seperate%20File%20Paths%20For%20Each%20Resolution)
            (if (Utilities|Enum|Equal(Enum) (Utilities|Array|Get(acopy) (Variables|SavedFiles|GetFile%20Paths-Resolution%20Specific) (Math|Conversions|ToInteger(Byte) (Variables|Resolution|GetCurrent%20Resolution))) "")
              _
              (else
                (if (Utilities|Enum|Equal(Enum) (Variables|Resolution|GetCurrent%20Resolution) "NewEnumerator0") :!label _label_2
                  (if (Variables|Resolution|Get8K%20Allowed)
                    ;;[1 1 1] Update Scene Capture Settings
                    (bind _output_get (Variables|/Script/Engine.SceneCaptureComponent2D|SetTextureTarget _scenecapturecomponent2d_2 (Utilities|Select :Index (Variables|Resolution|GetCurrent%20Resolution) :NewEnumerator0 "/Game/MiniMap/Textures/Renter_Target_Textures/Export_Map_8192_T.Export_Map_8192_T" :NewEnumerator1 "/Game/MiniMap/Textures/Renter_Target_Textures/Export_Map_4096_T.Export_Map_4096_T" :NewEnumerator2 "/Game/MiniMap/Textures/Renter_Target_Textures/Export_Map_2048_T.Export_Map_2048_T" :NewEnumerator3 "/Game/MiniMap/Textures/Renter_Target_Textures/Export_Map_1024_T.Export_Map_1024_T" :NewEnumerator4 "/Game/MiniMap/Textures/Renter_Target_Textures/Export_Map_512_T.Export_Map_512_T" :NewEnumerator5 "/Game/MiniMap/Textures/Renter_Target_Textures/Export_Map_256_T.Export_Map_256_T" :NewEnumerator6 "/Game/MiniMap/Textures/Renter_Target_Textures/Export_Map_128_T.Export_Map_128_T" :NewEnumerator7 "/Game/MiniMap/Textures/Renter_Target_Textures/Export_Map_64_T.Export_Map_64_T" :NewEnumerator9 "/Game/MiniMap/Textures/Renter_Target_Textures/Export_Map_32_T.Export_Map_32_T") :!label _label_3))
                    (Variables|Default|SetCurrent%20Render%20Target _output_get)
                    (Variables|/Script/Engine.TextureRenderTarget|SetTargetGamma (Variables|/Script/Engine.SceneCaptureComponent2D|GetTextureTarget _scenecapturecomponent2d_2) (Variables|Default|GetRender%20Target%20Gamma))
                    ;;[1 1 1] Force movement of camera to update rendertarget, and then move to actual location
                    (Transformation|SetRelativeLocation _scenecapturecomponent2d (Math|Vector|MakeVector 0.0 0.0 1.0) false false)
                    (Transformation|SetRelativeLocation _scenecapturecomponent2d (Math|Vector|MakeVector (.x _output) (.y _output) 0.0) false false)
                    ;;[1 1 1] Wait short delay for updates
                    (Utilities|FlowControl|Delay (* (Variables|Default|GetDelay%20Time) 0.35))
                    ;;[1 1 1] Save image file
                    (Rendering|ExportRenderTarget (Variables|Default|GetCurrent%20Render%20Target) (select (Variables|SavedFiles|GetUse%20Seperate%20File%20Paths%20For%20Each%20Resolution) (Utilities|Array|Get(acopy) (Variables|SavedFiles|GetFile%20Paths-Resolution%20Specific) (Math|Conversions|ToInteger(Byte) (Variables|Resolution|GetCurrent%20Resolution))) (Variables|SavedFiles|GetSave%20Images%20File%20Path)) (Utilities|String|ToString(Text) (Utilities|Text|FormatText "{T}{A}_{B}{D}{Y}.png" (select (Variables|SavedFiles|GetAdd%20"T_"%20to%20start%20of%20file%20names) "T_" "") (Utilities|Text|ToText(String) (Variables|SavedFiles|GetFile%20Name)) (Utilities|Text|ToText(String) (Utilities|String|RightChop _returnvalue_2 (- (Utilities|String|Len _returnvalue_2) 4))) (select (Variables|SavedFiles|GetInclude%20Resolution%20In%20Name) (Utilities|Text|FormatText "_{A}" (Utilities|Select :Index (Variables|Resolution|GetCurrent%20Resolution) :NewEnumerator0 "8192" :NewEnumerator1 "4096" :NewEnumerator2 "2048" :NewEnumerator3 "1024" :NewEnumerator4 "512" :NewEnumerator5 "256" :NewEnumerator6 "128" :NewEnumerator7 "64" :NewEnumerator9 "32")) "") (select (Variables|SavedFiles|GetAdd%20"_T"%20to%20end%20of%20file%20names) "_T" ""))))
                    ;;[1 1 1] Wait a bit after saving before continuing
                    (Utilities|FlowControl|Delay (* (Variables|Default|GetDelay%20Time) 0.65))
                    ;;[1 1 1] Continue onto next tile, or same tile with lower resolution
                    (if (Variables|Resolution|GetRender%20From%20Resolution%20Down%20To%20Minimum%20Resolution) :!label _label_4
                      (if (== (Variables|Resolution|GetCurrent%20Resolution) (Variables|Resolution|GetMinimum%20Resolution))
                        (Variables|Resolution|SetCurrent%20Resolution (Variables|Resolution|GetResolution))
                        (Development|PrintString (Utilities|String|ToString(Text) (Utilities|Text|FormatText "{A} Finished" _current_tile_3)) true true "(R=0.000000,G=0.660000,B=1.000000,A=1.000000)" 1e+01 :!label _label_5)
                        (Math|Integer|IncrementInt _current_tile_3
                          (:%20%20
                            (goto _label)))
                        (else
                          (Development|PrintString (Utilities|String|ToString(Text) (Utilities|Text|FormatText "{A} {B} Saved" _current_tile_4 (Utilities|Select :Index (Variables|Resolution|GetCurrent%20Resolution) :NewEnumerator0 "8192" :NewEnumerator1 "4096" :NewEnumerator2 "2048" :NewEnumerator3 "1024" :NewEnumerator4 "512" :NewEnumerator5 "256" :NewEnumerator6 "128" :NewEnumerator7 "64" :NewEnumerator9 "32"))) true true "(R=0.000000,G=0.153453,B=1.000000,A=1.000000)" 1e+01)))
                      (else
                        (goto _label_5)))
                    (elif (Variables|Resolution|GetRender%20From%20Resolution%20Down%20To%20Minimum%20Resolution)
                      (Development|PrintString (Utilities|String|ToString(Text) (Utilities|Text|FormatText "{A} {B} Skipped" _current_tile_4 (Utilities|Select :Index (Variables|Resolution|GetCurrent%20Resolution) :NewEnumerator0 "8192" :NewEnumerator1 "4096" :NewEnumerator2 "2048" :NewEnumerator3 "1024" :NewEnumerator4 "512" :NewEnumerator5 "256" :NewEnumerator6 "128" :NewEnumerator7 "64" :NewEnumerator9 "32"))) true true "(R=0.000000,G=0.153453,B=1.000000,A=1.000000)" 1e+01)
                      (else
                        (goto _label_4))))
                  (else
                    (goto _label_3)))
                (Variables|Resolution|SetCurrent%20Resolution (Utilities|Enum|ByteToEnumMap_Resolutions_Enum (+ (Variables|Resolution|GetCurrent%20Resolution) 1)))
                (goto _label)))
            (elif (Utilities|Enum|Equal(Enum) (Variables|SavedFiles|GetSave%20Images%20File%20Path) "")
              _
              (else
                (goto _label_2))))
          (Development|PrintString "No save file path found. Please set file paths" true true "(R=1.000000,G=0.000000,B=0.023671,A=1.000000)" 3e+01)))
      (else
        (Development|PrintString "Map_Camera_BP in level is not Active." true true "(R=1.000000,G=0.774232,B=0.000000,A=1.000000)" 1e+01)))))

(fn ConstructionScript
  (bind _resolution (Variables|Resolution|GetResolution))
  (bind _tile_width__meters_ (Variables|Default|GetTile%20Width%20%28Meters%29))
  (bind _tile_width__meters__2 (Variables|Default|GetTile%20Width%20%28Meters%29))
  (bind _tile_width__meters__3 (Variables|Default|GetTile%20Width%20%28Meters%29))
  (bind _grid (Variables|Default|GetGrid))
  (bind _grid_2 (Variables|Default|GetGrid))
  (bind _grid_3 (Variables|Default|GetGrid))
  (bind _tile_width__meters__4 (Variables|Default|GetTile%20Width%20%28Meters%29))
  (bind _returnvalue (Math|Float|Round (.y _grid_3)))
  (bind _returnvalue_2 (* _tile_width__meters__4 5e+01))
  (bind _returnvalue_3 (* _tile_width__meters_ 0.5))
  ;[1 1 1] Set initial box size and cameras ortho width
  (Variables|Resolution|SetCurrent%20Resolution _resolution)
  (if (== _resolution 0)
    ;[1 1 1] Give warning for 8k textures
    (Development|PrintString "Warning 8K textures are very epxpensive on graphical memory to render, and can take awhile to save." true true "(R=1.000000,G=0.000000,B=0.030547,A=1.000000)" 1e+01))
  (bind _output_get (Variables|/Script/Engine.SceneCaptureComponent2D|SetOrthoWidth (Variables|Default|GetSceneCaptureComponent2D) (* (Variables|Default|GetTile%20Width%20%28Meters%29) 1e+02)))
  (Class|CameraComponent|SetOrthoWidth (Variables|Default|GetCamera) _output_get)
  (Components|Box|SetBoxExtent (Variables|Default|GetBox) (Math|Vector|MakeVector (* (.x _grid_2) _tile_width__meters__3 5e+01) (* (.y _grid_2) _tile_width__meters__3 5e+01) (* _tile_width__meters__3 2e+01)) true)
  ;[1 1 1] Create a value for each location on the grid, using the current tiles grid location, the values will be adjusted so they are placed in the proper order next to eachother.
  (Utilities|Array|Clear (Variables|Default|GetGrid%20Locations))
  (for _index (range 1 (Math|Float|Round (.x _grid_3)))
    (for _index_2 (range 1 _returnvalue)
      ;[1 1 1] Take the initial grid position, and add the half size of the tiles so the position saved would be the tiles center point. Save the final central translation of the tiles location, and the scale it would be used at.
      (Utilities|Array|SetArrayElem (Variables|Default|GetGrid%20Locations) (+ (* (- _index 1) _returnvalue) (- _index_2 1)) (Math|Vector2D|MakeVector2D (* (- (- (- (* (.x (Variables|Default|GetGrid)) (Variables|Default|GetTile%20Width%20%28Meters%29) 1.0) (* _tile_width__meters_ (Math|Conversions|ToFloat(Integer) (- _index 1)))) (* (.x _grid) _tile_width__meters__2 0.5)) _returnvalue_3) 1e+02) (* (+ _returnvalue_3 (- (* _tile_width__meters_ (Math|Conversions|ToFloat(Integer) (- _index_2 1))) (* (.y _grid) _tile_width__meters__2 0.5))) 1e+02)) true)))
  ;[1 1 1] Create grid boxes and numbers for each tile location
  (for (_array_element _array_index) (Variables|Default|GetGrid%20Locations)
    (bind _returnvalue_4 (AddComponent|AddTextRenderComponent false (Math|Transform|MakeTransform (Math|Vector|MakeVector (.x _array_element) (.y _array_element) 0.0) "0,180.000000, 0" "1.000000,1.000000,1.000000")))
    (Rendering|Components|TextRender|SetText _returnvalue_4 (Utilities|Text|ToText(Integer) _array_index))
    (Rendering|Components|TextRender|SetWorldSize _returnvalue_4 (* (Variables|Default|GetTile%20Width%20%28Meters%29) 1e+01))
    (bind _returnvalue_5 (AddComponent|AddBoxComponent false (Math|Transform|MakeTransform (Math|Vector|MakeVector (.x _array_element) (.y _array_element) 0.0) "0, 0, 0" "1.000000,1.000000,1.000000")))
    (Components|Box|SetBoxExtent _returnvalue_5 (Math|Vector|MakeVector _returnvalue_2 _returnvalue_2 (* _tile_width__meters__4 2e+01)) false)
    (Collision|SetCollisionEnabled _returnvalue_5 "NoCollision")))