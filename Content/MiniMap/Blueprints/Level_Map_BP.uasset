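; Level map actor for the minimap system that marks a map's area in the level and holds its map image parts grouped by zoom.
; The construction script sizes the box from the map's dimensions in meters and sets the billboard sprite.
; An optional flag makes it turn off mipmap generation on every texture in the zoom-level image arrays.
; It has no active gameplay logic.
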(event EventBeginPlay)

(event Collision|EventActorBeginOverlap
  (params (OtherActor :type Actor%20Object%20Reference)))

(event EventTick
  (params (DeltaSeconds :type Float%20%28single-precision%29)))

(fn ConstructionScript
  (bind _map_dimension__in_meters_ (Variables|Default|GetMap%20Dimension%20%28In%20Meters%29))
  (bind _returnvalue (* (.x _map_dimension__in_meters_) 5e+01))
  (bind _returnvalue_2 (* (.y _map_dimension__in_meters_) 5e+01))
  ;[1 1 1] Size the box to match the maps dimensions, and set the billboard sprite.
  (Components|Box|SetBoxExtent (Variables|Default|GetBox) (Math|Vector|MakeVector _returnvalue _returnvalue_2 (* (+ _returnvalue _returnvalue_2) 0.1)) true)
  (Rendering|Components|Sprite|SetSprite (Variables|Default|GetBillboard) (Variables|Default|GetBilboard%20Image))
  ;[1 1 1] Set current textures to no mip maps if enabled
  (if (Variables|Default|GetDisable%20MipMaps%20On%20Added%20Textures)
    (for _array_element (Variables|Default|GetMap%20Parts%20By%20Zoom)
      (for _array_element_2 (.mapimagesarray _array_element)
        (bind _as텍스처 (Utilities|Casting|CastToTexture _array_element_2))
        (Variables|/Script/Engine.Texture|SetMipGenSettings _as텍스처 "TMGS_NoMipmaps")))))