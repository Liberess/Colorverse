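; BP_NPC is a non-player character that shows a name marker when the player comes near.
; On BeginPlay it hides its MarkerWidget and passes NPCName to the widget's user object as the displayed text.
; A TriggerZone overlap with BP_ColorverseCharacter reveals the marker and triggers its animation update, and end overlap hides it again.
; Calls reach the widget through message functions, without casting to a specific widget class.
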(event OnComponentEndOverlap(TriggerZone)
  (params (OverlappedComponent :type Primitive%20Component%20Object%20Reference) (OtherActor :type Actor%20Object%20Reference) (OtherComp :type Primitive%20Component%20Object%20Reference) (OtherBodyIndex :type Integer))
  (Utilities|Casting|CastToBP_ColorverseCharacter OtherActor)
  (Development|SetHiddeninGame (Variables|Default|GetMarkerWidget) true false))

(event OnComponentBeginOverlap(TriggerZone)
  (params (OverlappedComponent :type Primitive%20Component%20Object%20Reference) (OtherActor :type Actor%20Object%20Reference) (OtherComp :type Primitive%20Component%20Object%20Reference) (OtherBodyIndex :type Integer) (bFromSweep :type Boolean) (SweepResult :type Hit%20Result%20Structure%20%28by%20ref%29))
  (bind _markerwidget (Variables|Default|GetMarkerWidget))
  (Utilities|Casting|CastToBP_ColorverseCharacter OtherActor)
  (Development|SetHiddeninGame _markerwidget false false)
  (Class|BPIMarker|UpdateMarkerAnim(Message) (UserInterface|GetUserWidgetObject _markerwidget)))

(event EventBeginPlay
  (bind _markerwidget (Variables|Default|GetMarkerWidget))
  (Development|SetHiddeninGame _markerwidget true false)
  (Class|BPIMarker|UpdateNameText(Message) (UserInterface|GetUserWidgetObject _markerwidget) (Utilities|Text|ToText(Name) (Variables|Default|GetNPCName))))

(fn ConstructionScript)