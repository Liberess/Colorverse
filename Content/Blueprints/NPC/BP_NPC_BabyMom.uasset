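; BP_NPC_BabyMom is a talkable NPC in Colorverse that turns to face the player during conversation.
; Its trigger zone shows an animated name marker while the player is inside and ends the talk on exit.
; Beginning a talk plays a sound, hides the marker and interact UI, then calls the parent logic once the turn finishes.
; One LookAt timeline handles both turns, using IsTalking to target the player or the original rotation.
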(event OnComponentEndOverlap(TriggerZone)
  (params (OverlappedComponent :type Primitive%20Component%20Object%20Reference) (OtherActor :type Actor%20Object%20Reference) (OtherComp :type Primitive%20Component%20Object%20Reference) (OtherBodyIndex :type Integer))
  (Utilities|Casting|CastToBP_ColorverseCharacter OtherActor)
  (Development|SetHiddeninGame (Variables|Default|GetMarkerWidget) true false)
  (Class|IDialogue|OnEndTalk))

(event OnComponentBeginOverlap(TriggerZone)
  (params (OverlappedComponent :type Primitive%20Component%20Object%20Reference) (OtherActor :type Actor%20Object%20Reference) (OtherComp :type Primitive%20Component%20Object%20Reference) (OtherBodyIndex :type Integer) (bFromSweep :type Boolean) (SweepResult :type Hit%20Result%20Structure%20%28by%20ref%29))
  (bind _markerwidget (Variables|Default|GetMarkerWidget))
  (bind _returnvalue (UserInterface|GetUserWidgetObject _markerwidget))
  (Utilities|Casting|CastToBP_ColorverseCharacter OtherActor)
  (Development|SetHiddeninGame _markerwidget false false)
  (Class|BPIMarker|UpdateMarkerAnim(Message) _returnvalue)
  (Class|BPIMarker|UpdateNameText(Message) _returnvalue (.DisplayName (Utilities|Struct|BreakDialogue (Variables|Default|GetDialogueData)))))

(event EventBeginPlay
  (Development|SetHiddeninGame (Variables|Default|GetMarkerWidget) true false)
  (Variables|Default|SetOriginRotation (Transformation|GetActorRotation))
  (Variables|Default|SetOriginLocation (Transformation|GetActorLocation))
  (bind _returnvalue (UserInterface|CreateWidget "/Game/UI/BP_Dialogue.BP_Dialogue_C"))
  (Variables|Default|SetDialogueWidget _returnvalue)
  (bind _returnvalue_2 (UserInterface|CreateWidget "/Game/UI/BP_InteractWidget.BP_InteractWidget_C"))
  (Variables|Default|SetInteractWidget _returnvalue_2))

(event EventOnEndTalk
  ;[1 1 1] On End Talk Event
  (Variables|Default|SetbIsTalking false)
  (|CallParentFunction)
  ;[1 1 1] Camera Swap Animation
  (bind _time (Timeline|LookAt PlayFromStart)
    (:Update
      (Transformation|SetActorRotation (Math|Rotator|MakeRotator 0.0 0.0 (.yaw (Math|Interpolation|RInterpTo (Transformation|GetActorRotation) (Math|Rotator|SelectRotator (Math|Rotator|FindLookatRotation (Transformation|GetActorLocation) (Transformation|GetActorLocation (Game|GetPlayerCharacter 0))) (Variables|Default|GetOriginRotation) (Variables|Default|GetbIsTalking)) _time 1.0)))))
    (:Finished
      (if (Variables|Default|GetbIsTalking)
        (|CallParentFunction)))))

(event EventOnBeginTalk
  ;[1 1 1] On Begin Talk Event
  (if (Variables|Default|GetbIsTalking)
    (|CallParentFunction)
    (else
      (Variables|Default|SetbIsTalking true)
      (Audio|SpawnSoundatLocation "/Game/Sounds/Charater/Talking_NPC.Talking_NPC" (Transformation|GetActorLocation) "0, 0, 0" 1.0 1.0 0.0 0 0)
      (Class|NPC|SetActiveInteractUI false)
      (Development|SetHiddeninGame (Variables|Default|GetMarkerWidget) true false)
      ;[1 1 1] Camera Swap Animation
      (bind _time (Timeline|LookAt PlayFromStart)
        (:Update
          (Transformation|SetActorRotation (Math|Rotator|MakeRotator 0.0 0.0 (.yaw (Math|Interpolation|RInterpTo (Transformation|GetActorRotation) (Math|Rotator|SelectRotator (Math|Rotator|FindLookatRotation (Transformation|GetActorLocation) (Transformation|GetActorLocation (Game|GetPlayerCharacter 0))) (Variables|Default|GetOriginRotation) (Variables|Default|GetbIsTalking)) _time 1.0)))))
        (:Finished
          (if (Variables|Default|GetbIsTalking)
            (|CallParentFunction)))))))

(fn ConstructionScript)