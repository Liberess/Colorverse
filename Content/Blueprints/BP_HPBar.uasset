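; BP_HPBar is an actor that displays a monster's health bar in the world through a widget component.
; On BeginPlay it caches the progress bar from its BP_MonsterHP widget, and UpdateHPBar fills it with the ratio of its two inputs.
; SetHpBarLocation moves the actor to a given position and turns it toward the player pawn using only X and Y, keeping the bar upright.
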(event Custom|UpdateHPBar
  (params (NewParam :type Float%20%28double-precision%29) (NewParam2 :type Float%20%28double-precision%29))
  (Progress|SetPercent (Variables|Default|GetProgress%20Bar) (/ NewParam NewParam2)))

(event EventBeginPlay
  (bind _asbp_monster_hp (Utilities|Casting|CastToBP_MonsterHP (UserInterface|GetUserWidgetObject (Variables|Default|GetWidget))))
  (Variables|Default|SetProgress%20Bar (Variables|/Game/UI/BP_MonsterHP.BP_MonsterHP_C|GetProgressBar _asbp_monster_hp)))

(fn ConstructionScript)

(fn SetHpBarLocation
  (params (NewParam :type Vector))
  (bind _returnvalue (Game|Player|GetPlayerPawn 0))
  (bind _returnvalue_2 (Transformation|GetActorLocation _returnvalue))
  (Transformation|SetActorLocation (Math|Vector|MakeVector (.x NewParam) (.y NewParam) (.z NewParam)) false false)
  (Transformation|SetActorRotation (Math|Rotator|FindLookatRotation (Math|Vector|MakeVector (.x NewParam) (.y NewParam) 0.0) (Math|Vector|MakeVector (.x _returnvalue_2) (.y _returnvalue_2) 0.0))))