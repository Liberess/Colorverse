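; Player character Blueprint that handles a Roll input by choosing a roll speed from the character's current movement.
; The Roll event runs only when the character is not falling and passes through a DoOnce gate.
; It sets RollSpeed higher when velocity exceeds a threshold, prints it, then immediately resets the gate.
; No roll animation or movement is applied in this graph.
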(event EventRoll
  (bind _charactermovement (Variables|Character|GetCharacterMovement))
  (if (not (AI|Components|NavMovement|IsFalling _charactermovement))
    (Utilities|FlowControl|DoOnce false :!label _label
      (:Completed
        (if (> (Math|Vector|VectorLength (Variables|/Script/Engine.MovementComponent|GetVelocity _charactermovement)) 3e+02)
          (Variables|Default|SetRollSpeed 1.5)
          (else
            (Variables|Default|SetRollSpeed 1.0)))
        (Development|PrintString (Utilities|String|Append "Roll : " (Utilities|String|ToString(Float) (Variables|Default|GetRollSpeed))))
        (goto _label Reset)))))

(event Input|ActionEvents|InputActionRoll
  (params (Key :type Key%20Structure :default "None"))
  (:Pressed
    (Class|PlayerCharacter|Roll)))

(fn ConstructionScript)