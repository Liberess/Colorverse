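; BP_TestWoodStick is an interactable wood stick pickup that goes into the player's inventory.
; On BeginPlay it marks itself separated and loads its ItemData from the WoodStick row of DT_ItemData.
; Interact, when separated, adds that data through the InventoryManager and destroys the actor.
; Unconnected nodes for painting and brush dynamic materials and a delayed physics shutoff never run.
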(event EventInteract
  (bind _returnvalue (Subsystems|GetInventoryManager))
  (if (Variables|Default|GetbIsSeparated)
    (Utilities|IsValid _returnvalue
      (:Is%20Valid
        (Class|InventoryManager|AddInventoryItem _returnvalue (Variables|Default|GetItemData))
        (Actor|DestroyActor)))))

(event EventBeginPlay
  (|CallParentFunction)
  (Utilities|FlowControl|Sequence
    (:then_0
      (Variables|Default|SetbIsSeparated true))
    (:then_1
      (bind _returnvalue (Utilities|GetDataTableRow "/Game/DataTables/DT_ItemData.DT_ItemData" "WoodStick")
        (:then
          (Variables|Default|SetItemData _returnvalue))))))

(fn ConstructionScript)