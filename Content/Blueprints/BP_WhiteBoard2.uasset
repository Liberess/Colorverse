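; Whiteboard actor that players or tools can draw on at runtime by painting into a render target.
; BeginPlay creates dynamic board and brush materials, plus render targets modeled on a template, and feeds the cleared pallet target into the board material.
; DrawOnWhiteBoard sets brush location and board pen color, then draws the brush material into the pallet; Alpha is unused.
; The copy target's canvas compositing is unconnected, and its OnRep is empty.
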(event Custom|DrawOnWhiteBoard
  (params (LocationToDraw :type Vector%202D%20Structure) (Alpha :type Boolean) (Color :type Linear%20Color%20Structure))
  (bind _brushmatinst (Variables|세팅|GetBrushMatInst))
  ;[1 1 1] Draw on WhiteBoard
  (Rendering|Material|SetVectorParameterValue _brushmatinst "DrawLocation" (Math|Conversions|ToLinearColor(Vector) (Math|Conversions|ToVector(Vector2D) LocationToDraw 0.1)) :!class /Script/Engine.MaterialInstanceDynamic)
  (Rendering|Material|SetVectorParameterValue (Variables|세팅|GetPaintingMatInst) "PenColor" Color :!class /Script/Engine.MaterialInstanceDynamic)
  (Rendering|DrawMaterialtoRenderTarget (Variables|세팅|GetPaintingRenderTargetPallet) _brushmatinst))

(event EventBeginPlay
  (Utilities|FlowControl|Sequence
    (:then_0
      ;[1 1 1] Instantiate Dynamic Material (PaintingMat, BrushMat)
      (bind _returnvalue (Rendering|Material|CreateDynamicMaterialInstance "/Game/Painter/WhiteBoardMat.WhiteBoardMat" "PaintingMatInst" "None" :!class /Script/Engine.KismetMaterialLibrary))
      (bind _output_get (Variables|세팅|SetPaintingMatInst _returnvalue))
      (Rendering|Material|SetMaterial (Variables|Default|GetStaticMesh) 0 _output_get)
      (bind _returnvalue_2 (Rendering|Material|CreateDynamicMaterialInstance "/Game/Painter/WhiteBoardMarkerMat.WhiteBoardMarkerMat" "BrushMatInst" "None" :!class /Script/Engine.KismetMaterialLibrary))
      (Variables|세팅|SetBrushMatInst _returnvalue_2))
    (:then_1
      ;[1 1 1] Instantiate Painting Render Target Pallet
      (bind _returnvalue_3 (CallFunction|CreateRenderTarget))
      (Variables|세팅|SetPaintingRenderTargetPallet _returnvalue_3)
      (Rendering|Material|SetTextureParameterValue (Variables|세팅|GetPaintingMatInst) "RenderTarget" (Variables|세팅|GetPaintingRenderTargetPallet))
      (Rendering|ClearRenderTarget2D (Variables|세팅|GetPaintingRenderTargetPallet) (Variables|/Script/Engine.TextureRenderTarget2D|GetClearColor (Variables|세팅|GetPaintingRenderTargetPallet))))
    (:then_2
      ;[1 1 1] Instantiate Painting Render Target Copy
      (bind _returnvalue_4 (CallFunction|CreateRenderTarget))
      (Variables|세팅|SetPaintingRenderTargetCopy _returnvalue_4))))

(event EventTick
  (params (DeltaSeconds :type Float%20%28single-precision%29)))

(fn ConstructionScript)

(fn OnRepPaintingRenderTargetCopy)

(fn CreateRenderTarget
  (bind _paintingrendertarget (Variables|Settings|GetPaintingRenderTarget))
  (bind _returnvalue (Rendering|CreateRenderTarget2D (Variables|/Script/Engine.TextureRenderTarget2D|GetSizeX _paintingrendertarget) (Variables|/Script/Engine.TextureRenderTarget2D|GetSizeY _paintingrendertarget) (Variables|/Script/Engine.TextureRenderTarget2D|GetRenderTargetFormat _paintingrendertarget) (Variables|/Script/Engine.TextureRenderTarget2D|GetClearColor _paintingrendertarget) (Variables|/Script/Engine.TextureRenderTarget2D|GetbAutoGenerateMips _paintingrendertarget)))
  (return _returnvalue))