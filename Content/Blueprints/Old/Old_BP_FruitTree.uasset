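; Paintable fruit tree actor whose colour state sets its textures, leaf tint and the colour of its collectible objects.
; Draw events render a brush material into a copy render target, which Tick composites into the palette target read by the painting and brush materials.
; While colour is active, a looping timer, with its interval randomised once at BeginPlay, spawns a capped number of physics-simulated wood collectibles nearby.
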(event Custom|SpawnWoodStick
  (bind _returnvalue (Transformation|GetActorLocation))
  (if (and (Variables|Default|GetIsColorActive) (<= (Utilities|Array|Length (Variables|Default|GetSpawnedCollectObj)) 5))
    (bind _returnvalue_2 (Game|SpawnActorfromClass "/Game/Blueprints/BP_CollectObject.BP_CollectObject_C" (Math|Conversions|ToTransform(Vector) (Math|Vector|MakeVector (+ (.x _returnvalue) (Math|Random|RandomFloatinRange 5e+01 2e+02)) (+ (.y _returnvalue) (Math|Random|RandomFloatinRange 5e+01 2e+02)) (.z _returnvalue))) "AdjustIfPossibleButDontSpawnIfColliding" 0 0))
    (Utilities|IsValid _returnvalue_2
      (:Is%20Valid
        (Utilities|FlowControl|Sequence
          (:then_0
            (Class|CollectObject|SetCollectObjectData _returnvalue_2 (Variables|Default|GetSeparatedItemName))
            (Variables|/Script/Colorverse.CollectObject|SetbIsSeparated _returnvalue_2 true)
            (Variables|/Script/Colorverse.InteractObject|SetIsInteractable _returnvalue_2 true)
            (bind _returnvalue_3 (Utilities|Array|Add (Variables|Default|GetSpawnedCollectObj) _returnvalue_2)))
          (:then_1
            (Components|StaticMesh|SetStaticMesh (Variables|/Script/Colorverse.CollectObject|GetStaticMesh _returnvalue_2) "/Game/Stylized_VFX_StPack/Meshes/SM_Wood.SM_Wood")
            (Rendering|Material|SetMaterial (Variables|/Script/Colorverse.CollectObject|GetStaticMesh _returnvalue_2) 0 "/Game/StarterContent/Materials/M_Wood_Oak.M_Wood_Oak")
            (Physics|SetSimulatePhysics (Variables|/Script/Colorverse.CollectObject|GetStaticMesh _returnvalue_2) true))
          (:then_2
            (Game|AssignOnDestroyed _returnvalue_2 (delegate Custom|OnDestroyed_이벤트))))))))

(event Custom|EndDrawOnWhiteBoard
  ;[1 1 1] End Draw On WhiteBoard Event
  (Variables|Default|SetIsDrawing false))

(event Custom|OnDestroyed_이벤트
  (params (DestroyedActor :type Actor%20Object%20Reference))
  (Utilities|Array|RemoveIndex (Variables|Default|GetSpawnedCollectObj) (stale Custom|SpawnWoodStick _returnvalue_3)))

(event EventBeginPlay
  (|CallParentFunction)
  (Utilities|FlowControl|Sequence
    (:then_0
      ;[1 1 1] Instantiate Dynamic Material (PaintingMat, BrushMat)
      (bind _returnvalue (Rendering|Material|CreateDynamicMaterialInstance (Variables|Default|GetPaintingMatTemplate) "PaintingMatInst" "None" :!class /Script/Engine.KismetMaterialLibrary))
      (bind _output_get (Variables|Default|SetPaintingMatInst _returnvalue))
      (Rendering|Material|SetMaterial (Variables|Default|GetStaticMesh) 0 _output_get)
      (bind _returnvalue_2 (Rendering|Material|CreateDynamicMaterialInstance (Variables|Default|GetBrushMatTemplate) "BrushMatInst" "None" :!class /Script/Engine.KismetMaterialLibrary))
      (Variables|Default|SetBrushMatInst _returnvalue_2)
      (bind _returnvalue_3 (Rendering|Material|CreateDynamicMaterialInstance "/Game/Meshes/M_Tree/MI_Leaves.MI_Leaves" "LeaveMatInst" "None" :!class /Script/Engine.KismetMaterialLibrary))
      (bind _output_get_2 (Variables|Default|SetGroupMatInst _returnvalue_3))
      (Rendering|Material|SetMaterial (Variables|Default|GetLeaves01) 0 _output_get_2))
    (:then_1
      (Utilities|FlowControl|Delay 0.1)
      ;[1 1 1] Set BaseTexture
      (if (Variables|Default|GetIsColorActive)
        (Rendering|Material|SetTextureParameterValue (Variables|Default|GetPaintingMatInst) "BaseTexture" (Variables|Default|GetActiveTexture))
        (Class|PaintedCollectObject|SetChildCollectObjectTexture (Variables|Default|GetChildActiveTexture))
        (Rendering|Material|SetVectorParameterValue (Variables|Default|GetGroupMatInst) "OverlayColor" (Variables|Default|GetGroupActiveColor) :!class /Script/Engine.MaterialInstanceDynamic)
        (for _array_element (Variables|Default|GetCollectObjects)
          (Class|CollectObject|SetPaintedColor _array_element (.ResultColor (Utilities|Struct|BreakPaintCombo (Variables|Default|GetPaintComboData))))
          (Variables|/Script/Colorverse.InteractObject|SetIsInteractable _array_element true))
        (else
          (Rendering|Material|SetTextureParameterValue (Variables|Default|GetPaintingMatInst) "BaseTexture" (Variables|Default|GetInActiveTexture))
          (Class|PaintedCollectObject|SetChildCollectObjectTexture (Variables|Default|GetChildInActiveTexture))
          (Rendering|Material|SetVectorParameterValue (Variables|Default|GetGroupMatInst) "OverlayColor" (Variables|Default|GetGroupInActiveColor) :!class /Script/Engine.MaterialInstanceDynamic)
          (for _array_element_2 (Variables|Default|GetCollectObjects)
            (Class|CollectObject|SetPaintedColor _array_element_2 "(R=0.500000,G=0.500000,B=0.500000,A=1.000000)")
            (Variables|Default|SetIsInteractable false)))))
    (:then_2
      ;[1 1 1] Instantiate Painting Render Target Pallet
      (bind _returnvalue_4 (CallFunction|CreateRenderTarget))
      (Variables|Default|SetPaintingRenderTargetPallet _returnvalue_4)
      (Rendering|Material|SetTextureParameterValue (Variables|Default|GetPaintingMatInst) "RenderTarget" (Variables|Default|GetPaintingRenderTargetPallet))
      (Rendering|Material|SetTextureParameterValue (Variables|Default|GetBrushMatInst) "RenderTarget" (Variables|Default|GetPaintingRenderTargetPallet))
      (Rendering|ClearRenderTarget2D (Variables|Default|GetPaintingRenderTargetPallet) (Variables|/Script/Engine.TextureRenderTarget2D|GetClearColor (Variables|Default|GetPaintingRenderTargetPallet))))
    (:then_3
      ;[1 1 1] Instantiate Painting Render Target Copy
      (bind _returnvalue_5 (CallFunction|CreateRenderTarget))
      (Variables|Default|SetPaintingRenderTargetCopy _returnvalue_5))
    (:then_4
      (Utilities|Time|SetTimerbyEvent (delegate Custom|SpawnWoodStick) (Math|Random|RandomFloatinRange 5.0 2e+01) true))))

(event EventTick
  (params (DeltaSeconds :type Float%20%28single-precision%29))
  (bind _brushmatinst (Variables|Default|GetBrushMatInst))
  (if (Variables|Default|GetIsDrawing)
    _
    (else
      ;[1 1 1] Tick : Copy the temporary texture to the main one
      (Rendering|Material|SetScalarParameterValue _brushmatinst "DeltaTime" (Utilities|Time|GetWorldDeltaSeconds) :!class /Script/Engine.MaterialInstanceDynamic)
      (Rendering|Material|SetVectorParameterValue _brushmatinst "BrushPositionUV" "(R=0.000000,G=0.000000,B=0.000000,A=1.000000)" :!class /Script/Engine.MaterialInstanceDynamic)
      (bind (_canvas _size _context) (Rendering|BeginDrawCanvastoRenderTarget (Variables|Default|GetPaintingRenderTargetCopy)))
      (Canvas|DrawMaterial :self _canvas :RenderMaterial _brushmatinst :ScreenSize _size :CoordinateSize "(X=1.000000,Y=1.000000)" :PivotPoint "(X=0.500000,Y=0.500000)")
      (Rendering|EndDrawCanvastoRenderTarget _context)))
  (bind (_canvas_2 _size_2 _context_2) (Rendering|BeginDrawCanvastoRenderTarget (Variables|Default|GetPaintingRenderTargetPallet)))
  (Canvas|DrawTexture :self _canvas_2 :RenderTexture (Variables|Default|GetPaintingRenderTargetCopy) :ScreenSize _size_2 :CoordinateSize "(X=1.000000,Y=1.000000)" :RenderColor "(R=0.000000,G=0.000000,B=0.000000,A=0.000000)" :BlendMode "BLEND_Additive" :PivotPoint "(X=0.500000,Y=0.500000)")
  (Rendering|EndDrawCanvastoRenderTarget _context_2))

(event EventDrawonWhiteBoard
  (params (LocationToDraw :type Vector%202D%20Structure) (Alpha :type Boolean) (BrushColor :type Linear%20Color%20Structure))
  (bind _brushmatinst (Variables|Default|GetBrushMatInst))
  ;[1 1 1] Draw on WhiteBoard
  (Variables|Default|SetIsDrawing true)
  (Rendering|Material|SetVectorParameterValue _brushmatinst "BrushPositionUV" (Utilities|Struct|MakeLinearColor (.x LocationToDraw) (.y LocationToDraw) (select Alpha 1.0 0.0) 1.0) :!class /Script/Engine.MaterialInstanceDynamic)
  (Rendering|Material|SetVectorParameterValue _brushmatinst "BrushColor" BrushColor :!class /Script/Engine.MaterialInstanceDynamic)
  (bind (_canvas _size _context) (Rendering|BeginDrawCanvastoRenderTarget (Variables|Default|GetPaintingRenderTargetCopy)))
  (Canvas|DrawMaterial :self _canvas :RenderMaterial (Variables|Default|GetBrushMatInst) :ScreenSize _size :CoordinateSize "(X=1.000000,Y=1.000000)" :PivotPoint "(X=0.500000,Y=0.500000)")
  (Rendering|EndDrawCanvastoRenderTarget _context))

(fn ConstructionScript)

(fn CreateRenderTarget
  (bind _paintingrendertargettemplate (Variables|Default|GetPaintingRenderTargetTemplate))
  (bind _returnvalue (Rendering|CreateRenderTarget2D (Variables|/Script/Engine.TextureRenderTarget2D|GetSizeX _paintingrendertargettemplate) (Variables|/Script/Engine.TextureRenderTarget2D|GetSizeY _paintingrendertargettemplate) (Variables|/Script/Engine.TextureRenderTarget2D|GetRenderTargetFormat _paintingrendertargettemplate) (Variables|/Script/Engine.TextureRenderTarget2D|GetClearColor _paintingrendertargettemplate) (Variables|/Script/Engine.TextureRenderTarget2D|GetbAutoGenerateMips _paintingrendertargettemplate)))
  (return _returnvalue))