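; Whiteboard actor that players or other callers paint on at runtime through draw and end-draw events, using render targets.
; BeginPlay creates brush and painting material instances plus two render targets matching a template target's settings.
; The brush material reads the pallet target and draws into the copy at LocationToDraw, which Tick copies back each frame.
; While idle, Tick also redraws the brush with a zeroed position and frame delta time.
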(event Custom|DrawOnWhiteBoard
  (params (LocationToDraw :type Vector%202D%20Structure) (Alpha :type Boolean) (Color :type Linear%20Color%20Structure))
  (bind _brushmatinst (Variables|세팅|GetBrushMatInst))
  ;[1 1 1] Draw on WhiteBoard
  (Variables|Default|SetIsDrawing true)
  (Rendering|Material|SetVectorParameterValue _brushmatinst "BrushPositionUV" (Utilities|Struct|MakeLinearColor (.x LocationToDraw) (.y LocationToDraw) (select Alpha 1.0 0.0) 1.0) :!class /Script/Engine.MaterialInstanceDynamic)
  (Rendering|Material|SetVectorParameterValue _brushmatinst "BrushColor" Color :!class /Script/Engine.MaterialInstanceDynamic)
  (bind (_canvas _size _context) (Rendering|BeginDrawCanvastoRenderTarget (Variables|세팅|GetPaintingRenderTargetCopy)))
  (Canvas|DrawMaterial :self _canvas :RenderMaterial (Variables|세팅|GetBrushMatInst) :ScreenSize _size :CoordinateSize "(X=1.000000,Y=1.000000)" :PivotPoint "(X=0.500000,Y=0.500000)")
  (Rendering|EndDrawCanvastoRenderTarget _context))

(event Custom|EndDrawOnWhiteBoard
  ;[1 1 1] End Draw On WhiteBoard Event
  (Variables|Default|SetIsDrawing false))

(event EventBeginPlay
  (Utilities|FlowControl|Sequence
    (:then_0
      ;[1 1 1] Instantiate Dynamic Material (PaintingMat, BrushMat)
      (bind _returnvalue (Rendering|Material|CreateDynamicMaterialInstance "/Game/Painter/M_RenderTarget_Painting.M_RenderTarget_Painting" "PaintingMatInst" "None" :!class /Script/Engine.KismetMaterialLibrary))
      (bind _output_get (Variables|세팅|SetPaintingMatInst _returnvalue))
      (Rendering|Material|SetMaterial (Variables|Default|GetStaticMesh) 0 _output_get)
      (bind _returnvalue_2 (Rendering|Material|CreateDynamicMaterialInstance "/Game/Painter/M_RenderTarget_Brush.M_RenderTarget_Brush" "BrushMatInst" "None" :!class /Script/Engine.KismetMaterialLibrary))
      (Variables|세팅|SetBrushMatInst _returnvalue_2))
    (:then_1
      ;[1 1 1] Instantiate Painting Render Target Pallet
      (bind _returnvalue_3 (CallFunction|CreateRenderTarget))
      (Variables|세팅|SetPaintingRenderTargetPallet _returnvalue_3)
      (Rendering|Material|SetTextureParameterValue (Variables|세팅|GetPaintingMatInst) "RenderTarget" (Variables|세팅|GetPaintingRenderTargetPallet))
      (Rendering|Material|SetTextureParameterValue (Variables|세팅|GetBrushMatInst) "RenderTarget" (Variables|세팅|GetPaintingRenderTargetPallet))
      (Rendering|ClearRenderTarget2D (Variables|세팅|GetPaintingRenderTargetPallet) (Variables|/Script/Engine.TextureRenderTarget2D|GetClearColor (Variables|세팅|GetPaintingRenderTargetPallet))))
    (:then_2
      ;[1 1 1] Instantiate Painting Render Target Copy
      (bind _returnvalue_4 (CallFunction|CreateRenderTarget))
      (Variables|세팅|SetPaintingRenderTargetCopy _returnvalue_4))))

(event EventTick
  (params (DeltaSeconds :type Float%20%28single-precision%29))
  (bind _brushmatinst (Variables|세팅|GetBrushMatInst))
  (if (Variables|Default|GetIsDrawing)
    _
    (else
      ;[1 1 1] Copy the temporary texture to the main one
      (Rendering|Material|SetScalarParameterValue _brushmatinst "DeltaTime" (Utilities|Time|GetWorldDeltaSeconds) :!class /Script/Engine.MaterialInstanceDynamic)
      (Rendering|Material|SetVectorParameterValue _brushmatinst "BrushPositionUV" "(R=0.000000,G=0.000000,B=0.000000,A=1.000000)" :!class /Script/Engine.MaterialInstanceDynamic)
      (bind (_canvas _size _context) (Rendering|BeginDrawCanvastoRenderTarget (Variables|세팅|GetPaintingRenderTargetCopy)))
      (Canvas|DrawMaterial :self _canvas :RenderMaterial _brushmatinst :ScreenSize _size :CoordinateSize "(X=1.000000,Y=1.000000)" :PivotPoint "(X=0.500000,Y=0.500000)")
      (Rendering|EndDrawCanvastoRenderTarget _context)))
  (bind (_canvas_2 _size_2 _context_2) (Rendering|BeginDrawCanvastoRenderTarget (Variables|세팅|GetPaintingRenderTargetPallet)))
  (Canvas|DrawTexture :self _canvas_2 :RenderTexture (Variables|세팅|GetPaintingRenderTargetCopy) :ScreenSize _size_2 :CoordinateSize "(X=1.000000,Y=1.000000)" :RenderColor "(R=1.000000,G=1.000000,B=1.000000,A=0.000000)" :BlendMode "BLEND_Opaque" :PivotPoint "(X=0.500000,Y=0.500000)")
  (Rendering|EndDrawCanvastoRenderTarget _context_2))

(fn ConstructionScript)

(fn OnRepPaintingRenderTargetCopy)

(fn CreateRenderTarget
  (bind _paintingrendertarget (Variables|Settings|GetPaintingRenderTarget))
  (bind _returnvalue (Rendering|CreateRenderTarget2D (Variables|/Script/Engine.TextureRenderTarget2D|GetSizeX _paintingrendertarget) (Variables|/Script/Engine.TextureRenderTarget2D|GetSizeY _paintingrendertarget) (Variables|/Script/Engine.TextureRenderTarget2D|GetRenderTargetFormat _paintingrendertarget) (Variables|/Script/Engine.TextureRenderTarget2D|GetClearColor _paintingrendertarget) (Variables|/Script/Engine.TextureRenderTarget2D|GetbAutoGenerateMips _paintingrendertarget)))
  (return _returnvalue))