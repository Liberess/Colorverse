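; Red wolf enemy, using boss wolf animations, that attacks Colorverse characters and feeds color to tag-matched BP_Sanctum actors when destroyed.
; Attacks set AI blackboard attacking and random-cooldown flags; timelines drive a forward lunge or spin, then jump montages to End.
; HitCheck sphere-traces at the head socket, sending damage and skill-specific knockback to characters not already recorded.
; Zero health triggers the death montage and stops the SlimeAIController.
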(event Custom|CoolTime
  (AI|Components|Blackboard|SetValueasBool (AI|GetBlackboard (Pawn|GetController)) (Variables|Default|GetCool%20Time%20Key) true)
  (Utilities|FlowControl|Delay (Math|Random|RandomFloatinRange 3.0 7.0))
  (AI|Components|Blackboard|SetValueasBool (AI|GetBlackboard (Pawn|GetController)) (Variables|Default|GetCool%20Time%20Key) false))

(event Custom|blackborad%20isAttacking%20False
  (AI|Components|Blackboard|SetValueasBool (AI|GetBlackboard (Pawn|GetController)) (Variables|Default|GetIs%20Attacking%20Key) false)
  (Variables|Default|SetImpact "0, 0, 0"))

(event Custom|Destroy
  (bind _outactors (Actor|GetAllActorsOfClass "/Game/Blueprints/BP_Sanctum.BP_Sanctum_C"))
  (bind _array_element (Utilities|Array|ForEachLoopwithBreak _outactors)
    (:LoopBody
      (if (Utilities|Enum|Equal(Enum) (Variables|/Script/Colorverse.Sanctum|GetPuzzleTag _array_element) (Variables|Default|GetPuzzleTag))
        (Class|Sanctum|IncreaseColor _array_element))
      (Actor|DestroyActor))))

(event EventHitCheck
  (bind _mesh (Variables|Character|GetMesh))
  (bind _returnvalue (Transformation|GetSocketLocation _mesh "Head_M"))
  ;[1 1 1] Hit Check
  (bind (_outhits _returnvalue_2) (Collision|MultiSphereTraceForObjects _returnvalue _returnvalue 5e+02 (Variables|Default|GetObject%20Types) false 0 "ForDuration"))
  (if _returnvalue_2
    (for _array_element _outhits
      (if (== (Utilities|Array|FindItem (Variables|Default|GetAttackHitResults) (.HitActor (Collision|BreakHitResult _array_element))) -1)
        (Utilities|Array|AddUnique (Variables|Default|GetAttackHitResults) (.HitActor (Collision|BreakHitResult _array_element)))
        (bind _ascolorverse_character (Utilities|Casting|CastToColorverseCharacter (.HitActor (Collision|BreakHitResult _array_element))))
        (bind _returnvalue_3 (Class|CombatSystem|GetCurrentATK (Variables|Default|GetCombatSystem)))
        (Class|ColorverseCharacter|Attacked _ascolorverse_character (Utilities|Struct|MakeDamageMessage self _returnvalue_3 (.ImpactPoint (Collision|BreakHitResult _array_element)) (.ImpactNormal (Collision|BreakHitResult _array_element)) (Variables|Default|GetImpact)))
        (Niagara|SpawnSystematLocation "/Game/Stylized_VFX_StPack/Particles/UPDATE_1_3/P_Web_Hit_01.P_Web_Hit_01" (+ (Transformation|GetActorLocation) (* (Math|Vector|GetForwardVector (Variables|Default|GetFollowCamera)) 2e+02)) (Transformation|GetActorRotation))))))

(event EventAttacked
  (params (damageMessage :type Damage%20Message%20Structure))
  (Class|LivingEntity|ApplyDamage (Variables|Default|GetLivingEntity) damageMessage)
  (if (<= (Variables|/Script/Colorverse.LivingEntity|GetCurrentHealth (Variables|Default|GetLivingEntity)) 0)
    (Class|ColorverseCharacter|Dead)))

(event EventDead
  (|CallParentFunction)
  (Animation|Montage|MontagePlay (Components|SkeletalMesh|GetAnimInstance (Variables|Character|GetMesh)) "/Game/Mannequin/Wolf_Boss/Animations/Anim_WolfBoss_Death_WolfBoss_Death_Montage.Anim_WolfBoss_Death_WolfBoss_Death_Montage" 1.0 "MontageLength" 0.0 true)
  (bind _asslime_aicontroller (Utilities|Casting|CastToSlimeAIController (Pawn|GetController)))
  (Class|SlimeAIController|StopAI _asslime_aicontroller))

(event EventBeginPlay
  (|CallParentFunction)
  (Utilities|FlowControl|Sequence
    (:then_0
      (bind _ascolorverse_character_anim_instance (Utilities|Casting|CastToColorverseCharacterAnimInstance (Components|SkeletalMesh|GetAnimInstance (Variables|Character|GetMesh))))
      (EventDispatchers|BindEventtoOnEndAttack _ascolorverse_character_anim_instance (delegate Custom|blackborad%20isAttacking%20False)))))

(event EventAttack
  (params (skillNum :type Integer))
  ;[1 1 1] 공격
  (|CallParentFunction skillNum)
  (AI|Components|Blackboard|SetValueasBool (AI|GetBlackboard (Pawn|GetController)) (Variables|Default|GetIs%20Attacking%20Key) true)
  (CallFunction|CoolTime)
  (Utilities|FlowControl|Sequence
    (:then_0
      (if (== skillNum 0)
        (Variables|Default|SetImpact "1500.000000,1500.000000,500.000000")
        (bind _speed (Timeline|타임라인_0 PlayFromStart)
          (:Update
            (Transformation|SetActorLocation (+ (Transformation|GetActorLocation) (* (Transformation|GetActorForwardVector) _speed)) true false))
          (:Finished
            (Ability|Animation|MontageJumptoSection (Components|SkeletalMesh|GetAnimInstance (Variables|Character|GetMesh)) "End" "/Game/Mannequin/Wolf_Boss/Animations/Anim_WolfBoss_Jump_WolfBoss_Jump_Notransform_Montage.Anim_WolfBoss_Jump_WolfBoss_Jump_Notransform_Montage")))))
    (:then_1
      (if (== skillNum 2)
        (Variables|Default|SetImpact "700.000000,700.000000,500.000000")
        (bind _rot (Timeline|타임라인 PlayFromStart)
          (:Update
            (Transformation|AddWorldRotation (Variables|Default|GetCapsuleComponent) (Math|Rotator|MakeRotator 0.0 0.0 _rot) false false))
          (:Finished
            (Ability|Animation|MontageJumptoSection (Components|SkeletalMesh|GetAnimInstance (Variables|Character|GetMesh)) "End" "/Game/Mannequin/Wolf_Boss/Animations/Anim_WolfBoss_skill_1.Anim_WolfBoss_skill_1")))))))

(fn ConstructionScript)