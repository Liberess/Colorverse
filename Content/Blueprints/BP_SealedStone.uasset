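; BP_SealedStone is a sealed stone puzzle object that tracks whether three switches are activated in index order, apparently tied to a boss door.
; BeginPlay creates dynamic materials for three crystals and a main crystal with black emissive color.
; ChangeCrystalColor uses a timeline to fade a chosen crystal's emissive color from black.
; SetCompleteSwitch adds or removes switches, then marks completion or wrong order once three are registered.
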(event Custom|SetCompleteSwitch
  (params (Switch :type BP%20Multiple%20Laser%20Pressure%20Switch%20Object%20Reference) (IsComplete :type Boolean))
  (bind _switchs (Variables|Default|GetSwitchs))
  ;[1 1 1] Set Complete Switch
  (if (not (Variables|Default|GetIsComplete))
    (if IsComplete
      (if (not (Utilities|Array|ContainsItem (Variables|Default|GetSwitchs) Switch))
        (Utilities|Array|Add _switchs Switch)
        (if (>= (Utilities|Array|Length _switchs) 3)
          (bind (_array_element _array_index) (Utilities|Array|ForEachLoopwithBreak (Variables|Default|GetSwitchs) :!label _label)
            (:LoopBody
              (if (== (Variables|/Game/Blueprints/Puzzle/BP_MultipleLaserPressureSwitch.BP_MultipleLaserPressureSwitch_C|GetIndex _array_element) _array_index)
                (Variables|Default|SetIsWrongOrder false)
                (else
                  (Variables|Default|SetIsWrongOrder true)
                  (goto _label Break))))
            (:Completed
              (if (not (Variables|Default|GetIsWrongOrder))
                (Variables|Default|SetIsComplete true)
                (Variables|Default|SetIsWrongOrder false)
                (Development|PrintString "BossDoor::Complete!!!" true true "(R=0.000000,G=0.660000,B=1.000000,A=1.000000)" 4.0)
                (Variables|Default|SetCompleteCount 3))))))
      (else
        (bind _returnvalue (Utilities|Array|RemoveItem (Variables|Default|GetSwitchs) Switch))
        (if _returnvalue
          (Variables|Default|SetIsWrongOrder false))))))

(event Custom|ChangeCrystalColor
  (params (Index :type Integer) (Color :type Linear%20Color%20Structure) (IsMain :type Boolean))
  ;[1 1 1] Change Crystal Color
  (bind _time (Timeline|ChangeColor Play)
    (:Update
      (if IsMain
        (Rendering|Material|SetVectorParameterValue (Variables|Default|GetMainCrystalMI) "EmissiveColor" (Math|Color|Lerp(LinearColor) :B Color :Alpha _time) :!class /Script/Engine.MaterialInstanceDynamic)
        (else
          (Rendering|Material|SetVectorParameterValue (Utilities|Array|Get(acopy) (Variables|Default|GetCrystalMIs) Index) "EmissiveColor" (Math|Color|Lerp(LinearColor) :B Color :Alpha _time) :!class /Script/Engine.MaterialInstanceDynamic))))))

(event EventBeginPlay
  ;[1 1 1] BeginPlay :: Set MI
  (Utilities|Array|Clear (Variables|Default|GetCrystalMIs))
  (for _index (range 0 2)
    (bind _returnvalue (Rendering|Material|CreateDynamicMaterialInstance (Variables|Default|GetStaticMesh) _index (Variables|Default|GetCrystalMat) "None" :!class /Script/Engine.PrimitiveComponent))
    (Utilities|Array|Add (Variables|Default|GetCrystalMIs) _returnvalue)
    (Rendering|Material|SetVectorParameterValue _returnvalue "EmissiveColor" "(R=0.000000,G=0.000000,B=0.000000,A=0.500000)" :!class /Script/Engine.MaterialInstanceDynamic))
  (bind _returnvalue_2 (Rendering|Material|CreateDynamicMaterialInstance (Variables|Default|GetStaticMesh) 4 (Variables|Default|GetCrystalMat) "None" :!class /Script/Engine.PrimitiveComponent))
  (bind _output_get (Variables|Default|SetMainCrystalMI _returnvalue_2))
  (Rendering|Material|SetVectorParameterValue _output_get "EmissiveColor" "(R=0.000000,G=0.000000,B=0.000000,A=0.500000)" :!class /Script/Engine.MaterialInstanceDynamic))

(fn ConstructionScript)