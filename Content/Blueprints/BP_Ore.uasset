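; BP_Ore is an interactable ore pickup that breaks apart and adds its item to the player's inventory.
; Its GeometryCollection has physics simulation off at BeginPlay.
; Interact enables physics with a zero-vector impulse and passes ItemData to the InventoryManager.
; The Invisible timeline then drives the DefaultRoot's world scale and destroys the actor when it finishes.
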(event EventBeginPlay
  (|CallParentFunction)
  (Physics|SetSimulatePhysics (Variables|Default|GetGeometryCollection) false))

(event EventInteract
  (bind _geometrycollection (Variables|Default|GetGeometryCollection))
  ;[1 1 1] Interact Event
  (Physics|SetSimulatePhysics _geometrycollection true)
  (Physics|AddImpulse _geometrycollection "0.000000,0.000000,0.000000" "None" false)
  (Class|InventoryManager|AddInventoryItem (Subsystems|GetInventoryManager) (Variables|Default|GetItemData))
  (bind _scale (Timeline|Invisible PlayFromStart)
    (:Update
      (Transformation|SetWorldScale3D (Variables|Default|GetDefaultRoot) _scale))
    (:Finished
      (Actor|DestroyActor))))

(fn ConstructionScript)