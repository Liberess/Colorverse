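; BP_Slime is a slime character Blueprint that handles melee hit detection against Colorverse characters.
; While CombatSystem allows attack tracing, Tick runs HitCheck, a multi line trace with debug drawing between the first two sockets of the Sword component.
; AttackHitResults filters out already-hit actors, and each new Colorverse character receives Attacked with the current ATK and impact details.
; The parent HitCheck call is left unconnected.
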(event EventTick
  (params (DeltaSeconds :type Float%20%28single-precision%29))
  (if (Variables|/Script/Colorverse.CombatSystem|GetbIsCanAttackTrace (Variables|Default|GetCombatSystem))
    (Class|ColorverseCharacter|HitCheck)))

(event EventHitCheck
  (bind _sword (Variables|Default|Getsword))
  (bind _returnvalue (Transformation|GetAllSocketNames _sword))
  (bind (_outhits _returnvalue_2) (Class|KismetSystemLibrary|LineTraceMultiforObjects (Transformation|GetSocketLocation _sword (Utilities|Array|Get(acopy) _returnvalue)) (Transformation|GetSocketLocation _sword (Utilities|Array|Get(acopy) _returnvalue 1)) (Variables|Default|GetObject%20Types) false 0 "ForDuration" true))
  (if _returnvalue_2
    (for _array_element _outhits
      (if (== (Utilities|Array|FindItem (Variables|Default|GetAttackHitResults) (.HitActor (Collision|BreakHitResult _array_element))) -1)
        (Utilities|Array|AddUnique (Variables|Default|GetAttackHitResults) (.HitActor (Collision|BreakHitResult _array_element)))
        (bind _ascolorverse_character (Utilities|Casting|CastToColorverseCharacter (.HitActor (Collision|BreakHitResult _array_element))))
        (bind _returnvalue_3 (Class|CombatSystem|GetCurrentATK (Variables|Default|GetCombatSystem)))
        (Class|ColorverseCharacter|Attacked _ascolorverse_character (Utilities|Struct|MakeDamageMessage self _returnvalue_3 (.ImpactPoint (Collision|BreakHitResult _array_element)) (.ImpactNormal (Collision|BreakHitResult _array_element))))))))

(fn ConstructionScript)