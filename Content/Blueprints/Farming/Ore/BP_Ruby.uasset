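; BP_Ruby is a harvestable ruby ore node that gives the player an item and respawns after a random delay.
; On interact it hides its mesh, disables collision, plays a pickup sound, adds its item to the inventory and spawns destructible and ore dummy actors in its place.
; A timer then calls Reset, where a timeline scales the node back up before re-enabling collision and interaction.
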(event Custom|Reset
  (Development|SetHiddeninGame (Variables|Default|GetStaticMesh) false false)
  (bind _grown (Timeline|Show PlayFromStart)
    (:Update
      (Transformation|SetRelativeScale3D (Variables|Default|GetDefaultRoot) (Math|Conversions|ToVector(Float) _grown)))
    (:Finished
      (Collision|SetCollisionEnabled (Variables|Default|GetStaticMesh) "QueryAndPhysics")
      (Variables|Default|SetIsInteractable true))))

(event EventOnInteract
  (bind _staticmesh (Variables|Default|GetStaticMesh))
  ;[1 1 1] Interact Event
  (if (Variables|Default|GetIsInteractable)
    (Variables|Default|SetIsInteractable false)
    (Variables|Default|SetRespawnTime (Math|Random|RandomFloatinRange 1e+01 (Variables|Default|GetMaxRespawnTime)))
    (Audio|SpawnSoundatLocation "/Game/Sounds/Charater/Get_ore.Get_ore" (Transformation|GetActorLocation) "0, 0, 0" 1.0 1.0 0.0 0 0)
    (Development|SetHiddeninGame _staticmesh true false)
    (Collision|SetCollisionEnabled _staticmesh "NoCollision")
    (Utilities|FlowControl|Sequence
      (:then_0
        (Game|SpawnActorfromClass "/Game/Blueprints/BP_DestructibleDummy.BP_DestructibleDummy_C" (Transformation|GetActorTransform) "AdjustIfPossibleButAlwaysSpawn" 0 0)
        (Class|InventoryManager|AddInventoryItem (Subsystems|GetInventoryManager) (Variables|Default|GetItemData) true)
        (Utilities|Time|SetTimerbyEvent (delegate Custom|Reset) (Variables|Default|GetRespawnTime)))
      (:then_1
        (bind _returnvalue (Game|SpawnActorfromClass "/Game/Blueprints/Farming/Ore/BP_OreDummy.BP_OreDummy_C" (Transformation|GetActorTransform) "AlwaysSpawn" 0 0))
        (Components|StaticMesh|SetStaticMesh (Variables|/Game/Blueprints/Farming/Ore/BP_OreDummy.BP_OreDummy_C|GetStaticMesh _returnvalue) (Variables|CollectObject|GetOreMesh))
        (Default|HideEvent _returnvalue)))))

(fn ConstructionScript)