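; BP_Tulip is an interactable tulip in the farming content that disappears when used and respawns after a delay.
; On interact, if interactable, it runs the parent's interact logic, hides its static mesh and disables interaction.
; After RespawnTime elapses, it shows the mesh again and re-enables interaction, reusing the same actor without destroying it.
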(event EventOnInteract
  ;[1 1 1] Interact Event
  (if (Variables|Default|GetIsInteractable)
    (|CallParentFunction)
    (Development|SetHiddeninGame (Variables|Default|GetStaticMesh) true false)
    (Variables|Default|SetIsInteractable false)
    (Utilities|FlowControl|Delay (Variables|Default|GetRespawnTime))
    (Development|SetHiddeninGame (Variables|Default|GetStaticMesh) false false)
    (Variables|Default|SetIsInteractable true)))

(fn ConstructionScript)