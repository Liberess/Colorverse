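; BP_RedLily is a red lily flower pickup in the farming content that goes into the inventory when interacted with.
; Its mesh starts with physics off; Interact turns physics on, applies a zero-vector impulse and adds its ItemData through the InventoryManager.
; The Invisible timeline then drives the root's world scale, and the actor destroys itself when the timeline finishes.
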(event EventBeginPlay
  (|CallParentFunction)
  (Physics|SetSimulatePhysics (Variables|Default|GetStaticMesh) false))

(event EventInteract
  (bind _staticmesh (Variables|Default|GetStaticMesh))
  ;[1 1 1] Interact Event
  (Physics|SetSimulatePhysics _staticmesh true)
  (Physics|AddImpulse _staticmesh "0, 0, 0" "None" false)
  (Class|InventoryManager|AddInventoryItem (Subsystems|GetInventoryManager) (Variables|Default|GetItemData))
  (bind _scale (Timeline|Invisible PlayFromStart)
    (:Update
      (Transformation|SetWorldScale3D (Variables|Default|GetDefaultRoot) _scale))
    (:Finished
      (Actor|DestroyActor))))

(fn ConstructionScript)