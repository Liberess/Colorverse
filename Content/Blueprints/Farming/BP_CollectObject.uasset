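; BP_CollectObject is a collectable farming object that can be harvested into the player's inventory.
; ActiveGlown, when the object is grown, plays or reverses a timeline that scales the static mesh, depending on whether the current scale equals one.
; Interact, given a valid Geometry Collection, enables its physics, adds the item to the inventory manager, then runs a scale timeline and destroys the actor.
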(event EventActiveGlown
  ;[1 1 1] Active Glown Event
  (Development|PrintString "Glown")
  (if (Variables|Default|GetbIsGrown)
    (if (Class|KismetMathLibrary|EqualExactlyVectorVector (Variables|Default|GetCurrentScale) (Class|KismetMathLibrary|VectorOne))
      (bind _grown (Timeline|Glown Play)
        (:Update
          (Transformation|SetRelativeScale3D (Variables|Default|GetStaticMesh) (Math|Conversions|ToVector(Float) _grown))))
      (else
        (Timeline|Glown Reverse)))))

(event EventInteract
  (bind _geometrycollection (Variables|Default|GetGeometryCollection))
  ;[1 1 1] Interact Event
  (Utilities|IsValid _geometrycollection
    (:Is%20Valid
      (Physics|SetSimulatePhysics _geometrycollection true)
      (Physics|AddImpulse _geometrycollection "0, 0, 0" "None" false)
      (Class|InventoryManager|AddInventoryItem (Subsystems|GetInventoryManager) (Variables|Default|GetItemData))
      (bind _scale (Timeline|Invisible PlayFromStart)
        (:Update
          (Transformation|SetWorldScale3D (Variables|Default|GetDefaultRoot) _scale))
        (:Finished
          (Actor|DestroyActor))))))

(event EventBeginPlay
  (|CallParentFunction))

(fn ConstructionScript)