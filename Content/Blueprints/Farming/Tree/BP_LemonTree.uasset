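; BP_LemonTree is an interactable fruit tree whose fruits regrow and drop as its collect state toggles.
; At BeginPlay it caches child fruit meshes with their original locations and gives each a dynamic material.
; Activation teleports fruits back and runs timelines for growth and opacity, while deactivation enables physics and reverses the fade.
; Interaction, when allowed, plays a pickup sound before calling the parent's logic.
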(event EventBeginPlay
  ;[1 1 1] 과일 스태틱 메시 세팅
  (for _array_element (Components|GetChildrenComponents (Variables|Default|GetStaticMesh) false)
    (bind _as스태틱_메시_컴포넌트 (Utilities|Casting|CastToStaticMeshComponent _array_element))
    (Utilities|Array|Add (Variables|Default|GetFruitMeshes) _as스태틱_메시_컴포넌트)
    (Utilities|Array|Add (Variables|Default|GetOriginLocations) (Transformation|GetWorldLocation _as스태틱_메시_컴포넌트))
    (Variables|Default|SetOriginScale (Transformation|GetWorldScale _as스태틱_메시_컴포넌트))
    (Rendering|Material|CreateDynamicMaterialInstance _as스태틱_메시_컴포넌트 0 (Variables|Default|GetFruitMatTemplate) "None" :!class /Script/Engine.PrimitiveComponent)))

(event EventSetActiveCollectObject
  (params (active :type Boolean))
  ;[1 1 1] Set Active Fruits
  (if active
    (for (_array_element _array_index) (Variables|Default|GetFruitMeshes)
      (Physics|SetSimulatePhysics _array_element false)
      (Transformation|SetWorldLocation _array_element (Utilities|Array|Get(acopy) (Variables|Default|GetOriginLocations) _array_index) false true)
      (Utilities|FlowControl|Sequence
        (:then_0
          (bind _grown (Timeline|Grown PlayFromStart)
            (:Update
              (for _array_element_2 (Variables|Default|GetFruitMeshes)
                (Transformation|SetWorldScale3D _array_element_2 (Math|Conversions|ToVector(Float) _grown))))))
        (:then_1
          (bind _alpha (Timeline|Visible PlayFromStart)
            (:Update
              (for _array_element_3 (Variables|Default|GetFruitMeshes)
                (bind _as머티리얼_인스턴스_다이내믹 (Utilities|Casting|CastToMaterialInstanceDynamic (Rendering|Material|GetMaterial _array_element_3 0)))
                (Rendering|Material|SetScalarParameterValue _as머티리얼_인스턴스_다이내믹 "Opacity" _alpha :!class /Script/Engine.MaterialInstanceDynamic)))))))
    (else
      (for _array_element_4 (Variables|Default|GetFruitMeshes)
        (Physics|SetSimulatePhysics _array_element_4 true)
        (Timeline|Visible ReverseFromEnd)))))

(event EventOnInteract
  (if (Variables|Default|GetIsInteractable)
    (Audio|SpawnSoundatLocation "/Game/Sounds/Charater/Get_item.Get_item" (Transformation|GetActorLocation) "0, 0, 0" 1.0 1.0 0.0 0 0)
    (|CallParentFunction)))

(fn ConstructionScript)