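; Apple tree actor for farming whose fruit regrows or drops as its collectable state toggles.
; BeginPlay caches the tree mesh's child fruit meshes and their locations, and gives each a dynamic material instance.
; SetActiveCollectObject(true) snaps fruit back without physics, then timelines scale them up and drive material Opacity.
; Deactivating enables physics on the fruit and reverses the opacity timeline to fade them out.
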(event EventBeginPlay
  ;[1 1 1] 과일 스태틱 메시 세팅
  (for _array_element (Components|GetChildrenComponents (Variables|Default|GetStaticMesh) false)
    (bind _as스태틱_메시_컴포넌트 (Utilities|Casting|CastToStaticMeshComponent _array_element))
    (Utilities|Array|Add (Variables|Default|GetFruitMeshes) _as스태틱_메시_컴포넌트)
    (Utilities|Array|Add (Variables|Default|GetOriginLocations) (Transformation|GetWorldLocation _as스태틱_메시_컴포넌트))
    (Variables|Default|SetOriginScale (Transformation|GetWorldScale _as스태틱_메시_컴포넌트))
    (bind _returnvalue (Rendering|Material|CreateDynamicMaterialInstance _as스태틱_메시_컴포넌트 0 (Variables|Default|GetFruitMatTemplate) "None" :!class /Script/Engine.PrimitiveComponent))
    (Utilities|Array|Add (Variables|Default|GetChildFruitMIs) _returnvalue)))

(event EventSetActiveCollectObject
  (params (active :type Boolean))
  ;[1 1 1] Set Active Fruits
  (if active
    (for (_array_element _array_index) (Variables|Default|GetFruitMeshes)
      (Utilities|IsValid _array_element
        (:Is%20Valid
          (Physics|SetSimulatePhysics _array_element false)
          (Transformation|SetWorldLocation _array_element (Utilities|Array|Get(acopy) (Variables|Default|GetOriginLocations) _array_index) false true)
          (Utilities|FlowControl|Sequence
            (:then_0
              (bind _grown (Timeline|Grown PlayFromStart)
                (:Update
                  (for _array_element_2 (Variables|Default|GetFruitMeshes)
                    (Transformation|SetWorldScale3D _array_element_2 (Math|Conversions|ToVector(Float) _grown))))))
            (:then_1
              (bind _alpha (Timeline|Visible PlayFromStart)
                (:Update
                  (for _array_element_3 (Variables|Default|GetChildFruitMIs)
                    (Rendering|Material|SetScalarParameterValue _array_element_3 "Opacity" _alpha :!class /Script/Engine.MaterialInstanceDynamic)))))))))
    (else
      (for _array_element_4 (Variables|Default|GetFruitMeshes)
        (Utilities|IsValid _array_element_4
          (:Is%20Valid
            (Physics|SetSimulatePhysics _array_element_4 true)
            (Timeline|Visible ReverseFromEnd)))))))

(fn ConstructionScript
  (Utilities|Array|Clear (Variables|Default|GetFruitMeshes)))