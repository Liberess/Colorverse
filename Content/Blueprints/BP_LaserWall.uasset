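; BP_LaserWall is a paintable wall that controls the color of a laser paired with it by ID.
; On BeginPlay it searches all BP_Laser actors and caches the one with a matching ID as LinkedLaser.
; CompletePainted switches that laser to TargetColor and prints a debug string.
; PainttoObject extends the parent's paint logic, always flags the color as right, and resets the laser to white when the color tag is Empty.
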(event EventCompletePainted
  (bind _linkedlaser (Variables|Default|GetLinkedLaser))
  (Utilities|IsValid _linkedlaser
    (:Is%20Valid
      (Default|ChangeLaserColor _linkedlaser (Variables|Default|GetTargetColor))
      (Development|PrintString "Hello"))))

(event EventPainttoObject
  (params (PaintColor :type Linear%20Color%20Structure) (CurrentColorTag :type ECombineColors%20Enum :default "Red"))
  (bind _linkedlaser (Variables|Default|GetLinkedLaser))
  (|CallParentFunction PaintColor CurrentColorTag)
  (Variables|Default|SetbIsRightColor true)
  (if (Utilities|Enum|Equal(Enum) CurrentColorTag "Empty")
    (Utilities|IsValid _linkedlaser
      (:Is%20Valid
        (Default|ChangeLaserColor _linkedlaser "(R=1.000000,G=1.000000,B=1.000000,A=1.000000)")))))

(event EventBeginPlay
  (|CallParentFunction)
  (bind _outactors (Actor|GetAllActorsOfClass "/Game/Blueprints/BP_Laser.BP_Laser_C"))
  (bind _array_element (Utilities|Array|ForEachLoopwithBreak _outactors)
    (:LoopBody
      (if (== (Variables|/Game/Blueprints/BP_Laser.BP_Laser_C|GetID _array_element) (Variables|Default|GetID))
        (Variables|Default|SetLinkedLaser _array_element)))))

(fn ConstructionScript)