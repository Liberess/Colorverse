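; BP_Area is an area trigger that shows its AreaName on screen when a BP_ColorverseCharacter enters it.
; It creates its own BP_AreaWidget on BeginPlay, then on overlap begin sets the name, adds the widget to the viewport and shows it.
; Overlap end calls SetHideProgress on the widget, and both overlap events do nothing while the character is teleporting.
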(event Collision|EventActorBeginOverlap
  (params (OtherActor :type Actor%20Object%20Reference))
  (bind _areawidget (Variables|Default|GetAreaWidget))
  (bind _asbp_colorverse_character (Utilities|Casting|CastToBP_ColorverseCharacter OtherActor))
  (if (not (Variables|/Game/Blueprints/BP_ColorverseCharacter.BP_ColorverseCharacter_C|GetIsTeleporting _asbp_colorverse_character))
    (Default|SetAreaName _areawidget (Variables|Default|GetAreaName))
    (UserInterface|Viewport|AddtoViewport _areawidget 1)
    (Default|Show _areawidget)))

(event EventBeginPlay
  (bind _returnvalue (UserInterface|CreateWidget "/Game/UI/BP_AreaWidget.BP_AreaWidget_C"))
  (bind _output_get (Variables|Default|SetAreaWidget _returnvalue))
  (Widget|RemovefromParent _output_get))

(event Collision|EventActorEndOverlap
  (params (OtherActor :type Actor%20Object%20Reference))
  (bind _asbp_colorverse_character (Utilities|Casting|CastToBP_ColorverseCharacter OtherActor))
  (if (not (Variables|/Game/Blueprints/BP_ColorverseCharacter.BP_ColorverseCharacter_C|GetIsTeleporting _asbp_colorverse_character))
    (Default|SetHideProgress (Variables|Default|GetAreaWidget))))

(fn ConstructionScript)