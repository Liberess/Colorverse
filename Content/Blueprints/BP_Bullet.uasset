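; BP_Bullet is a projectile actor that damages slimes on contact.
; While Active, Tick moves it forward by a fixed, frame-rate-dependent step without sweeping, accumulates the distance travelled and calls Deactivate once a short range limit is reached.
; A Collision component overlap with a BP_Slime calls its Attacked function, clears Active and calls Deactivate, while other overlapping actors are ignored.
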(event OnComponentBeginOverlap(collision)
  (params (OverlappedComponent :type Primitive%20Component%20Object%20Reference) (OtherActor :type Actor%20Object%20Reference) (OtherComp :type Primitive%20Component%20Object%20Reference) (OtherBodyIndex :type Integer) (bFromSweep :type Boolean) (SweepResult :type Hit%20Result%20Structure%20%28by%20ref%29))
  (bind _asbp_slime (Utilities|Casting|CastToBP_Slime OtherActor))
  (Class|ColorverseCharacter|Attacked _asbp_slime)
  (Variables|Default|Setactive false)
  (Class|PooledObject|Deactivate))

(event EventTick
  (params (DeltaSeconds :type Float%20%28single-precision%29))
  (if (Variables|Default|Getactive)
    (Transformation|SetActorLocation (+ (Transformation|GetActorLocation) (* (Transformation|GetActorForwardVector) 5.0)) false false)
    (bind _output_get (Variables|Default|Setdistance (+ (Variables|Default|Getdistance) 5.0)))
    (if (>= _output_get 5e+01)
      (Class|PooledObject|Deactivate))))

(fn ConstructionScript)