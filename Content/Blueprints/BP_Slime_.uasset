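; Slime enemy actor that deals contact damage to Colorverse characters during its attack window and reacts to being hit.
; While CombatSystem flags attack tracing, Tick runs a sphere overlap trace at the slime's location.
; Each newly hit actor is recorded in AttackHitResults to prevent repeat hits, and characters receive CombatSystem's current ATK as damage.
; Attacked calls the parent handler and prints the damager and current health.
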(event EventTick
  (params (DeltaSeconds :type Float%20%28single-precision%29))
  (if (Variables|/Script/Colorverse.CombatSystem|GetbIsCanAttackTrace (Variables|Default|GetCombatSystem))
    (Class|ColorverseCharacter|HitCheck)))

(event EventHitCheck
  (bind _returnvalue (Transformation|GetActorLocation))
  (bind (_outhits _returnvalue_2) (Collision|MultiSphereTraceForObjects _returnvalue _returnvalue 5e+01 (Variables|Default|GetObject%20Types) false 0 "ForDuration"))
  (if _returnvalue_2
    (for _array_element _outhits
      (if (== (Utilities|Array|FindItem (Variables|Default|GetAttackHitResults) (.HitActor (Collision|BreakHitResult _array_element))) -1)
        (Utilities|Array|AddUnique (Variables|Default|GetAttackHitResults) (.HitActor (Collision|BreakHitResult _array_element)))
        (bind _ascolorverse_character (Utilities|Casting|CastToColorverseCharacter (.HitActor (Collision|BreakHitResult _array_element))))
        (bind _returnvalue_3 (Class|CombatSystem|GetCurrentATK (Variables|Default|GetCombatSystem)))
        (Class|ColorverseCharacter|Attacked _ascolorverse_character (Utilities|Struct|MakeDamageMessage self _returnvalue_3 (.ImpactPoint (Collision|BreakHitResult _array_element)) (.ImpactNormal (Collision|BreakHitResult _array_element))))))))

(event EventAttacked
  (params (damageMessage :type Damage%20Message%20Structure))
  (|CallParentFunction (Utilities|Struct|MakeDamageMessage (.damager damageMessage) (.damageamount damageMessage) (.hitpoint damageMessage) (.hitnormal damageMessage)))
  (Development|PrintString (Utilities|GetDisplayName (.damager damageMessage)))
  (Development|PrintString (Utilities|String|ToString(Integer) (Variables|/Script/Colorverse.LivingEntity|GetCurrentHealth (Variables|Default|GetLivingEntity)))))

(fn ConstructionScript)