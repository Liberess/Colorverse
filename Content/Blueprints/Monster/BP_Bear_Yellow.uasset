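; Yellow bear monster character that fights the Colorverse player and yields FreshMeat when destroyed.
; Spawns a world HP bar actor that follows it, and feeds attack cooldown and damaged states to its AI Blackboard from anim instance callbacks and hit events.
; A sphere trace at the right-hand socket damages each player once per hit list.
; Incoming hits deal bonus damage when the attacker's paint is Red, and knock the bear back.
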(event Custom|CoolTime
  ;[1 1 1] 애님 노티파이 이벤트
  (AI|Components|Blackboard|SetValueasBool (AI|GetBlackboard (Pawn|GetController)) (Variables|Default|GetCoolTimeKey) true)
  (Utilities|FlowControl|Delay (Variables|Default|GetAttackCoolTime))
  (AI|Components|Blackboard|SetValueasBool (AI|GetBlackboard (Pawn|GetController)) (Variables|Default|GetCoolTimeKey) false))

(event Custom|OnEndDamaged_이벤트
  ;[1 1 1] 애님 노티파이 이벤트
  (Variables|Default|SetbIsAttacked false)
  (AI|Components|Blackboard|SetValueasBool (AI|GetBlackboard (Pawn|GetController)) (Variables|Default|GetDamaged) false))

(event EventAttack
  (params (skillNum :type Integer))
  ;[1 1 1] 공격
  (|CallParentFunction skillNum))

(event EventHitCheck
  (bind _mesh (Variables|Character|GetMesh))
  (bind _returnvalue (Transformation|GetSocketLocation _mesh "Fingers1_R"))
  ;[1 1 1] Hit Check
  (bind (_outhits _returnvalue_2) (Collision|MultiSphereTraceForObjects _returnvalue _returnvalue 1e+02 (Variables|Default|GetObject%20Types) false 0 "None"))
  (if _returnvalue_2
    (for _array_element _outhits
      (if (== (Utilities|Array|FindItem (Variables|Default|GetAttackHitResults) (.HitActor (Collision|BreakHitResult _array_element))) -1)
        (Utilities|Array|AddUnique (Variables|Default|GetAttackHitResults) (.HitActor (Collision|BreakHitResult _array_element)))
        (bind _ascolorverse_character (Utilities|Casting|CastToColorverseCharacter (.HitActor (Collision|BreakHitResult _array_element))))
        (bind _returnvalue_3 (Class|CombatSystem|GetCurrentATK (Variables|Default|GetCombatSystem)))
        (Class|ColorverseCharacter|Attacked _ascolorverse_character (Utilities|Struct|MakeDamageMessage self _returnvalue_3 (.ImpactPoint (Collision|BreakHitResult _array_element)) (.ImpactNormal (Collision|BreakHitResult _array_element)) "700.000000,700.000000,0.000000"))
        (Niagara|SpawnSystematLocation "/Game/Stylized_VFX_StPack/Particles/UPDATE_1_3/P_Web_Hit_01.P_Web_Hit_01" (+ (Transformation|GetActorLocation) (* (Math|Vector|GetForwardVector (Variables|Default|GetFollowCamera)) 2e+02)) (Transformation|GetActorRotation))))))

(event EventTick
  (params (DeltaSeconds :type Float%20%28single-precision%29))
  (bind _hpbar (Variables|Default|GetHPBar))
  (|CallParentFunction DeltaSeconds)
  (Utilities|IsValid _hpbar
    (:Is%20Valid
      (Default|SetHpBarLocation _hpbar (Transformation|GetWorldLocation (Variables|Default|GetHP))))))

(event EventDead
  ;[1 1 1] 죽음
  (|CallParentFunction)
  (Animation|Montage|MontagePlay (Components|SkeletalMesh|GetAnimInstance (Variables|Character|GetMesh)) "/Game/Mannequin/Bear/Animations/Anim_Bear_Death_Bear_Death_Montage.Anim_Bear_Death_Bear_Death_Montage" 1.0 "MontageLength" 0.0 true)
  (Actor|DestroyActor (Variables|Default|GetHPBar)))

(event EventAttacked
  (params (damageMessage :type Damage%20Message%20Structure))
  (bind _rootcomponent (Variables|/Script/Engine.Actor|GetRootComponent (.damager damageMessage)))
  (bind _returnvalue (Math|Vector|GetForwardVector _rootcomponent))
  ;[1 1 1] Damaged
  (bind _asbp_colorverse_character (Utilities|Casting|CastToBP_ColorverseCharacter (.damager damageMessage)))
  (if (Utilities|Enum|Equal(Enum) (Variables|/Script/Colorverse.CombatSystem|GetCurrentPaintColor (Variables|/Script/Colorverse.ColorverseCharacter|GetCombatSystem _asbp_colorverse_character)) "Red")
    (Variables|Default|SetNewDamage (+ (.damageamount damageMessage) 2e+01))
    (Audio|PlaySoundatLocation "/Game/Sounds/Charater/Attack_strong.Attack_strong" (Transformation|GetActorLocation) "0, 0, 0" 1.0 1.0 0.0 0 0 0 0)
    (else
      (Variables|Default|SetNewDamage (.damageamount damageMessage))))
  (|CallParentFunction (Utilities|Struct|MakeDamageMessage (.damager damageMessage) (Variables|Default|GetNewDamage) (.hitpoint damageMessage) (.hitnormal damageMessage) (.hitimpact damageMessage)))
  (AI|Components|Blackboard|SetValueasBool (AI|GetBlackboard (Pawn|GetController)) (Variables|Default|GetDamaged) true)
  (Class|ColorverseCharacter|SetDisabledAttack)
  (Character|LaunchCharacter (Math|Vector|MakeVector (* (.x _returnvalue) 5e+02) (* (.y _returnvalue) 5e+02) 0.0) true true)
  (Audio|PlaySoundatLocation "/Game/Sounds/Slime_Damaged.Slime_Damaged" (Transformation|GetActorLocation) "0, 0, 0" 1.0 1.0 0.0 0 0 0 0))

(event EventDestroy
  (bind _returnvalue (Subsystems|GetInventoryManager))
  ;[1 1 1] 죽음
  (Utilities|FlowControl|Delay 0.5)
  ;;[1 1 1] 몬스터 부산물 생성
  (Utilities|IsValid _returnvalue
    (:Is%20Valid
      (bind _returnvalue_2 (Utilities|GetDataTableRow "/Game/DataTables/DT_ItemData.DT_ItemData" "FreshMeat")
        (:then
          (Class|InventoryManager|AddInventoryItem _returnvalue _returnvalue_2 true)
          (Actor|DestroyActor))))))

(event EventBeginPlay
  ;[1 1 1] BeginPlay
  (|CallParentFunction)
  (Utilities|FlowControl|Sequence
    (:then_0
      ;[1 1 1] 애님 노티파이 이벤트
      (bind _ascolorverse_character_anim_instance (Utilities|Casting|CastToColorverseCharacterAnimInstance (Components|SkeletalMesh|GetAnimInstance (Variables|Character|GetMesh))))
      (Utilities|FlowControl|Sequence
        (:then_0
          (EventDispatchers|BindEventtoOnEndAttack _ascolorverse_character_anim_instance (delegate Custom|CoolTime)))
        (:then_1
          (EventDispatchers|AssignOnEndDamaged _ascolorverse_character_anim_instance (delegate Custom|OnEndDamaged_이벤트)))))
    (:then_1
      (bind _returnvalue (Game|SpawnActorfromClass "/Game/Blueprints/Monster/BP_HPBar.BP_HPBar_C" (Math|Transform|MakeTransform (Transformation|GetWorldLocation (Variables|Default|GetHP))) "Undefined" 0 0))
      (bind _output_get (Variables|Default|SetHPBar _returnvalue))
      (bind _asbp_monster_hp (Utilities|Casting|CastToBP_MonsterHP (UserInterface|GetWidget (Variables|/Game/Blueprints/Monster/BP_HPBar.BP_HPBar_C|GetWidget _output_get))))
      (Variables|/Game/UI/BP_MonsterHP.BP_MonsterHP_C|SetLivingEntity _asbp_monster_hp (Variables|Default|GetLivingEntity)))))

(fn ConstructionScript)