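; Blue deer boss with three water-themed attacks that, when destroyed, increases color on Sanctums sharing its PuzzleTag.
; Attack selects staggered water-ball shots, capped temporary water pools, or a brief floor skill that sets a strong hit impact.
; Skills drive blackboard attacking and random-cooldown flags, while HitCheck sphere-traces from the head to damage each player once.
; Lethal damage plays a death montage and stops the AI, borrowed from the slime controller class.
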(event Custom|CoolTime
  (AI|Components|Blackboard|SetValueasBool (AI|GetBlackboard (Pawn|GetController)) (Variables|Default|GetCool%20Time%20Key) true)
  (Utilities|FlowControl|Delay (Math|Random|RandomFloatinRange 3.0 7.0))
  (AI|Components|Blackboard|SetValueasBool (AI|GetBlackboard (Pawn|GetController)) (Variables|Default|GetCool%20Time%20Key) false))

(event Custom|blackborad%20isAttacking%20False
  (AI|Components|Blackboard|SetValueasBool (AI|GetBlackboard (Pawn|GetController)) (Variables|Default|GetIs%20Attacking%20Key) false)
  (Variables|Default|SetImpact "0, 0, 0"))

(event EventHitCheck
  (bind _mesh (Variables|Character|GetMesh))
  (bind _returnvalue (Transformation|GetSocketLocation _mesh "Head_M"))
  ;[1 1 1] Hit Check
  (bind (_outhits _returnvalue_2) (Collision|MultiSphereTraceForObjects _returnvalue _returnvalue 5e+02 (Variables|Default|GetObject%20Types) false 0 "ForDuration"))
  (if _returnvalue_2
    (for _array_element _outhits
      (if (== (Utilities|Array|FindItem (Variables|Default|GetAttackHitResults) (.HitActor (Collision|BreakHitResult _array_element))) -1)
        (Utilities|Array|AddUnique (Variables|Default|GetAttackHitResults) (.HitActor (Collision|BreakHitResult _array_element)))
        (bind _ascolorverse_character (Utilities|Casting|CastToColorverseCharacter (.HitActor (Collision|BreakHitResult _array_element))))
        (bind _returnvalue_3 (Class|CombatSystem|GetCurrentATK (Variables|Default|GetCombatSystem)))
        (Class|ColorverseCharacter|Attacked _ascolorverse_character (Utilities|Struct|MakeDamageMessage self _returnvalue_3 (.ImpactPoint (Collision|BreakHitResult _array_element)) (.ImpactNormal (Collision|BreakHitResult _array_element)) (Variables|Default|GetImpact)))
        (Niagara|SpawnSystematLocation "/Game/Stylized_VFX_StPack/Particles/UPDATE_1_3/P_Web_Hit_01.P_Web_Hit_01" (+ (Transformation|GetActorLocation) (* (Math|Vector|GetForwardVector (Variables|Default|GetFollowCamera)) 2e+02)) (Transformation|GetActorRotation))))))

(event EventBeginPlay
  (Class|ColorverseMonster|SetActive false)
  (Utilities|FlowControl|Sequence
    (:then_0
      (bind _ascolorverse_character_anim_instance (Utilities|Casting|CastToColorverseCharacterAnimInstance (Components|SkeletalMesh|GetAnimInstance (Variables|Character|GetMesh))))
      (EventDispatchers|BindEventtoOnEndAttack _ascolorverse_character_anim_instance (delegate Custom|blackborad%20isAttacking%20False)))
    (:then_1
      (Utilities|Array|Add (Variables|Default|GetPoints) (Variables|Default|Getpoint1))
      (Utilities|Array|Add (Variables|Default|GetPoints) (Variables|Default|Getpoint2))
      (Utilities|Array|Add (Variables|Default|GetPoints) (Variables|Default|Getpoint3)))))

(event EventAttacked
  (params (damageMessage :type Damage%20Message%20Structure))
  (Class|LivingEntity|ApplyDamage (Variables|Default|GetLivingEntity) damageMessage)
  (if (<= (Variables|/Script/Colorverse.LivingEntity|GetCurrentHealth (Variables|Default|GetLivingEntity)) 0)
    (Class|ColorverseCharacter|Dead)))

(event EventDead
  (|CallParentFunction)
  (Animation|Montage|MontagePlay (Components|SkeletalMesh|GetAnimInstance (Variables|Character|GetMesh)) "/Game/Mannequin/Moose_Boss/Animations/Anim_MooseBoss_Death_Moose_Death_Montage.Anim_MooseBoss_Death_Moose_Death_Montage" 1.0 "MontageLength" 0.0 true)
  (bind _asslime_aicontroller (Utilities|Casting|CastToSlimeAIController (Pawn|GetController)))
  (Class|SlimeAIController|StopAI _asslime_aicontroller))

(event EventDestroy
  (bind _outactors (Actor|GetAllActorsOfClass "/Game/Blueprints/BP_Sanctum.BP_Sanctum_C"))
  (bind _array_element (Utilities|Array|ForEachLoopwithBreak _outactors)
    (:LoopBody
      (if (Utilities|Enum|Equal(Enum) (Variables|/Script/Colorverse.Sanctum|GetPuzzleTag _array_element) (Variables|Default|GetPuzzleTag))
        (Class|Sanctum|IncreaseColor _array_element))
      (Actor|DestroyActor))))

(event EventAttack
  (params (skillNum :type Integer))
  ;[1 1 1] 공격
  (|CallParentFunction skillNum)
  (AI|Components|Blackboard|SetValueasBool (AI|GetBlackboard (Pawn|GetController)) (Variables|Default|GetIs%20Attacking%20Key) true)
  (Utilities|FlowControl|Sequence
    (:then_0
      (if (== skillNum 0)
        (Variables|Default|SetImpact "0, 0, 0")
        (for _index (range 0 2)
          (bind _returnvalue (Game|SpawnActorfromClass "/Game/Blueprints/Monster/Boss/BP_WaterBall.BP_WaterBall_C" (Math|Transform|MakeTransform (Transformation|GetWorldLocation (Utilities|Array|Get(acopy) (Variables|Default|GetPoints) _index)) (Transformation|GetActorRotation) "1.000000,1.000000,1.000000") "Undefined" 0 false 0))
          (Utilities|Array|Add (Variables|Default|GetWaterBalls) _returnvalue))
        (Utilities|FlowControl|Delay 1.5)
        (Default|Shot (Utilities|Array|Get(acopy) (Variables|Default|GetWaterBalls)))
        (Utilities|FlowControl|Delay 1.5)
        (Default|Shot (Utilities|Array|Get(acopy) (Variables|Default|GetWaterBalls) 1))
        (Utilities|FlowControl|Delay 1.5)
        (Default|Shot (Utilities|Array|Get(acopy) (Variables|Default|GetWaterBalls) 2))
        (Utilities|FlowControl|Delay 2.0)
        (AI|Components|Blackboard|SetValueasBool (AI|GetBlackboard (Pawn|GetController)) (Variables|Default|GetIs%20Attacking%20Key) false)
        (Class|ColorverseCharacter|SetDisabledAttack)
        (Utilities|Array|Clear (Variables|Default|GetWaterBalls))
        (CallFunction|CoolTime)))
    (:then_1
      (if (== 1 skillNum)
        (Variables|Default|SetImpact "0, 0, 0")
        (if (< (Variables|Default|GetWaterPoolCount) 3)
          (Utilities|FlowControl|Delay 0.2)
          (bind _returnvalue_2 (Game|SpawnActorfromClass "/Game/Blueprints/Monster/Boss/BP_WaterPool.BP_WaterPool_C" (Math|Transform|MakeTransform (.RandomLocation (AI|Navigation|GetRandomReachablePointinRadius (Transformation|GetActorLocation) 5e+02 0 0)) (Transformation|GetActorRotation) "1.000000,1.000000,1.000000") "Undefined" 0 0))
          (Variables|Default|SetWaterPoolCount (+ (Variables|Default|GetWaterPoolCount) 1))
          (Utilities|FlowControl|Delay 0.5)
          (AI|Components|Blackboard|SetValueasBool (AI|GetBlackboard (Pawn|GetController)) (Variables|Default|GetIs%20Attacking%20Key) false)
          (Class|ColorverseCharacter|SetDisabledAttack)
          (CallFunction|CoolTime)
          (Utilities|FlowControl|Delay 5.0)
          (Actor|DestroyActor _returnvalue_2)
          (Variables|Default|SetWaterPoolCount (+ (Variables|Default|GetWaterPoolCount) -1)))))
    (:then_2
      (if (== skillNum 2)
        (Variables|Default|SetImpact "700.000000,700.000000,500.000000")
        (bind _returnvalue_3 (Game|SpawnActorfromClass "/Game/Blueprints/Monster/Boss/BP_SkillFloor.BP_SkillFloor_C" (Math|Transform|MakeTransform (+ (Transformation|GetActorLocation) "0.000000,0.000000,-80.000000") (Transformation|GetActorRotation) "1.000000,1.000000,1.000000") "Undefined" 0 0))
        (Utilities|FlowControl|Delay 0.5)
        (Actor|DestroyActor _returnvalue_3)
        (AI|Components|Blackboard|SetValueasBool (AI|GetBlackboard (Pawn|GetController)) (Variables|Default|GetIs%20Attacking%20Key) false)
        (Class|ColorverseCharacter|SetDisabledAttack)
        (CallFunction|CoolTime)))))

(fn ConstructionScript)