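; Yellow wild boar boss that takes bonus damage from red paint and, on destruction, increases color on Sanctums with a matching puzzle tag.
; RunAI flags the blackboard and shows a boss HP bar; attacks set attacking and random-cooldown keys.
; Attack picks a timeline-driven rush, a timeline leap toward a floor marker at the player, or a dirt-spike burst.
; Leap and burst damage characters through socket-centered sphere traces with per-skill radius and impact.
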(event Custom|CoolTime
  (AI|Components|Blackboard|SetValueasBool (AI|GetBlackboard (Pawn|GetController)) (Variables|Default|GetCool%20Time%20Key) true)
  (Utilities|FlowControl|Delay (Math|Random|RandomFloatinRange 3.0 7.0))
  (AI|Components|Blackboard|SetValueasBool (AI|GetBlackboard (Pawn|GetController)) (Variables|Default|GetCool%20Time%20Key) false))

(event Custom|blackborad%20isAttacking%20False
  (bind _skill1 (Variables|Default|GetSkill1))
  (AI|Components|Blackboard|SetValueasBool (AI|GetBlackboard (Pawn|GetController)) (Variables|Default|GetIs%20Attacking%20Key) false)
  (Variables|Default|SetImpact "0, 0, 0")
  (Utilities|IsValid _skill1
    (:Is%20Valid
      (Utilities|FlowControl|Delay 1.0)
      (Actor|DestroyActor _skill1))))

(event EventHitCheck
  (bind _socket (Variables|Default|GetSocket))
  (bind _mesh (Variables|Character|GetMesh))
  (bind _returnvalue (Transformation|GetSocketLocation _mesh _socket))
  ;[1 1 1] Hit Check
  (bind (_outhits _returnvalue_2) (Collision|MultiSphereTraceForObjects _returnvalue _returnvalue (Variables|Default|GetskillRange) (Variables|Default|GetObject%20Types) false 0 "ForDuration"))
  (if _returnvalue_2
    (for _array_element _outhits
      (if (== (Utilities|Array|FindItem (Variables|Default|GetAttackHitResults) (.HitActor (Collision|BreakHitResult _array_element))) -1)
        (Utilities|Array|AddUnique (Variables|Default|GetAttackHitResults) (.HitActor (Collision|BreakHitResult _array_element)))
        (bind _ascolorverse_character (Utilities|Casting|CastToColorverseCharacter (.HitActor (Collision|BreakHitResult _array_element))))
        (bind _returnvalue_3 (Class|CombatSystem|GetCurrentATK (Variables|Default|GetCombatSystem)))
        (Class|ColorverseCharacter|Attacked _ascolorverse_character (Utilities|Struct|MakeDamageMessage self _returnvalue_3 (.ImpactPoint (Collision|BreakHitResult _array_element)) (.ImpactNormal (Collision|BreakHitResult _array_element)) (Variables|Default|GetImpact)))
        (Niagara|SpawnSystematLocation "/Game/Stylized_VFX_StPack/Particles/UPDATE_1_3/P_Web_Hit_01.P_Web_Hit_01" (+ (Transformation|GetActorLocation) (* (Math|Vector|GetForwardVector (Variables|Default|GetFollowCamera)) 2e+02)) (Transformation|GetActorRotation))))))

(event EventAttacked
  (params (damageMessage :type Damage%20Message%20Structure))
  (bind _asbp_colorverse_character (Utilities|Casting|CastToBP_ColorverseCharacter (.damager damageMessage)))
  (if (Utilities|Enum|Equal(Enum) (Variables|/Script/Colorverse.CombatSystem|GetCurrentPaintColor (Variables|/Script/Colorverse.ColorverseCharacter|GetCombatSystem _asbp_colorverse_character)) "Red")
    (Variables|Default|SetNewDamage (+ (.damageamount damageMessage) 2e+01))
    (Audio|PlaySoundatLocation "/Game/Sounds/Charater/Attack_strong.Attack_strong" (Transformation|GetActorLocation) "0, 0, 0" 1.0 1.0 0.0 0 0 0 0)
    (else
      (Variables|Default|SetNewDamage (.damageamount damageMessage))))
  (Class|LivingEntity|ApplyDamage (Variables|Default|GetLivingEntity) (Utilities|Struct|MakeDamageMessage 0 (Variables|Default|GetNewDamage) "0.000000,0.000000,0.000000" "0.000000,0.000000,0.000000" "0.000000,0.000000,0.000000"))
  (if (<= (Variables|/Script/Colorverse.LivingEntity|GetCurrentHealth (Variables|Default|GetLivingEntity)) 0)
    (Class|ColorverseCharacter|Dead)
    (Audio|PlaySoundatLocation "/Game/Sounds/Slime_Damaged.Slime_Damaged" (Transformation|GetActorLocation) "0, 0, 0" 1.0 1.0 0.0 0 0 0 0)))

(event EventBeginPlay
  (Class|ColorverseMonster|SetActive false)
  (|CallParentFunction)
  (Utilities|FlowControl|Sequence
    (:then_0
      (bind _ascolorverse_character_anim_instance (Utilities|Casting|CastToColorverseCharacterAnimInstance (Components|SkeletalMesh|GetAnimInstance (Variables|Character|GetMesh))))
      (EventDispatchers|BindEventtoOnEndAttack _ascolorverse_character_anim_instance (delegate Custom|blackborad%20isAttacking%20False)))))

(event EventDead
  (|CallParentFunction)
  (Collision|SetCollisionObjectType (Variables|Character|GetMesh) "ECC_GameTraceChannel8")
  (Animation|Montage|MontagePlay (Components|SkeletalMesh|GetAnimInstance (Variables|Character|GetMesh)) "/Game/Mannequin/Boar_Boss/Animations/Anim_BoarBoss_Death_BoarBoss_Death_Montage.Anim_BoarBoss_Death_BoarBoss_Death_Montage" 1.0 "MontageLength" 0.0 true)
  (bind _asslime_aicontroller (Utilities|Casting|CastToSlimeAIController (Pawn|GetController)))
  (Class|SlimeAIController|StopAI _asslime_aicontroller))

(event EventRunAI
  (AI|Components|Blackboard|SetValueasBool (AI|GetBlackboard (Pawn|GetController)) (Variables|Default|GetKey%20Name) true)
  (bind _returnvalue (UserInterface|CreateWidget "/Game/UI/BP_BossHP.BP_BossHP_C"))
  (Variables|Default|SetHPBar _returnvalue)
  (Variables|/Game/UI/BP_BossHP.BP_BossHP_C|SetLivingEntity (Variables|Default|GetHPBar) (Variables|Default|GetLivingEntity))
  (UserInterface|Viewport|AddtoViewport (Variables|Default|GetHPBar) 0))

(event EventDestroy
  (Utilities|FlowControl|Sequence
    (:then_0
      (bind _outactors (Actor|GetAllActorsOfClass "/Game/Blueprints/BP_Sanctum.BP_Sanctum_C"))
      (bind _array_element (Utilities|Array|ForEachLoopwithBreak _outactors)
        (:LoopBody
          (if (Utilities|Enum|Equal(Enum) (Variables|/Script/Colorverse.Sanctum|GetPuzzleTag _array_element) (Variables|Default|GetPuzzleTag))
            (Class|Sanctum|IncreaseColor _array_element)))))
    (:then_1
      (Widget|RemovefromParent (Variables|Default|GetHPBar))
      (Actor|DestroyActor))))

(event EventAttack
  (params (skillNum :type Integer))
  (bind _returnvalue (Transformation|GetActorTransform))
  (bind _returnvalue_2 (Game|Player|GetPlayerPawn 0))
  (bind _returnvalue_3 (Transformation|GetActorTransform))
  ;[1 1 1] 공격
  (|CallParentFunction skillNum)
  (AI|Components|Blackboard|SetValueasBool (AI|GetBlackboard (Pawn|GetController)) (Variables|Default|GetIs%20Attacking%20Key) true)
  (CallFunction|CoolTime)
  (Utilities|FlowControl|Sequence
    (:then_0
      (if (== skillNum 0)
        (Variables|Default|SetImpact "1500.000000,1500.000000,500.000000")
        (Utilities|FlowControl|Delay 1.9)
        (Variables|Default|SetTarget (Transformation|GetActorLocation (Game|Player|GetPlayerPawn 0)))
        (Variables|Default|SetStartPos (Transformation|GetActorLocation))
        (Variables|Default|SetSocket "Head_M")
        (Variables|Default|SetskillRange 3e+02)
        (bind _returnvalue_4 (Game|SpawnActorfromClass "/Game/Blueprints/Monster/Boss/YellowBosSkill1.YellowBosSkill1_C" (Math|Transform|MakeTransform (Math|Vector|MakeVector (.x (.location _returnvalue_3)) (.y (.location _returnvalue_3)) (- (.z (.location _returnvalue_3)) 9e+01)) (Math|Rotator|FindLookatRotation (Variables|Default|GetStartPos) (Variables|Default|GetTarget)) (.scale _returnvalue_3)) "Undefined" 0 0))
        (Variables|Default|SetSkill1 _returnvalue_4)
        (Transformation|SetActorRotation (Math|Rotator|FindLookatRotation (Variables|Default|GetStartPos) (Variables|Default|GetTarget)))
        (Audio|PlaySoundatLocation "/Game/Sounds/Monster/YellowBoss_Rush.YellowBoss_Rush" (Transformation|GetActorLocation) "0, 0, 0" 1.0 1.0 0.0 0 0 0 0)
        (bind _speed (Timeline|타임라인 PlayFromStart)
          (:Update
            (Transformation|SetActorLocation (+ (Transformation|GetActorLocation) (* (Math|Vector|GetUnitDirection(Vector) (Variables|Default|GetStartPos) (Variables|Default|GetTarget)) _speed)) false false))
          (:Finished
            (Ability|Animation|MontageJumptoSection (Components|SkeletalMesh|GetAnimInstance (Variables|Character|GetMesh)) "End" "/Game/Mannequin/Boar_Boss/Animations/Boar_Skill_1.Boar_Skill_1")))))
    (:then_1
      (if (== 1 skillNum)
        (Variables|Default|SetImpact "1000.000000,1000.000000,500.000000")
        (bind _returnvalue_5 (Game|SpawnActorfromClass "/Game/Blueprints/Monster/Boss/BP_SkillFloor.BP_SkillFloor_C" (Math|Transform|MakeTransform (+ (Transformation|GetActorLocation _returnvalue_2) "0.000000,0.000000,-80.000000") (Transformation|GetActorRotation _returnvalue_2) "3.000000,3.000000,3.000000") "Undefined" 0 0))
        (Variables|Default|SetSocket "Chest_M")
        (Variables|Default|SetskillRange 7e+02)
        (Utilities|FlowControl|Delay 1.0)
        (Variables|Default|SetStartPos (Transformation|GetActorLocation))
        (Physics|SetEnableGravity (Variables|Default|GetCapsuleComponent) false)
        (Audio|PlaySoundatLocation "/Game/Sounds/Boss/YellowBoss_Jump.YellowBoss_Jump" (Transformation|GetActorLocation) "0, 0, 0" 1.0 1.0 0.0 0 0 0 0)
        (bind _새_트랙_3 (Timeline|타임라인_1 PlayFromStart)
          (:Update
            (Transformation|SetActorLocation (Math|Vector|MakeVector (.x (+ (Variables|Default|GetStartPos) (* (Transformation|GetActorForwardVector) (Math|Vector|MakeVector (* (.x _새_트랙_3) (Math|Vector|Distance(Vector) (Variables|Default|GetStartPos) (Transformation|GetActorLocation _returnvalue_5))) (* (.y _새_트랙_3) (Math|Vector|Distance(Vector) (Variables|Default|GetStartPos) (Transformation|GetActorLocation _returnvalue_5))) 0.0)))) (.y (+ (Variables|Default|GetStartPos) (* (Transformation|GetActorForwardVector) (Math|Vector|MakeVector (* (.x _새_트랙_3) (Math|Vector|Distance(Vector) (Variables|Default|GetStartPos) (Transformation|GetActorLocation _returnvalue_5))) (* (.y _새_트랙_3) (Math|Vector|Distance(Vector) (Variables|Default|GetStartPos) (Transformation|GetActorLocation _returnvalue_5))) 0.0)))) (* (.z _새_트랙_3) 5e+02)) true true))
          (:Finished
            (Physics|SetEnableGravity (Variables|Default|GetCapsuleComponent) true)
            (Utilities|Array|Clear (Variables|Default|GetAttackHitResults))
            (Class|ColorverseCharacter|HitCheck)
            (Audio|PlaySoundatLocation "/Game/Sounds/Boss/YellowBoss_JumpDown.YellowBoss_JumpDown" (Transformation|GetActorLocation) "0, 0, 0" 1.0 1.0 0.0 0 0 0 0)
            (bind _returnvalue_6 (Game|SpawnActorfromClass "/Game/Blueprints/Monster/Boss/YellowBosSkill2.YellowBosSkill2_C" (Math|Transform|MakeTransform (Math|Vector|MakeVector (.x (.location _returnvalue)) (.y (.location _returnvalue)) (- (.z (.location _returnvalue)) 9e+01)) (.rotation _returnvalue) (.scale _returnvalue)) "Undefined" 0 0))
            (Utilities|FlowControl|Delay 0.5)
            (AI|Components|Blackboard|SetValueasBool (AI|GetBlackboard (Pawn|GetController)) (Variables|Default|GetIs%20Attacking%20Key) false)
            (Actor|DestroyActor _returnvalue_6)
            (Class|ColorverseCharacter|SetDisabledAttack)))))
    (:then_2
      (if (== skillNum 2)
        (Variables|Default|SetSocket "Chest_M")
        (Variables|Default|SetskillRange 7e+02)
        (Variables|Default|SetImpact "700.000000,700.000000,500.000000")
        (Utilities|FlowControl|Delay 0.5)
        (Niagara|SpawnSystematLocation "/Game/Stylized_VFX_StPack/Particles/UPDATE_1_3/P_Dirt_Spikes_01.P_Dirt_Spikes_01" (+ (Transformation|GetActorLocation) "0.000000,0.000000,-80.000000") (Transformation|GetActorRotation) "4.000000,4.000000,4.000000")
        (Audio|PlaySoundatLocation "/Game/Sounds/Boss/YellowBoss_Rock.YellowBoss_Rock" (Transformation|GetActorLocation) "0, 0, 0" 1.0 1.0 0.0 0 0 0 0)
        (Utilities|Array|Clear (Variables|Default|GetAttackHitResults))
        (Class|ColorverseCharacter|HitCheck)
        (Utilities|FlowControl|Delay 0.5)
        (AI|Components|Blackboard|SetValueasBool (AI|GetBlackboard (Pawn|GetController)) (Variables|Default|GetIs%20Attacking%20Key) false)
        (Class|ColorverseCharacter|SetDisabledAttack)))))

(fn ConstructionScript)