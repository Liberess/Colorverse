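; Red wolf boss that takes bonus damage from Blue paint and, on removal, raises color in matching-tag Sanctums.
; Attack runs a timeline-driven lunge at the player with a spawned skill actor, or a timeline spin with Niagara fire.
; Blackboard flags track attacking and randomized cooldown for the AI.
; HitCheck sphere-traces from the head socket for attack damage and impact, while RunAI shows the boss HP bar and death stops the AI.
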(event Custom|CoolTime
  (AI|Components|Blackboard|SetValueasBool (AI|GetBlackboard (Pawn|GetController)) (Variables|Default|GetCool%20Time%20Key) true)
  (Utilities|FlowControl|Delay (Math|Random|RandomFloatinRange 3.0 7.0))
  (AI|Components|Blackboard|SetValueasBool (AI|GetBlackboard (Pawn|GetController)) (Variables|Default|GetCool%20Time%20Key) false))

(event Custom|blackborad%20isAttacking%20False
  (bind _skill1 (Variables|Default|GetSkill1))
  (AI|Components|Blackboard|SetValueasBool (AI|GetBlackboard (Pawn|GetController)) (Variables|Default|GetIs%20Attacking%20Key) false)
  (Variables|Default|SetImpact "0, 0, 0")
  (Utilities|IsValid _skill1
    (:Is%20Valid
      (Utilities|FlowControl|Delay 1.0)
      (Actor|DestroyActor _skill1))))

(event EventHitCheck
  (bind _mesh (Variables|Character|GetMesh))
  (bind _returnvalue (Transformation|GetSocketLocation _mesh "Head_M"))
  ;[1 1 1] Hit Check
  (bind (_outhits _returnvalue_2) (Collision|MultiSphereTraceForObjects _returnvalue _returnvalue 5e+02 (Variables|Default|GetObject%20Types) false 0 "None"))
  (if _returnvalue_2
    (for _array_element _outhits
      (if (== (Utilities|Array|FindItem (Variables|Default|GetAttackHitResults) (.HitActor (Collision|BreakHitResult _array_element))) -1)
        (Utilities|Array|AddUnique (Variables|Default|GetAttackHitResults) (.HitActor (Collision|BreakHitResult _array_element)))
        (bind _ascolorverse_character (Utilities|Casting|CastToColorverseCharacter (.HitActor (Collision|BreakHitResult _array_element))))
        (bind _returnvalue_3 (Class|CombatSystem|GetCurrentATK (Variables|Default|GetCombatSystem)))
        (Class|ColorverseCharacter|Attacked _ascolorverse_character (Utilities|Struct|MakeDamageMessage self _returnvalue_3 (.ImpactPoint (Collision|BreakHitResult _array_element)) (.ImpactNormal (Collision|BreakHitResult _array_element)) (Variables|Default|GetImpact)))
        (Niagara|SpawnSystematLocation "/Game/Stylized_VFX_StPack/Particles/UPDATE_1_3/P_Web_Hit_01.P_Web_Hit_01" (+ (Transformation|GetActorLocation) (* (Math|Vector|GetForwardVector (Variables|Default|GetFollowCamera)) 2e+02)) (Transformation|GetActorRotation))))))

(event EventBeginPlay
  (Class|ColorverseMonster|SetActive false)
  (|CallParentFunction)
  (Utilities|FlowControl|Sequence
    (:then_0
      (bind _ascolorverse_character_anim_instance (Utilities|Casting|CastToColorverseCharacterAnimInstance (Components|SkeletalMesh|GetAnimInstance (Variables|Character|GetMesh))))
      (EventDispatchers|BindEventtoOnEndAttack _ascolorverse_character_anim_instance (delegate Custom|blackborad%20isAttacking%20False)))))

(event EventAttacked
  (params (damageMessage :type Damage%20Message%20Structure))
  (bind _asbp_colorverse_character (Utilities|Casting|CastToBP_ColorverseCharacter (.damager damageMessage)))
  (if (Utilities|Enum|Equal(Enum) (Variables|/Script/Colorverse.CombatSystem|GetCurrentPaintColor (Variables|/Script/Colorverse.ColorverseCharacter|GetCombatSystem _asbp_colorverse_character)) "Blue")
    (Variables|Default|SetNewDamage (+ (.damageamount damageMessage) 2e+01))
    (Audio|PlaySoundatLocation "/Game/Sounds/Charater/Attack_strong.Attack_strong" (Transformation|GetActorLocation) "0, 0, 0" 1.0 1.0 0.0 0 0 0 0)
    (else
      (Variables|Default|SetNewDamage (.damageamount damageMessage))))
  (Class|LivingEntity|ApplyDamage (Variables|Default|GetLivingEntity) (Utilities|Struct|MakeDamageMessage 0 (Variables|Default|GetNewDamage) "0.000000,0.000000,0.000000" "0.000000,0.000000,0.000000" "0.000000,0.000000,0.000000"))
  (if (<= (Variables|/Script/Colorverse.LivingEntity|GetCurrentHealth (Variables|Default|GetLivingEntity)) 0)
    (Class|ColorverseCharacter|Dead)
    (Audio|PlaySoundatLocation "/Game/Sounds/Slime_Damaged.Slime_Damaged" (Transformation|GetActorLocation) "0, 0, 0" 1.0 1.0 0.0 0 0 0 0)))

(event EventDead
  (|CallParentFunction)
  (Collision|SetCollisionObjectType (Variables|Character|GetMesh) "ECC_GameTraceChannel8")
  (Animation|Montage|MontagePlay (Components|SkeletalMesh|GetAnimInstance (Variables|Character|GetMesh)) "/Game/Mannequin/Wolf_Boss/Animations/Anim_WolfBoss_Death_WolfBoss_Death_Montage.Anim_WolfBoss_Death_WolfBoss_Death_Montage" 1.0 "MontageLength" 0.0 true)
  (bind _asslime_aicontroller (Utilities|Casting|CastToSlimeAIController (Pawn|GetController)))
  (Class|SlimeAIController|StopAI _asslime_aicontroller))

(event EventRunAI
  (AI|Components|Blackboard|SetValueasBool (AI|GetBlackboard (Pawn|GetController)) (Variables|Default|GetKey%20Name) true)
  (bind _returnvalue (UserInterface|CreateWidget "/Game/UI/BP_BossHP.BP_BossHP_C"))
  (Variables|Default|SetHPBar _returnvalue)
  (Variables|/Game/UI/BP_BossHP.BP_BossHP_C|SetLivingEntity (Variables|Default|GetHPBar) (Variables|Default|GetLivingEntity))
  (UserInterface|Viewport|AddtoViewport (Variables|Default|GetHPBar) 0))

(event EventDestroy
  (Utilities|FlowControl|Sequence
    (:then_0
      (bind _outactors (Actor|GetAllActorsOfClass "/Game/Blueprints/BP_Sanctum.BP_Sanctum_C"))
      (bind _array_element (Utilities|Array|ForEachLoopwithBreak _outactors)
        (:LoopBody
          (if (Utilities|Enum|Equal(Enum) (Variables|/Script/Colorverse.Sanctum|GetPuzzleTag _array_element) (Variables|Default|GetPuzzleTag))
            (Class|Sanctum|IncreaseColor _array_element)))))
    (:then_1
      (bind _hpbar (Variables|Default|GetHPBar)
        (:then
          (Widget|RemovefromParent _hpbar)
          (bind _asbp_colorverse_character (Utilities|Casting|CastToBP_ColorverseCharacter (Game|GetPlayerCharacter 0)))
          (Default|StopBGM _asbp_colorverse_character)
          (Actor|DestroyActor))
        (:else)))))

(event EventAttack
  (params (skillNum :type Integer))
  (bind _returnvalue (Transformation|GetActorTransform))
  ;[1 1 1] 공격
  (|CallParentFunction skillNum)
  (AI|Components|Blackboard|SetValueasBool (AI|GetBlackboard (Pawn|GetController)) (Variables|Default|GetIs%20Attacking%20Key) true)
  (Utilities|FlowControl|Sequence
    (:then_0
      (if (== skillNum 0)
        (Variables|Default|SetImpact "1500.000000,1500.000000,500.000000")
        (Utilities|FlowControl|Delay 1.9)
        (Variables|Default|SetTarget (Transformation|GetActorLocation (Game|Player|GetPlayerPawn 0)))
        (Variables|Default|SetStartPos (Transformation|GetActorLocation))
        (bind _returnvalue_2 (Game|SpawnActorfromClass "/Game/Blueprints/Monster/Boss/RedBosSkill1.RedBosSkill1_C" (Math|Transform|MakeTransform (Math|Vector|MakeVector (.x (.location _returnvalue)) (.y (.location _returnvalue)) (- (.z (.location _returnvalue)) 9e+01)) (Math|Rotator|FindLookatRotation (Variables|Default|GetStartPos) (Variables|Default|GetTarget)) (.scale _returnvalue)) "Undefined" 0 0))
        (Variables|Default|SetSkill1 _returnvalue_2)
        (bind _speed (Timeline|타임라인_0 PlayFromStart)
          (:Update
            (Transformation|SetActorLocation (+ (Transformation|GetActorLocation) (* (Math|Vector|GetUnitDirection(Vector) (Variables|Default|GetStartPos) (Variables|Default|GetTarget)) _speed)) false false))
          (:Finished
            (Ability|Animation|MontageJumptoSection (Components|SkeletalMesh|GetAnimInstance (Variables|Character|GetMesh)) "End" "/Game/Mannequin/Wolf_Boss/Animations/Anim_WolfBoss_Jump_WolfBoss_Jump_Notransform_Montage.Anim_WolfBoss_Jump_WolfBoss_Jump_Notransform_Montage")
            (CallFunction|CoolTime)))))
    (:then_1
      (if (== skillNum 2)
        (Variables|Default|SetImpact "700.000000,700.000000,500.000000")
        (Utilities|FlowControl|Delay 0.3)
        (bind _returnvalue_3 (Niagara|SpawnSystemAttached "/Game/Effects/ImproveFights_Vfx/Particles/P_FireProjectile_02.P_FireProjectile_02" (Variables|Default|GetCapsuleComponent) "None" "180.000000,0.000000,0.000000" "0, 0, 0" "KeepRelativeOffset" false))
        (bind _output_get (Variables|Default|SetSkill2Effect _returnvalue_3))
        (Effects|Components|ParticleSystem|SetFloatParameter _output_get "Scale" 1.0)
        (Effects|Components|ParticleSystem|SetFloatParameter _output_get "Size" 5.0)
        (Effects|Components|ParticleSystem|SetFloatParameter _output_get "RibbonLenght" 5.0)
        (Effects|Components|ParticleSystem|SetFloatParameter _output_get "RibbonWidth" 3e+02)
        (Variables|Default|SetNewVar (Transformation|GetWorldRotation (Variables|Default|GetCapsuleComponent)))
        (bind _rot (Timeline|타임라인 PlayFromStart)
          (:Update
            (Transformation|SetWorldRotation (Variables|Default|GetCapsuleComponent) (Math|Rotator|CombineRotators (Variables|Default|GetNewVar) (Math|Rotator|MakeRotator 0.0 0.0 _rot)) false false))
          (:Finished
            (Ability|Animation|MontageJumptoSection (Components|SkeletalMesh|GetAnimInstance (Variables|Character|GetMesh)) "End" "/Game/Mannequin/Wolf_Boss/Animations/Anim_WolfBoss_skill_1.Anim_WolfBoss_skill_1")
            (CallFunction|CoolTime)
            (bind _rot_2 (Timeline|타임라인_1 PlayFromStart)
              (:Update
                (Effects|Components|ParticleSystem|SetFloatParameter (Variables|Default|GetSkill2Effect) "RibbonWidth" _rot_2))
              (:Finished
                (Utilities|FlowControl|Delay 1.0)
                (Components|DestroyComponent (Variables|Default|GetSkill2Effect))))))))))

(fn ConstructionScript)