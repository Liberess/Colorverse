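; BP_BigWaterBall is a boss water projectile that is launched at the player by its shot event.
; shot locks the direction to the player's current position and plays a throw sound, then Tick sweeps it along that line at a frame-rate-dependent speed.
; Sphere overlap damages and knocks back the player character without destroying the ball.
; Overlapping WorldStatic spawns a water explosion and a BP_WaterPool_2, then destroys it.
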(event OnComponentBeginOverlap(Sphere1)
  (params (OverlappedComponent :type Primitive%20Component%20Object%20Reference) (OtherActor :type Actor%20Object%20Reference) (OtherComp :type Primitive%20Component%20Object%20Reference) (OtherBodyIndex :type Integer) (bFromSweep :type Boolean) (SweepResult :type Hit%20Result%20Structure%20%28by%20ref%29))
  (bind _returnvalue (Transformation|GetActorLocation))
  (bind _returnvalue_2 (Transformation|GetActorRotation))
  (Utilities|FlowControl|Sequence
    (:then_0
      (bind _asbp_colorverse_character (Utilities|Casting|CastToBP_ColorverseCharacter OtherActor))
      (Class|ColorverseCharacter|Attacked _asbp_colorverse_character (Utilities|Struct|MakeDamageMessage self 5e+01 "0.000000,0.000000,0.000000" "0.000000,0.000000,0.000000" "700.000000,700.000000,500.000000")))
    (:then_1
      (if (Utilities|Enum|Equal(Enum) (Collision|GetCollisionObjectType OtherComp) "ECC_WorldStatic")
        (Niagara|SpawnSystematLocation "/Game/Effects/ImproveFights_Vfx/Particles/P_Water_Explosion.P_Water_Explosion" _returnvalue _returnvalue_2)
        (Game|SpawnActorfromClass "/Game/Blueprints/Monster/Boss/BP_WaterPool_2.BP_WaterPool_2_C" (Math|Transform|MakeTransform (+ _returnvalue "0.000000,0.000000,10.000000") _returnvalue_2 "1.000000,1.000000,1.000000") "Undefined" 0 0)
        (Actor|DestroyActor)))))

(event Custom|shot
  (Variables|Default|Setmove true)
  (Variables|Default|SetDir (Math|Vector|GetUnitDirection(Vector) (Transformation|GetActorLocation) (Transformation|GetActorLocation (Game|Player|GetPlayerPawn 0))))
  (Audio|PlaySoundatLocation "/Game/Sounds/Boss/LastBoss_Throw_WaterShot.LastBoss_Throw_WaterShot" (Transformation|GetActorLocation) "0, 0, 0" 1.0 1.0 0.0 0 0 0 0))

(event EventTick
  (params (DeltaSeconds :type Float%20%28single-precision%29))
  (if (Variables|Default|Getmove)
    (Class|SceneComponent|AddWorldTransform (Variables|Default|GetDefaultSceneRoot) (Math|Transform|MakeTransform (* (Variables|Default|GetDir) (Variables|Default|Getspeed)) "0, 0, 0" "1.000000,1.000000,1.000000") true false)))

(fn ConstructionScript)