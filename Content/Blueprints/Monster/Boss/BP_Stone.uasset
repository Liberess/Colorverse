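; BP_Stone is a boss-attack stone that hurts and launches the player character in two timed area hits.
; BeginPlay runs two delayed branches: an early sphere trace that applies damage, and a later one that disables capsule collision and spawns the asteroid hit effect before tracing again.
; Each trace calls Attacked on a hit BP_ColorverseCharacter with damage and impact.
; The actor destroys itself only when the second trace hits that character.
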(event EventBeginPlay
  (bind _returnvalue (Transformation|GetActorLocation))
  (bind _returnvalue_2 (Transformation|GetActorLocation))
  (Utilities|FlowControl|Sequence
    (:then_0
      (Utilities|FlowControl|Delay 0.5)
      (bind _outhit (Collision|SphereTraceForObjects _returnvalue _returnvalue 4e+02 (Variables|Default|GetObject%20Types) false 0 "None"))
      (if true
        (bind _asbp_colorverse_character (Utilities|Casting|CastToBP_ColorverseCharacter (.HitActor (Collision|BreakHitResult _outhit))))
        (Class|ColorverseCharacter|Attacked _asbp_colorverse_character (Utilities|Struct|MakeDamageMessage self 5e+01 "0.000000,0.000000,0.000000" "0.000000,0.000000,0.000000" "700.000000,700.000000,500.000000"))))
    (:then_1
      (Utilities|FlowControl|Delay 2.7)
      (Collision|SetCollisionEnabled (Variables|Default|GetCapsule) "NoCollision")
      (Niagara|SpawnSystematLocation "/Game/Stylized_VFX_StPack/Particles/UPDATE_1_3/P_Asteroid_Hit.P_Asteroid_Hit" (Transformation|GetActorLocation) (Transformation|GetActorRotation))
      (Utilities|FlowControl|Delay 0.1)
      (bind _outhit_2 (Collision|SphereTraceForObjects _returnvalue_2 _returnvalue_2 4e+02 (Variables|Default|GetObject%20Types) false 0 "None"))
      (if true
        (bind _asbp_colorverse_character_2 (Utilities|Casting|CastToBP_ColorverseCharacter (.HitActor (Collision|BreakHitResult _outhit_2))))
        (Class|ColorverseCharacter|Attacked _asbp_colorverse_character_2 (Utilities|Struct|MakeDamageMessage self 5e+01 "0.000000,0.000000,0.000000" "0.000000,0.000000,0.000000" "700.000000,700.000000,500.000000"))
        (Actor|DestroyActor)))))

(fn ConstructionScript)