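; BP_Wave is a boss wave attack that damages and knocks back characters it touches.
; It finds BP_LastBoss on BeginPlay, then sweeps toward it every tick by Speed, unscaled by delta time, and destroys itself after a fixed delay.
; Capsule overlap calls Attacked on any ColorverseCharacter whose mesh is not on GameTraceChannel1, passing fixed damage and impact, plus a debug print.
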(event OnComponentBeginOverlap(Capsule)
  (params (OverlappedComponent :type Primitive%20Component%20Object%20Reference) (OtherActor :type Actor%20Object%20Reference) (OtherComp :type Primitive%20Component%20Object%20Reference) (OtherBodyIndex :type Integer) (bFromSweep :type Boolean) (SweepResult :type Hit%20Result%20Structure%20%28by%20ref%29))
  (bind _ascolorverse_character (Utilities|Casting|CastToColorverseCharacter OtherActor))
  (if (not (Utilities|Enum|Equal(Enum) (Collision|GetCollisionObjectType (Variables|/Script/Engine.Character|GetMesh _ascolorverse_character)) "ECC_GameTraceChannel1"))
    (Class|ColorverseCharacter|Attacked _ascolorverse_character (Utilities|Struct|MakeDamageMessage self 5e+01 "0.000000,0.000000,0.000000" "0.000000,0.000000,0.000000" "700.000000,700.000000,500.000000"))
    (Development|PrintString "Hello")))

(event EventTick
  (params (DeltaSeconds :type Float%20%28single-precision%29))
  (Class|SceneComponent|AddWorldTransform (Variables|Default|GetDefaultSceneRoot) (Math|Transform|MakeTransform (* (Math|Vector|GetUnitDirection(Vector) (Transformation|GetActorLocation) (Transformation|GetActorLocation (Variables|Default|Getmaster))) (Variables|Default|Getspeed)) "0, 0, 0" "1.000000,1.000000,1.000000") true false))

(event EventBeginPlay
  (bind _returnvalue (Actor|GetActorOfClass "/Game/Blueprints/Monster/Boss/BP_LastBoss.BP_LastBoss_C"))
  (Variables|Default|Setmaster _returnvalue)
  (Utilities|FlowControl|Delay 7.0)
  (Actor|DestroyActor))

(fn ConstructionScript)