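; Final boss character for Colorverse that advances through health-threshold phases, stepping its paint color toward Blue.
; Attack picks montages by phase and skill number, including a fireball volley, syncing attack and random cooldown flags to the AI blackboard; phase 2 skills are empty.
; HitCheck sphere-traces at the head socket to damage players with per-skill impact.
; Death stops the AI; Destroy raises color on Sanctums matching its puzzle tag.
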(event Custom|CoolTime
  (AI|Components|Blackboard|SetValueasBool (AI|GetBlackboard (Pawn|GetController)) (Variables|Default|GetCool%20Time%20Key) true)
  (Utilities|FlowControl|Delay (Math|Random|RandomFloatinRange 3.0 7.0))
  (AI|Components|Blackboard|SetValueasBool (AI|GetBlackboard (Pawn|GetController)) (Variables|Default|GetCool%20Time%20Key) false))

(event Custom|blackborad%20isAttacking%20False
  (AI|Components|Blackboard|SetValueasBool (AI|GetBlackboard (Pawn|GetController)) (Variables|Default|GetIs%20Attacking%20Key) false)
  (Variables|Default|SetImpact "0, 0, 0"))

(event Custom|ChangePhase
  (bind _combatsystem (Variables|Default|GetCombatSystem))
  (Variables|Default|Setphase (+ (Variables|Default|Getphase) 1))
  (Variables|Default|SetNextPhaseHP (Utilities|Array|Get(acopy) (Variables|Default|GetPhaseHPs) (+ (Variables|Default|Getphase) 1)))
  (if (not (Utilities|Enum|Equal(Enum) (Variables|/Script/Colorverse.CombatSystem|GetCurrentPaintColor _combatsystem) "Blue"))
    (Variables|/Script/Colorverse.CombatSystem|SetCurrentPaintColor _combatsystem (Utilities|Enum|ByteToEnumECombineColors (+ (Variables|/Script/Colorverse.CombatSystem|GetCurrentPaintColor _combatsystem) 1)))))

(event Custom|shot
  (bind _returnvalue (Game|SpawnActorfromClass "/Game/Blueprints/Monster/Boss/BP_FireBall.BP_FireBall_C" (Math|Transform|MakeTransform (Transformation|GetWorldLocation (Variables|Default|GetShotPos)) (Transformation|GetActorRotation) "1.000000,1.000000,1.000000") "Undefined" 0 false 0))
  (Default|Shot _returnvalue))

(event EventHitCheck
  (bind _mesh (Variables|Character|GetMesh))
  (bind _returnvalue (Transformation|GetSocketLocation _mesh "Head_M"))
  ;[1 1 1] Hit Check
  (bind (_outhits _returnvalue_2) (Collision|MultiSphereTraceForObjects _returnvalue _returnvalue 5e+02 (Variables|Default|GetObject%20Types) false 0 "ForDuration"))
  (if _returnvalue_2
    (for _array_element _outhits
      (if (== (Utilities|Array|FindItem (Variables|Default|GetAttackHitResults) (.HitActor (Collision|BreakHitResult _array_element))) -1)
        (Utilities|Array|AddUnique (Variables|Default|GetAttackHitResults) (.HitActor (Collision|BreakHitResult _array_element)))
        (bind _ascolorverse_character (Utilities|Casting|CastToColorverseCharacter (.HitActor (Collision|BreakHitResult _array_element))))
        (bind _returnvalue_3 (Class|CombatSystem|GetCurrentATK (Variables|Default|GetCombatSystem)))
        (Class|ColorverseCharacter|Attacked _ascolorverse_character (Utilities|Struct|MakeDamageMessage self _returnvalue_3 (.ImpactPoint (Collision|BreakHitResult _array_element)) (.ImpactNormal (Collision|BreakHitResult _array_element)) (Variables|Default|GetImpact)))
        (Niagara|SpawnSystematLocation "/Game/Stylized_VFX_StPack/Particles/UPDATE_1_3/P_Web_Hit_01.P_Web_Hit_01" (+ (Transformation|GetActorLocation) (* (Math|Vector|GetForwardVector (Variables|Default|GetFollowCamera)) 2e+02)) (Transformation|GetActorRotation))))))

(event EventTick
  (params (DeltaSeconds :type Float%20%28single-precision%29))
  (if (<= (Variables|/Script/Colorverse.LivingEntity|GetCurrentHealth (Variables|Default|GetLivingEntity)) (Variables|Default|GetNextPhaseHP))
    (CallFunction|ChangePhase)))

(event EventAttacked
  (params (damageMessage :type Damage%20Message%20Structure))
  (Class|LivingEntity|ApplyDamage (Variables|Default|GetLivingEntity) damageMessage)
  (if (<= (Variables|/Script/Colorverse.LivingEntity|GetCurrentHealth (Variables|Default|GetLivingEntity)) 0)
    (Class|ColorverseCharacter|Dead)))

(event EventDead
  (|CallParentFunction)
  (Animation|Montage|MontagePlay (Components|SkeletalMesh|GetAnimInstance (Variables|Character|GetMesh)) "/Game/Mannequin/Moose_Boss/Animations/Anim_MooseBoss_Death_Moose_Death_Montage.Anim_MooseBoss_Death_Moose_Death_Montage" 1.0 "MontageLength" 0.0 true)
  (bind _asslime_aicontroller (Utilities|Casting|CastToSlimeAIController (Pawn|GetController)))
  (Class|SlimeAIController|StopAI _asslime_aicontroller))

(event EventDestroy
  (bind _outactors (Actor|GetAllActorsOfClass "/Game/Blueprints/BP_Sanctum.BP_Sanctum_C"))
  (bind _array_element (Utilities|Array|ForEachLoopwithBreak _outactors)
    (:LoopBody
      (if (Utilities|Enum|Equal(Enum) (Variables|/Script/Colorverse.Sanctum|GetPuzzleTag _array_element) (Variables|Default|GetPuzzleTag))
        (Class|Sanctum|IncreaseColor _array_element))
      (Actor|DestroyActor))))

(event EventBeginPlay
  (Class|ColorverseMonster|SetActive true)
  (|CallParentFunction)
  (Utilities|FlowControl|Sequence
    (:then_0
      (bind _ascolorverse_character_anim_instance (Utilities|Casting|CastToColorverseCharacterAnimInstance (Components|SkeletalMesh|GetAnimInstance (Variables|Character|GetMesh))))
      (EventDispatchers|BindEventtoOnEndAttack _ascolorverse_character_anim_instance (delegate Custom|blackborad%20isAttacking%20False)))
    (:then_1
      (bind _output_get (Variables|Default|Setphase 0))
      (Variables|Default|SetNextPhaseHP (Utilities|Array|Get(acopy) (Variables|Default|GetPhaseHPs) _output_get)))))

(event EventAttack
  (params (skillNum :type Integer))
  (bind _mesh (Variables|Character|GetMesh))
  (bind _mesh_2 (Variables|Character|GetMesh))
  (bind _mesh_3 (Variables|Character|GetMesh))
  (bind _mesh_4 (Variables|Character|GetMesh))
  (bind _returnvalue (Components|SkeletalMesh|GetAnimInstance _mesh))
  (bind _returnvalue_2 (Components|SkeletalMesh|GetAnimInstance _mesh_2))
  (bind _returnvalue_3 (Components|SkeletalMesh|GetAnimInstance _mesh_3))
  (bind _returnvalue_4 (Components|SkeletalMesh|GetAnimInstance _mesh_4))
  (if (and (not (Class|LivingEntity|GetDead (Variables|Default|GetLivingEntity))) (not (Variables|Default|GetbIsAttacking)))
    (Variables|Default|SetbIsAttacking true)
    (AI|Components|Blackboard|SetValueasBool (AI|GetBlackboard (Pawn|GetController)) (Variables|Default|GetIs%20Attacking%20Key) true)
    ;[1 1 1] 페이즈
    (switch int (Variables|Default|Getphase)
      (:0
        ;[1 1 1] 공격
        (Utilities|FlowControl|Sequence
          (:then_0
            (if (== skillNum 0)
              (bind _ascolorverse_character_anim_instance (Utilities|Casting|CastToColorverseCharacterAnimInstance _returnvalue_3))
              (Animation|Montage|MontagePlay _returnvalue_3 (Utilities|Array|Get(acopy) (Variables|/Script/Colorverse.ColorverseCharacterAnimInstance|GetAttackMontage _ascolorverse_character_anim_instance)) 1.0 "MontageLength" 0.0 true)
              (Utilities|FlowControl|Delay 1.0)
              (CallFunction|Shot)
              (Utilities|FlowControl|Delay 0.5)
              (CallFunction|Shot)
              (Utilities|FlowControl|Delay 0.5)
              (CallFunction|Shot)
              (Utilities|FlowControl|Delay 0.5)
              (CallFunction|Shot)
              (Utilities|FlowControl|Delay 0.5)
              (CallFunction|Shot)
              (Utilities|FlowControl|Delay 0.5)
              (Ability|Animation|MontageJumptoSection (Components|SkeletalMesh|GetAnimInstance (Variables|Character|GetMesh)) "End" "/Game/Mannequin/SpaceElemental/Animations/Anim_Idle3_Montage.Anim_Idle3_Montage")
              (CallFunction|CoolTime)))
          (:then_1
            (if (== 1 skillNum)
              (Variables|Default|SetImpact "0, 0, 0")
              (Class|ColorverseCharacter|SetDisabledAttack)
              (AI|Components|Blackboard|SetValueasBool (AI|GetBlackboard (Pawn|GetController)) (Variables|Default|GetIs%20Attacking%20Key) false)
              (CallFunction|CoolTime)))
          (:then_2
            (if (== skillNum 2)
              (Variables|Default|SetImpact "700.000000,700.000000,500.000000")
              (bind _ascolorverse_character_anim_instance_2 (Utilities|Casting|CastToColorverseCharacterAnimInstance _returnvalue_2))
              (Animation|Montage|MontagePlay _returnvalue_2 (Utilities|Array|Get(acopy) (Variables|/Script/Colorverse.ColorverseCharacterAnimInstance|GetAttackMontage _ascolorverse_character_anim_instance_2) 1) 1.0 "MontageLength" 0.0 true)
              (CallFunction|CoolTime)))))
      (:1
        (Utilities|FlowControl|Sequence
          (:then_0
            (if (== 0 skillNum)
              (bind _ascolorverse_character_anim_instance_3 (Utilities|Casting|CastToColorverseCharacterAnimInstance _returnvalue))
              (Animation|Montage|MontagePlay _returnvalue (Utilities|Array|Get(acopy) (Variables|/Script/Colorverse.ColorverseCharacterAnimInstance|GetAttackMontage _ascolorverse_character_anim_instance_3)) 1.0 "MontageLength" 0.0 true)
              (Utilities|FlowControl|Delay 1.5)))
          (:then_1
            (if (== 1 skillNum)
              (bind _ascolorverse_character_anim_instance_4 (Utilities|Casting|CastToColorverseCharacterAnimInstance _returnvalue_4))
              (Animation|Montage|MontagePlay _returnvalue_4 (Utilities|Array|Get(acopy) (Variables|/Script/Colorverse.ColorverseCharacterAnimInstance|GetAttackMontage _ascolorverse_character_anim_instance_4) 2) 1.0 "MontageLength" 0.0 true)
              (Utilities|FlowControl|Delay 1.5)))
          (:then_2
            (if (== 2 skillNum)
              (Variables|Default|SetImpact "0, 0, 0")
              (Class|ColorverseCharacter|SetDisabledAttack)
              (AI|Components|Blackboard|SetValueasBool (AI|GetBlackboard (Pawn|GetController)) (Variables|Default|GetIs%20Attacking%20Key) false)
              (CallFunction|CoolTime)))))
      (:2
        (Utilities|FlowControl|Sequence
          (:then_0
            (if (== 0 skillNum)
              _))
          (:then_1
            (if (== 1 skillNum)
              _))
          (:then_2
            (if (== 2 skillNum)
              _)))))))

(fn ConstructionScript)