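; BP_FireBall is a boss projectile that flies at the player and deals damage on contact.
; Calling shot locks its direction toward the player pawn's current position, and Tick then sweeps it along that fixed line at a per-frame speed.
; Sphere overlap calls Attacked on a BP_ColorverseCharacter and destroys the fireball, which also dies on WorldStatic overlap or four seconds after spawning.
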(event OnComponentBeginOverlap(Sphere1)
  (params (OverlappedComponent :type Primitive%20Component%20Object%20Reference) (OtherActor :type Actor%20Object%20Reference) (OtherComp :type Primitive%20Component%20Object%20Reference) (OtherBodyIndex :type Integer) (bFromSweep :type Boolean) (SweepResult :type Hit%20Result%20Structure%20%28by%20ref%29))
  (Utilities|FlowControl|Sequence
    (:then_0
      (bind _asbp_colorverse_character (Utilities|Casting|CastToBP_ColorverseCharacter OtherActor))
      (Class|ColorverseCharacter|Attacked _asbp_colorverse_character (Utilities|Struct|MakeDamageMessage self 1e+01 "0.000000,0.000000,0.000000" "0.000000,0.000000,0.000000" "0.000000,0.000000,0.000000"))
      (Actor|DestroyActor))
    (:then_1
      (if (Utilities|Enum|Equal(Enum) (Collision|GetCollisionObjectType OtherComp) "ECC_WorldStatic")
        (Actor|DestroyActor)))))

(event Custom|shot
  (Variables|Default|Setmove true)
  (Variables|Default|SetDir (Math|Vector|GetUnitDirection(Vector) (Transformation|GetActorLocation) (Transformation|GetActorLocation (Game|Player|GetPlayerPawn 0)))))

(event EventTick
  (params (DeltaSeconds :type Float%20%28single-precision%29))
  (if (Variables|Default|Getmove)
    (Class|SceneComponent|AddWorldTransform (Variables|Default|GetDefaultSceneRoot) (Math|Transform|MakeTransform (* (Variables|Default|GetDir) (Variables|Default|Getspeed)) "0, 0, 0" "1.000000,1.000000,1.000000") true false)))

(event EventBeginPlay
  (Utilities|FlowControl|Delay 4.0)
  (Actor|DestroyActor))

(fn ConstructionScript)