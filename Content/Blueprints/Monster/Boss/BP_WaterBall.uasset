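; Reusable boss water-ball projectile that launches toward the player's position when shot, moving along that fixed direction each tick.
; ChangeDir redirects it, marks it friendly and swaps its Niagara effect to red or yellow.
; On overlap, friendly balls damage characters whose mesh is on GameTraceChannel1, while hostile ones damage other characters.
; A hit plays a sound and deactivates the ball at the world origin, resetting its allegiance and effect.
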(event OnComponentBeginOverlap(Sphere1)
  (params (OverlappedComponent :type Primitive%20Component%20Object%20Reference) (OtherActor :type Actor%20Object%20Reference) (OtherComp :type Primitive%20Component%20Object%20Reference) (OtherBodyIndex :type Integer) (bFromSweep :type Boolean) (SweepResult :type Hit%20Result%20Structure%20%28by%20ref%29))
  (bind _ascolorverse_character (Utilities|Casting|CastToColorverseCharacter OtherActor))
  (if (Utilities|Enum|Equal(Enum) (Collision|GetCollisionObjectType (Variables|/Script/Engine.Character|GetMesh _ascolorverse_character)) "ECC_GameTraceChannel1")
    (if (Variables|Default|GetisFriend)
      (Class|ColorverseCharacter|Attacked _ascolorverse_character (Utilities|Struct|MakeDamageMessage self 1e+01 "0.000000,0.000000,0.000000" "0.000000,0.000000,0.000000" "0.000000,0.000000,0.000000"))
      (CallFunction|SetActiveFalse "0, 0, 0")
      (Audio|PlaySoundatLocation "/Game/Sounds/Boss/LastBoss_WaterShot_attacked.LastBoss_WaterShot_attacked" (Transformation|GetActorLocation) "0, 0, 0" 1.0 1.0 0.0 0 0 0 0))
    (elif (not (Variables|Default|GetisFriend))
      (Class|ColorverseCharacter|Attacked _ascolorverse_character (Utilities|Struct|MakeDamageMessage self 1e+01 "0.000000,0.000000,0.000000" "0.000000,0.000000,0.000000" "0.000000,0.000000,0.000000"))
      (CallFunction|SetActiveFalse "0, 0, 0")
      (Audio|PlaySoundatLocation "/Game/Sounds/Boss/LastBoss_WaterShot_attacked.LastBoss_WaterShot_attacked" (Transformation|GetActorLocation) "0, 0, 0" 1.0 1.0 0.0 0 0 0 0))))

(event Custom|shot
  (Audio|PlaySoundatLocation "/Game/Sounds/Boss/BlueBoss__Throw_Watershot.BlueBoss__Throw_Watershot" (Transformation|GetActorLocation) "0, 0, 0" 1.0 1.0 0.0 0 0 0 0)
  (Variables|Default|Setmove true)
  (Variables|Default|SetDir (Math|Vector|GetUnitDirection(Vector) (Transformation|GetActorLocation) (Transformation|GetActorLocation (Game|Player|GetPlayerPawn 0)))))

(event Custom|SetActive
  (params (active :type Boolean) (location :type Vector))
  (Transformation|SetActorLocation location false false)
  (Components|Activation|SetActive (Variables|Default|GetNiagara) active false)
  (Components|Activation|SetActive (Variables|Default|GetSphere1) active false)
  (Variables|Default|Setmove false)
  (Class|NiagaraComponent|SetAsset (Variables|Default|GetNiagara) "/Game/Stylized_VFX_StPack/Particles/UPDATE_1_3/P_Liquid_Projectile_01.P_Liquid_Projectile_01" true))

(event Custom|SetActiveFalse
  (params (NewParam :type Vector))
  (Variables|Default|Setmove false)
  (Variables|Default|SetisFriend false)
  (Class|NiagaraComponent|SetAsset (Variables|Default|GetNiagara) "/Game/Stylized_VFX_StPack/Particles/UPDATE_1_3/P_Liquid_Projectile_01.P_Liquid_Projectile_01" true)
  (CallFunction|SetActive false NewParam))

(event Custom|ChangeDir
  (params (NewParam :type ECombineColors%20Enum :default "Red") (Dir :type Vector))
  (switch Utilities|FlowControl|Switch|SwitchonECombineColors NewParam
    (:Red
      (Variables|Default|SetCurrentColor "Red")
      (Class|NiagaraComponent|SetAsset (Variables|Default|GetNiagara) "/Game/Stylized_VFX_StPack/Particles/UPDATE_1_3/P_Liquid_Projectile_02.P_Liquid_Projectile_02" true))
    (:Yellow
      (Variables|Default|SetCurrentColor "Yellow")
      (Class|NiagaraComponent|SetAsset (Variables|Default|GetNiagara) "/Game/Stylized_VFX_StPack/Particles/UPDATE_1_3/P_Liquid_Projectile_03.P_Liquid_Projectile_03" true)))
  (Variables|Default|SetDir Dir)
  (Variables|Default|SetisFriend true))

(event EventTick
  (params (DeltaSeconds :type Float%20%28single-precision%29))
  (if (Variables|Default|Getmove)
    (Class|SceneComponent|AddWorldTransform (Variables|Default|GetDefaultSceneRoot) (Math|Transform|MakeTransform (* (Variables|Default|GetDir) (Variables|Default|Getspeed)) "0, 0, 0" "1.000000,1.000000,1.000000") true false)))

(fn ConstructionScript)