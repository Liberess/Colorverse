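; BP_CollectObject is an interactable pickup that can be collected into the inventory once it is flagged as separated.
; On BeginPlay it creates dynamic painting and brush material instances, applies the painting one to the mesh, then disables physics simulation after a short delay.
; On interaction, if separated and the inventory manager is valid, it adds its item data to the inventory and destroys itself.
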(event Custom|Interact_1
  (bind _returnvalue (Subsystems|GetInventoryManager))
  (if (Variables|Default|GetbIsSeparated)
    (Utilities|IsValid _returnvalue
      (:Is%20Valid
        (Class|InventoryManager|AddInventoryItem _returnvalue (Variables|Default|GetItemData))
        (Actor|DestroyActor)))))

(event EventBeginPlay
  (|CallParentFunction)
  (bind _returnvalue (Rendering|Material|CreateDynamicMaterialInstance (Variables|Default|GetPaintingMatTemplate) "PaintingMatInst" "None" :!class /Script/Engine.KismetMaterialLibrary))
  (bind _output_get (Variables|Default|SetPaintingMatInst _returnvalue))
  (Rendering|Material|SetMaterial (Variables|Default|GetStaticMesh) 0 _output_get)
  (bind _returnvalue_2 (Rendering|Material|CreateDynamicMaterialInstance (Variables|Default|GetBrushMatTemplate) "BrushMatInst" "None" :!class /Script/Engine.KismetMaterialLibrary))
  (Variables|Default|SetBrushMatInst _returnvalue_2)
  (Utilities|FlowControl|Delay 0.5)
  (Physics|SetSimulatePhysics (Variables|Default|GetStaticMesh) false))

(fn ConstructionScript)