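; AI controller for the slime enemy that feeds sight-based player tracking into its Blackboard.
; On possessed pawn change, it records a HomePos location.
; Perception updates scan sight-perceived actors; a successfully sensed Player-tagged actor becomes Target, sets HasLineOfSight and cancels the loss timer.
; Otherwise a LineOfSightTimer delay starts, after which line of sight and Target are cleared.
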(event OnTargetPerceptionUpdated(AIPerception)
  (params (Actor :type Actor%20Object%20Reference) (Stimulus :type AI%20Stimulus%20Structure))
  (bind _blackboard (Variables|Default|GetBlackboard))
  (bind _array_element (Utilities|Array|ForEachLoopwithBreak (Class|AIPerceptionComponent|GetPerceivedActors (Variables|Default|GetAIPerception) "/Script/AIModule.AISense_Sight") :!label _label)
    (:LoopBody
      (if (and (Actor|ActorHasTag _array_element "Player") (.bSuccessfullySensed (Utilities|Struct|BreakAIStimulus Stimulus)))
        (Utilities|Time|ClearandInvalidateTimerbyHandle (Variables|Default|GetEnemy%20Timer))
        (AI|Components|Blackboard|SetValueasBool _blackboard (Variables|Default|GetHas%20Line%20Of%20Sight) true)
        (AI|Components|Blackboard|SetValueasObject _blackboard (Variables|Default|GetTarget) _array_element)
        (goto _label Break)
        (else
          (bind _returnvalue (Utilities|Time|SetTimerbyEvent (delegate Custom|StartEnemyTimer) (Variables|Default|GetLine%20Of%20Sight%20Timer)))
          (Variables|Default|SetEnemy%20Timer _returnvalue))))))

(event Custom|StartEnemyTimer
  (bind _blackboard (Variables|Default|GetBlackboard))
  (AI|Components|Blackboard|SetValueasBool _blackboard (Variables|Default|GetHas%20Line%20Of%20Sight) false)
  (AI|Components|Blackboard|SetValueasObject _blackboard (Variables|Default|GetTarget) 0))

(event Custom|setHomPos
  (params (OldPawn :type Pawn%20Object%20Reference) (NewPawn :type Pawn%20Object%20Reference))
  (AI|Components|Blackboard|SetValueasVector (Variables|Default|GetBlackboard) (Variables|Default|GetHomePos) (Transformation|GetActorLocation)))

(event EventBeginPlay
  (Pawn|BindEventtoOnPossessedPawnChanged (delegate Custom|setHomPos)))

(fn ConstructionScript)