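; BP_WolfController is the wolf AI controller that turns perception updates into blackboard state for targeting the player.
; Sensing an actor tagged Player cancels the forget timer and sets HasLineOfSight and Target on the blackboard.
; Any other perception update, including losing the player, starts a one-shot LineOfSightTimer delay, after which both keys are cleared.
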(event OnTargetPerceptionUpdated(AIPerception)
  (params (Actor :type Actor%20Object%20Reference) (Stimulus :type AI%20Stimulus%20Structure))
  (bind _blackboard (Variables|Default|GetBlackboard))
  (if (and (Actor|ActorHasTag Actor "Player") (.bSuccessfullySensed (Utilities|Struct|BreakAIStimulus Stimulus)))
    (Utilities|Time|ClearandInvalidateTimerbyHandle (Variables|Default|GetEnemy%20Timer))
    (AI|Components|Blackboard|SetValueasBool _blackboard (Variables|Default|GetHas%20Line%20Of%20Sight) true)
    (AI|Components|Blackboard|SetValueasObject _blackboard (Variables|Default|GetTarget) Actor)
    (else
      (bind _returnvalue (Utilities|Time|SetTimerbyEvent (delegate Custom|StartEnemyTimer) (Variables|Default|GetLine%20Of%20Sight%20Timer)))
      (Variables|Default|SetEnemy%20Timer _returnvalue))))

(event Custom|StartEnemyTimer
  (bind _blackboard (Variables|Default|GetBlackboard))
  (AI|Components|Blackboard|SetValueasBool _blackboard (Variables|Default|GetHas%20Line%20Of%20Sight) false)
  (AI|Components|Blackboard|SetValueasObject _blackboard (Variables|Default|GetTarget) 0))

(event EventBeginPlay)

(fn ConstructionScript)