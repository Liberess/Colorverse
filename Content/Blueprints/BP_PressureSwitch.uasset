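; BP_PressureSwitch is a pressure switch that drives a linked Statue when an actor steps on or off it.
; BoxCol overlaps ignore BP_PuzzleStone and accept any other actor, with a boolean latch preventing repeat triggers.
; Entering calls IncreaseColor on the Statue and plays a timeline that moves the switch mesh on Z.
; Leaving calls DecreaseColor and reverses the timeline, without counting remaining overlapping actors.
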(event OnComponentBeginOverlap(BoxCol)
  (params (OverlappedComponent :type Primitive%20Component%20Object%20Reference) (OtherActor :type Actor%20Object%20Reference) (OtherComp :type Primitive%20Component%20Object%20Reference) (OtherBodyIndex :type Integer) (bFromSweep :type Boolean) (SweepResult :type Hit%20Result%20Structure%20%28by%20ref%29))
  (bind _statue (Variables|Default|GetStatue))
  (Utilities|Casting|CastToBP_PuzzleStone OtherActor
    (:CastFailed
      (if (not (Variables|Default|GetIsAlreadyInteract))
        (Variables|Default|SetIsAlreadyInteract true)
        (Utilities|IsValid _statue
          (:Is%20Valid
            (Class|Statue|IncreaseColor _statue)
            (bind _switchposition (Timeline|SwitchActivate Play)
              (:Update
                (Transformation|SetRelativeLocation (Variables|Default|GetSwitch) (Math|Vector|MakeVector 0.0 0.0 _switchposition) false false)))))))))

(event OnComponentEndOverlap(BoxCol)
  (params (OverlappedComponent :type Primitive%20Component%20Object%20Reference) (OtherActor :type Actor%20Object%20Reference) (OtherComp :type Primitive%20Component%20Object%20Reference) (OtherBodyIndex :type Integer))
  (bind _statue (Variables|Default|GetStatue))
  (Utilities|Casting|CastToBP_PuzzleStone OtherActor
    (:CastFailed
      (if (Variables|Default|GetIsAlreadyInteract)
        (Variables|Default|SetIsAlreadyInteract false)
        (Utilities|IsValid _statue
          (:Is%20Valid
            (Class|Statue|DecreaseColor _statue)
            (bind _switchposition (Timeline|SwitchActivate Reverse)
              (:Update
                (Transformation|SetRelativeLocation (Variables|Default|GetSwitch) (Math|Vector|MakeVector 0.0 0.0 _switchposition) false false)))))))))

(fn ConstructionScript)