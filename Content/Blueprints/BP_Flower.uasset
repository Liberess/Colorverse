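; BP_Flower is an interactable flower pickup that goes into the inventory when used.
; Physics stays off from BeginPlay until Interact, which turns it on, applies a zero-vector impulse and passes ItemData to the InventoryManager.
; The Invisible timeline then drives the root's world scale, and the actor destroys itself when the timeline finishes.
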(event EventBeginPlay
  (|CallParentFunction)
  (Physics|SetSimulatePhysics false))

(event EventInteract
  ;[1 1 1] Interact Event
  (Physics|SetSimulatePhysics true)
  (Physics|AddImpulse "0, 0, 0" "None" false)
  (Class|InventoryManager|AddInventoryItem (Subsystems|GetInventoryManager) (Variables|Default|GetItemData))
  (bind _scale (Timeline|Invisible PlayFromStart)
    (:Update
      (Transformation|SetWorldScale3D (Variables|Default|GetDefaultRoot) _scale))
    (:Finished
      (Actor|DestroyActor))))

(fn ConstructionScript)