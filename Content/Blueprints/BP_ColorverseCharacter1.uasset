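; Player character Blueprint for Colorverse, wielding a brush-sword that fights and paints in the equipped color.
; CombatSystem supplies color, paint amount and attack state, driving the brush material, Niagara trail and hit effects.
; Tick runs sphere traces for drawing on UVs and for damaging or painting hit targets, while anim notifies trigger lunges and paint use.
; Also handles rolling, knockback, death, camera lock-on, interaction outlines, sanctum teleport and cheats.
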(event OnComponentBeginOverlap(CapsuleComponent)
  (params (OverlappedComponent :type Primitive%20Component%20Object%20Reference) (OtherActor :type Actor%20Object%20Reference) (OtherComp :type Primitive%20Component%20Object%20Reference) (OtherBodyIndex :type Integer) (bFromSweep :type Boolean) (SweepResult :type Hit%20Result%20Structure%20%28by%20ref%29))
  ;[1 1 1] Interact Outline
  (Utilities|Casting|CastToBP_ball OtherActor
    (:CastFailed
      (CallFunction|SetInteractOutline OtherActor true))))

(event OnComponentEndOverlap(CapsuleComponent)
  (params (OverlappedComponent :type Primitive%20Component%20Object%20Reference) (OtherActor :type Actor%20Object%20Reference) (OtherComp :type Primitive%20Component%20Object%20Reference) (OtherBodyIndex :type Integer))
  ;[1 1 1] Interact Outline
  (Utilities|Casting|CastToBP_ball OtherActor
    (:CastFailed
      (CallFunction|SetInteractOutline OtherActor false))))

(event Custom|OnEndDamaged_이벤트
  ;[1 1 1] 애님노티파이 - EndDamaged
  (Variables|Default|SetbIsAttacked false))

(event Custom|Launch
  (if (not (AI|Components|NavMovement|IsFalling (Variables|Character|GetCharacterMovement)))
    (bind _output_get (Variables|Default|SetCurLot (Transformation|GetWorldLocation (Variables|Default|GetCapsuleComponent))))
    (bind _새_트랙_0 (Timeline|타임라인 PlayFromStart)
      (:Update
        (Transformation|SetWorldLocation (Variables|Default|GetCapsuleComponent) (+ _output_get (* (Math|Vector|GetForwardVector (Variables|Default|GetCapsuleComponent)) _새_트랙_0)) true false)))))

(event Custom|DisablePaintEffect
  (bind _niagara (Variables|Default|GetNiagara))
  ;[1 1 1] 애님노티파이 - Next Attack Check
  (Rendering|SetVisibility _niagara false false)
  (Niagara|ResetSystem _niagara))

(event Custom|UsePaint
  ;[1 1 1] 애님노티파이 - End Attack Trace
  (if (Variables|/Script/Colorverse.CombatSystem|GetbIsOnColor (Variables|Default|GetCombatSystem))
    (Class|CombatSystem|SetCurrentPaintColorAmount (Variables|Default|GetCombatSystem) -5.0)))

(event EventCheatStanctumBlue
  ;[1 1 1] Cheat Stanctums
  (bind _outactors (Actor|GetAllActorsOfClass "/Game/Blueprints/Puzzle/BP_BossDoor.BP_BossDoor_C"))
  (bind _array_element (Utilities|Array|ForEachLoopwithBreak _outactors :!label _label)
    (:LoopBody
      (if (Utilities|Enum|Equal(Enum) (Variables|/Game/Blueprints/Puzzle/BP_BossDoor.BP_BossDoor_C|GetPuzzleTag _array_element) "Puzzle_Blue")
        (Default|IncreaseCount _array_element)
        (Default|IncreaseCount _array_element)
        (Default|IncreaseCount _array_element)
        (goto _label Break)))))

(event EventBeginPlay
  ;[1 1 1] BeginPlay
  (|CallParentFunction)
  (Utilities|FlowControl|Sequence
    (:then_0
      (bind _ascolorverse_character_anim_instance (Utilities|Casting|CastToColorverseCharacterAnimInstance (Components|SkeletalMesh|GetAnimInstance (Variables|Character|GetMesh))))
      (bind _output_get (Variables|Default|SetColorverseAnim _ascolorverse_character_anim_instance))
      ;[1 1 1] 애님노티파이 - EndDamaged
      (EventDispatchers|AssignOnEndDamaged _output_get (delegate Custom|OnEndDamaged_이벤트))
      (EventDispatchers|BindEventtoOnStartAttackJudg _output_get (delegate Custom|Launch))
      ;[1 1 1] 애님노티파이 - End Attack Trace
      (EventDispatchers|BindEventtoOnEndAttackJudg _output_get (delegate Custom|UsePaint))
      ;[1 1 1] 애님노티파이 - Next Attack Check
      (EventDispatchers|BindEventtoOnNextAttackCheck _output_get (delegate Custom|DisablePaintEffect)))
    (:then_1
      ;[1 1 1] 이펙트 설정
      (Rendering|SetVisibility (Variables|Default|GetNiagara) false false)
      (bind _returnvalue (Class|CombatSystem|GetCurrentPaintLinearColor (Variables|Default|GetCombatSystem)))
      (Rendering|Material|SetVectorParameterValue (Variables|Default|GetBrushPaint) "Color" _returnvalue :!class /Script/Engine.MaterialInstanceDynamic))))

(event EventOnJumped
  ;[1 1 1] On Jumped
  (|CallParentFunction)
  (Class|ColorverseCharacter|SetDisabledAttack))

(event EventRoll
  ;[1 1 1] 구르기 이벤트
  (|CallParentFunction)
  (if (not (Math|Boolean|ORBoolean (not (Variables|/Script/Colorverse.CombatSystem|GetbIsCanInput (Variables|Default|GetCombatSystem))) (Variables|Default|GetbIsAttacked) (Variables|Default|GetbIsRolling) (AI|Components|NavMovement|IsFalling (Variables|Character|GetCharacterMovement))))
    (Class|ColorverseCharacter|SetDisabledAttack)
    (Variables|Default|SetbIsRolling true)
    (Animation|Montage|MontagePlay (Components|SkeletalMesh|GetAnimInstance (Variables|Character|GetMesh)) "/Game/Animation/RTG_Animations/Sprinting_Forward_Roll_Anim_mixamo_com_Montage.Sprinting_Forward_Roll_Anim_mixamo_com_Montage" 1.0 "MontageLength" 0.0 true)
    (Variables|Default|SetRollRot (Transformation|GetActorForwardVector))))

(event EventCheatInventory
  ;[1 1 1] Cheat - Inventory
  (if (<= (Utilities|Array|Length (Variables|Default|GetResourceItems)) 0)
    (bind _outrownames (DataTable|GetDataTableRowNames "/Game/DataTables/DT_ItemData.DT_ItemData"))
    (for (_array_element _array_index) _outrownames
      (bind _returnvalue (Utilities|GetDataTableRow "/Game/DataTables/DT_ItemData.DT_ItemData" _array_element)
        (:then
          (if (not (Utilities|Enum|Equal(Enum) (.CombineType (Utilities|Struct|BreakItem _returnvalue)) "None"))
            (bind _structout (Utilities|Struct|SetmembersinItem _returnvalue 10))
            (Utilities|Array|SetArrayElem (Variables|Default|GetResourceItems) _array_index _structout true))))))
  (for _array_element_2 (Variables|Default|GetResourceItems)
    (Class|InventoryManager|AddInventoryItem (Subsystems|GetInventoryManager) _array_element_2 false)))

(event EventCheatStanctumRed
  ;[1 1 1] Cheat Stanctums
  (bind _outactors (Actor|GetAllActorsOfClass "/Game/Blueprints/Puzzle/BP_BossDoor.BP_BossDoor_C"))
  (bind _array_element (Utilities|Array|ForEachLoopwithBreak _outactors :!label _label)
    (:LoopBody
      (if (Utilities|Enum|Equal(Enum) (Variables|/Game/Blueprints/Puzzle/BP_BossDoor.BP_BossDoor_C|GetPuzzleTag _array_element) "Puzzle_Red")
        (Default|IncreaseCount _array_element)
        (Default|IncreaseCount _array_element)
        (Default|IncreaseCount _array_element)
        (goto _label Break)))))

(event EventCheatStanctumYellow
  ;[1 1 1] Cheat Stanctums
  (bind _outactors (Actor|GetAllActorsOfClass "/Game/Blueprints/Puzzle/BP_BossDoor.BP_BossDoor_C"))
  (bind _array_element (Utilities|Array|ForEachLoopwithBreak _outactors :!label _label)
    (:LoopBody
      (if (Utilities|Enum|Equal(Enum) (Variables|/Game/Blueprints/Puzzle/BP_BossDoor.BP_BossDoor_C|GetPuzzleTag _array_element) "Puzzle_Yellow")
        (Default|IncreaseCount _array_element)
        (Default|IncreaseCount _array_element)
        (Default|IncreaseCount _array_element)
        (goto _label Break)))))

(event EventChangeEquipPaint
  (params (CombineColor :type ECombineColors%20Enum :default "Red"))
  (bind _combatsystem (Variables|Default|GetCombatSystem))
  (bind _sword (Variables|Default|Getsword))
  (bind _returnvalue (Transformation|GetAllSocketNames _sword))
  (bind _output (Utilities|Array|Get(acopy) _returnvalue))
  ;[1 1 1] 장착 색 변경 이벤트
  (if (and (not (== CombineColor (Math|Conversions|ToInteger(Byte) (Variables|/Script/Colorverse.CombatSystem|GetCurrentPaintColor (Variables|Default|GetCombatSystem))))) (Variables|/Script/Colorverse.CombatSystem|GetbIsCanInput (Variables|Default|GetCombatSystem)))
    (bind _returnvalue_2 (Class|CombatSystem|GetCurrentPaintColorAmount _combatsystem))
    (if (not (and (<= _returnvalue_2 0.0) (Utilities|Enum|Equal(Enum) (Variables|/Script/Colorverse.CombatSystem|GetCurrentPaintColor _combatsystem) "Empty")))
      (|CallParentFunction CombineColor)
      ;;[1 1 1] 붓 페인트 메터리얼 변경
      (bind _returnvalue_3 (Class|CombatSystem|GetCurrentPaintLinearColor (Variables|Default|GetCombatSystem)))
      (Rendering|Material|SetVectorParameterValue (Variables|Default|GetBrushPaint) "Color" _returnvalue_3 :!class /Script/Engine.MaterialInstanceDynamic)
      (CallFunction|ChangePaintColor (Transformation|GetSocketLocation _sword _output) (Transformation|GetSocketRotation _sword _output))
      (CallFunction|PaintEffect))))

(event EventTick
  (params (DeltaSeconds :type Float%20%28single-precision%29))
  (bind _sword (Variables|Default|Getsword))
  (bind _combatsystem (Variables|Default|GetCombatSystem))
  (bind _niagara (Variables|Default|GetNiagara))
  ;[1 1 1] Tick
  (|CallParentFunction DeltaSeconds)
  (Utilities|FlowControl|Sequence
    (:then_0
      ;[1 1 1] Painting
      (if (Variables|Default|GetIsDrawing)
        (bind (_outhits _returnvalue) (Collision|MultiSphereTraceByChannel (Transformation|GetActorLocation) (Transformation|GetSocketLocation _sword (Utilities|Array|Get(acopy) (Transformation|GetAllSocketNames _sword) 1)) 3e+01 "TraceTypeQuery1" true 0 "None" true "(R=1.000000,G=0.000000,B=0.000000,A=1.000000)" "(R=0.000000,G=1.000000,B=0.000000,A=1.000000)" 2.0))
        (for _array_element _outhits
          (bind _aspainted_collect_object (Utilities|Casting|CastToPaintedCollectObject (.HitActor (Collision|BreakHitResult _array_element))))
          (bind _output_get (Variables|Default|SetCurrentPaintedCollectObj _aspainted_collect_object))
          (Class|PaintedCollectObject|DrawonWhiteBoard _output_get (.UV (Class|GameplayStatics|FindCollisionUV _array_element)) (and (.ReturnValue (Class|GameplayStatics|FindCollisionUV _array_element)) _returnvalue) (CallFunction|GetCurrentBrushColor)))))
    (:then_1
      ;[1 1 1] Hit Check
      (if (Variables|/Script/Colorverse.CombatSystem|GetbIsCanAttackTrace (Variables|Default|GetCombatSystem))
        (Class|ColorverseCharacter|HitCheck)))
    (:then_2
      ;[1 1 1] 색 버프 설정
      (Class|CombatSystem|SetColorBuff _combatsystem)
      (bind _returnvalue_2 (Class|CombatSystem|GetCurrentPaintColorAmount _combatsystem))
      (if (not (> _returnvalue_2 0.0))
        (Class|ColorverseCharacter|ChangeEquipPaint "Empty")
        (CallFunction|PaintEffect)))
    (:then_3
      ;[1 1 1] 나이아가라 위치 설정
      (if (Utilities|IsValid _niagara)
        (Effects|Components|ParticleSystem|SetVectorParameter _niagara "User.Position" (Transformation|GetSocketLocation (Variables|Default|Getsword) "Socket1"))))
    (:then_4
      ;[1 1 1] 붓 위치 설정
      (if (Variables|Default|GetbIsAttacking)
        (Transformation|AttachComponentToComponent (Variables|Default|Getsword) (Variables|Character|GetMesh) "sword" "KeepRelative" "KeepRelative" "KeepRelative" true)
        (else
          (Transformation|AttachComponentToComponent (Variables|Default|Getsword) (Variables|Character|GetMesh) "Brush" "KeepRelative" "KeepRelative" "KeepRelative" true))))
    (:then_5
      (if (Variables|Default|GetbIsRolling)
        (Pawn|Input|AddMovementInput (Variables|Default|GetRollRot) 1.0 false)))))

(event EventTeleportStanctumRed
  (params (Rate :type Float%20%28single-precision%29))
  (if (>= Rate 2.0)
    (bind _outactors (Actor|GetAllActorsOfClass "/Game/Blueprints/BP_TeleportPoint.BP_TeleportPoint_C"))
    (bind _array_element (Utilities|Array|ForEachLoopwithBreak _outactors :!label _label)
      (:LoopBody
        (if (Utilities|Enum|Equal(Enum) (Variables|/Game/Blueprints/BP_TeleportPoint.BP_TeleportPoint_C|GetPointTag _array_element) "NewEnumerator0")
          (Transformation|SetActorLocation (Transformation|GetActorLocation _array_element) false false)
          (goto _label Break))))))

(event EventSetDisabledRoll
  ;[1 1 1] 구르기 End 이벤트
  (Variables|Default|SetbIsRolling false)
  (Collision|SetCollisionEnabled (Variables|Character|GetMesh) "QueryAndPhysics"))

(event Input|ActionEvents|InputActionCameraLockOn
  (params (Key :type Key%20Structure :default "None"))
  (bind _returnvalue (Transformation|GetActorLocation))
  (bind _returnvalue_2 (Pawn|GetController))
  (bind _returnvalue_3 (Transformation|GetActorLocation))
  (bind _followcamera (Variables|Default|GetFollowCamera))
  (bind _returnvalue_4 (Transformation|GetActorRotation _returnvalue_2))
  (bind _returnvalue_5 (Math|Vector|GetForwardVector _followcamera))
  (bind _returnvalue_6 (* _returnvalue_5 5e+02))
  (bind _returnvalue_7 (+ _returnvalue_6 _returnvalue_3))
  ;[1 1 1] 시점 고정
  (:Pressed
    ;;[1 1 1] Check Range
    (bind (_outhits _returnvalue_8) (Collision|MultiSphereTraceForObjects _returnvalue_7 _returnvalue_7 (Variables|Default|GetAttack%20Range) (Variables|Default|GetObject%20Types) false 0 "None"))
    (if _returnvalue_8
      (Variables|Default|SetLock%20on%20Target (.HitActor (Collision|BreakHitResult (Utilities|Array|Get(acopy) _outhits))))
      ;;[1 1 1] Find Most Near
      (for _array_element _outhits
        (if (< (Math|Vector|Distance(Vector) (Transformation|GetActorLocation (.HitActor (Collision|BreakHitResult _array_element))) _returnvalue) (Math|Vector|Distance(Vector) _returnvalue (Transformation|GetActorLocation (Variables|Default|GetLock%20on%20Target))))
          (Variables|Default|SetLock%20on%20Target (.HitActor (Collision|BreakHitResult _array_element)))))
      ;;[1 1 1] Set Camera Rotation
      (Pawn|SetControlRotation _returnvalue_2 (Math|Rotator|MakeRotator (.Roll (Math|Rotator|BreakRotator _returnvalue_4)) (.pitch (Math|Interpolation|RInterpTo _returnvalue_4 (Math|Rotator|FindLookatRotation (Transformation|GetActorLocation) (Math|Vector|MakeVector (.x (Transformation|GetActorLocation (Variables|Default|GetLock%20on%20Target))) (.y (Transformation|GetActorLocation (Variables|Default|GetLock%20on%20Target))) (- (.z (Transformation|GetActorLocation (Variables|Default|GetLock%20on%20Target))) 1.5e+02))) (Utilities|Time|GetWorldDeltaSeconds) 0.0)) (.yaw (Math|Interpolation|RInterpTo _returnvalue_4 (Math|Rotator|FindLookatRotation (Transformation|GetActorLocation) (Math|Vector|MakeVector (.x (Transformation|GetActorLocation (Variables|Default|GetLock%20on%20Target))) (.y (Transformation|GetActorLocation (Variables|Default|GetLock%20on%20Target))) (- (.z (Transformation|GetActorLocation (Variables|Default|GetLock%20on%20Target))) 1.5e+02))) (Utilities|Time|GetWorldDeltaSeconds) 0.0)))))))

(event Custom|Attack%20Effect
  (params (Pos :type Vector) (Rot :type Rotator))
  (bind _combatsystem (Variables|Default|GetCombatSystem))
  ;[1 1 1] 붓 공격 이펙트
  (if (and (Variables|/Script/Colorverse.CombatSystem|GetbIsOnColor _combatsystem) (!= (Variables|/Script/Colorverse.CombatSystem|GetCurrentPaintColor _combatsystem) 3))
    (Niagara|SpawnSystematLocation (Utilities|Array|Get(acopy) (Variables|Default|GetAttackEffects) (Math|Conversions|ToInteger(Byte) (Variables|/Script/Colorverse.CombatSystem|GetCurrentPaintColor (Variables|Default|GetCombatSystem)))) Pos Rot)
    (else
      (Niagara|SpawnSystematLocation "/Game/Stylized_VFX_StPack/Particles/UPDATE_1_2/P_Classic_Hit_01.P_Classic_Hit_01" Pos Rot))))

(event Custom|PaintEffect
  (bind _combatsystem (Variables|Default|GetCombatSystem))
  ;[1 1 1] 붓 trail 이펙트 설정
  (if (Variables|/Script/Colorverse.CombatSystem|GetbIsOnColor (Variables|Default|GetCombatSystem))
    (bind _returnvalue (Class|CombatSystem|GetCurrentPaintLinearColorbyEnum _combatsystem (Variables|/Script/Colorverse.CombatSystem|GetCurrentPaintColor _combatsystem)))
    (Effects|Components|ParticleSystem|SetColorParameter (Variables|Default|GetNiagara) "User.Color" _returnvalue)
    (else
      (Rendering|SetVisibility (Variables|Default|GetNiagara) false false))))

(event Custom|ChangePaintColor
  (params (NewParam :type Vector) (NewParam2 :type Rotator))
  (bind _combatsystem (Variables|Default|GetCombatSystem))
  (bind _combatsystem_2 (Variables|Default|GetCombatSystem))
  ;[1 1 1] 붓 색 변경 이펙트
  (if (and (Variables|/Script/Colorverse.CombatSystem|GetbIsOnColor _combatsystem_2) (!= (Variables|/Script/Colorverse.CombatSystem|GetCurrentPaintColor _combatsystem_2) 3))
    (bind _returnvalue (Niagara|SpawnSystematLocation (Variables|Default|GetChangeEffects) NewParam NewParam2))
    (bind _returnvalue_2 (Class|CombatSystem|GetCurrentPaintLinearColorbyEnum _combatsystem (Variables|/Script/Colorverse.CombatSystem|GetCurrentPaintColor _combatsystem)))
    (Effects|Components|ParticleSystem|SetColorParameter _returnvalue "color" _returnvalue_2)
    (else
      (Niagara|SpawnSystematLocation "/Game/Stylized_VFX_StPack/Particles/UPDATE_1_2/P_Ice_Hit_01.P_Ice_Hit_01" NewParam NewParam2))))

(event Custom|Destroy
  ;[1 1 1] Destroy Event
  (bind _returnvalue (UserInterface|CreateWidget "/Game/UI/BP_GameOver.BP_GameOver_C"))
  (UserInterface|Viewport|AddtoViewport _returnvalue 0)
  (Actor|DestroyActor))

(event Custom|무적
  ;[1 1 1] 무적 이벤트
  (Collision|SetCollisionEnabled (Variables|Character|GetMesh) "NoCollision"))

(event EventSetDisabledAttack
  (bind _niagara (Variables|Default|GetNiagara))
  ;[1 1 1] Attack End Event
  (|CallParentFunction)
  (Rendering|SetVisibility _niagara false false)
  (Niagara|ResetSystem _niagara)
  (Animation|StopAnimMontage "/Game/Animation/RTG_Animations/PrimaryAttack_Slow_Montage.PrimaryAttack_Slow_Montage"))

(event EventInteract
  ;[1 1 1] Interact Event
  (|CallParentFunction)
  (for _array_element (Collision|GetOverlappingActors "/Script/Colorverse.NPC" :!class /Script/Engine.Actor)
    (if (Utilities|DoesObjectImplementInterface _array_element "/Script/Colorverse.IDialogue")
      (Class|IDialogue|OnBeginTalk(Message) _array_element))))

(event EventSetVisibleInteractableOutline
  (params (Visible :type Boolean))
  ;[1 1 1] Set Visible Interactable Outline Event
  (if Visible
    (Default|CallVisibleInteractOutline)
    (else
      (Default|CallInvisibleInteractOutline))))

(event EventDead
  ;[1 1 1] Dead Event
  (|CallParentFunction)
  (Animation|Montage|MontagePlay (Components|SkeletalMesh|GetAnimInstance (Variables|Character|GetMesh)) "/Game/Animation/Hit_Death/ANI_Player_Death_02_Montage.ANI_Player_Death_02_Montage" 1.0 "MontageLength" 0.0 true))

(event EventAttack
  (params (skillNum :type Integer))
  ;[1 1 1] Attack Event
  (|CallParentFunction 0)
  (if (not (or (Variables|Default|GetbIsAttacked) (Variables|Default|GetbIsRolling)))
    (CallFunction|PaintEffect)
    (if (Variables|/Script/Colorverse.CombatSystem|GetbIsOnColor (Variables|Default|GetCombatSystem))
      (Rendering|SetVisibility (Variables|Default|GetNiagara) true false))))

(event EventHitCheck
  (bind _combatsystem (Variables|Default|GetCombatSystem))
  (bind _sword (Variables|Default|Getsword))
  ;[1 1 1] Hit Event
  (bind (_outhits _returnvalue) (Collision|MultiSphereTraceForObjects (Transformation|GetActorLocation) (Transformation|GetSocketLocation _sword (Utilities|Array|Get(acopy) (Transformation|GetAllSocketNames _sword))) 5e+01 (Variables|Default|GetObject%20Types) false 0 "None" true "(R=1.000000,G=0.000000,B=0.000000,A=1.000000)" "(R=0.000000,G=1.000000,B=0.000000,A=1.000000)" 3.0))
  (if _returnvalue
    (for _array_element _outhits
      (if (== (Utilities|Array|FindItem (Variables|Default|GetAttackHitResults) (.HitActor (Collision|BreakHitResult _array_element))) -1)
        (Utilities|Array|AddUnique (Variables|Default|GetAttackHitResults) (.HitActor (Collision|BreakHitResult _array_element)))
        (Utilities|FlowControl|Sequence
          (:then_0
            (bind _ascolorverse_character (Utilities|Casting|CastToColorverseCharacter (.HitActor (Collision|BreakHitResult _array_element))))
            (bind _returnvalue_2 (Class|CombatSystem|GetCurrentATK (Variables|Default|GetCombatSystem)))
            (Class|ColorverseCharacter|Attacked _ascolorverse_character (Utilities|Struct|MakeDamageMessage self _returnvalue_2 (.ImpactPoint (Collision|BreakHitResult _array_element)) (.ImpactNormal (Collision|BreakHitResult _array_element)) "0.000000,0.000000,0.000000"))
            (Game|Feedback|ClientStartCameraShake (Game|GetPlayerController 0) "/Game/Blueprints/CameraShake_Attack.CameraShake_Attack_C" 1.0 "CameraLocal" "0, 0, 0")
            (CallFunction|AttackEffect (.ImpactPoint (Collision|BreakHitResult _array_element)) (Math|Conversions|RotationFromXVector (.ImpactNormal (Collision|BreakHitResult _array_element)))))
          (:then_1
            ;;[1 1 1] Paint To Object
            (bind _returnvalue_3 (Class|CombatSystem|GetCurrentPaintColorAmount _combatsystem))
            (if (>= _returnvalue_3 5.0)
              (bind _aspainted_collect_object (Utilities|Casting|CastToPaintedCollectObject (.HitActor (Collision|BreakHitResult _array_element))))
              (Class|PaintedCollectObject|PainttoObject _aspainted_collect_object (Variables|/Script/Colorverse.CombatSystem|GetCurrentPaintColor _combatsystem) (CallFunction|GetCurrentBrushColor))
              (Class|CombatSystem|SetCurrentPaintColorAmount (Variables|Default|GetCombatSystem) -5.0)))
          (:then_2
            (bind _aspaintable_object (Utilities|Casting|CastToPaintableObject (.HitActor (Collision|BreakHitResult _array_element))))
            (Class|PaintableObject|PainttoObject _aspaintable_object (CallFunction|GetCurrentBrushColor) (Variables|/Script/Colorverse.CombatSystem|GetCurrentPaintColor (Variables|Default|GetCombatSystem)))))))))

(event EventAttacked
  (params (damageMessage :type Damage%20Message%20Structure))
  (bind _returnvalue (Transformation|GetActorLocation (.damager damageMessage)))
  (bind _returnvalue_2 (Transformation|GetActorLocation))
  (bind (_x _y _z) (Math|Vector|BreakVector (.hitimpact damageMessage)))
  (bind _returnvalue_3 (Math|Vector|GetUnitDirection(Vector) _returnvalue _returnvalue_2))
  (bind (_x_2 _y_2) (Math|Vector|BreakVector _returnvalue_3))
  ;[1 1 1] Damaged Event
  (|CallParentFunction (Utilities|Struct|MakeDamageMessage (.damager damageMessage) (.damageamount damageMessage) (.hitpoint damageMessage) (.hitnormal damageMessage) (.hitimpact damageMessage)))
  (Utilities|FlowControl|Sequence
    (:then_0
      (Variables|Default|SetbIsAttacked true)
      (Class|ColorverseCharacter|SetDisabledAttack)
      (Variables|Default|SetbIsRolling false))
    (:then_1
      (Utilities|Casting|CastToColorverseMonster_middle (.damager damageMessage)
        (:then
          _)
        (:CastFailed
          (Utilities|Casting|CastToBP_PuzzleGolem (.damager damageMessage))))
      (Animation|Montage|MontageStop (Components|SkeletalMesh|GetAnimInstance (Variables|Character|GetMesh)) 0.0 "/Game/Animation/Hit_Death/ANI_Player_Hit_02_Montage.ANI_Player_Hit_02_Montage")
      (bind _ascolorverse_character_anim_bp (Utilities|Casting|CastToColorverseCharacter_AnimBP (Components|SkeletalMesh|GetAnimInstance (Variables|Character|GetMesh))))
      (Variables|/Game/Animations/ColorverseCharacter_AnimBP.ColorverseCharacter_AnimBP_C|SetIsStrongAttacked _ascolorverse_character_anim_bp true))
    (:then_2
      (Character|LaunchCharacter (Math|Vector|MakeVector (* _x_2 _x) (* _y_2 _y) _z) true true)
      (Game|Feedback|ClientStartCameraShake (Game|GetPlayerController 0) "/Game/Blueprints/CameraShake_Attack.CameraShake_Attack_C" 2.0 "CameraLocal" "0, 0, 0"))))

(fn ConstructionScript
  (bind _returnvalue (Rendering|Material|CreateDynamicMaterialInstance (Variables|Default|Getsword) 1 "/Game/Models/new/M_Paint_Inst.M_Paint_Inst" "None" :!class /Script/Engine.PrimitiveComponent))
  (Variables|Default|SetBrushPaint _returnvalue))

(fn GetCurrentBrushColor
  (bind _returnvalue (Class|CombatSystem|GetCurrentPaintLinearColor (Variables|Default|GetCombatSystem)))
  (return _returnvalue))

(fn MouseInput
  (bind _returnvalue (Game|GetPlayerController 0))
  (if (Variables|Default|GetMouseVisibility)
    (Variables|/Script/Engine.PlayerController|SetbShowMouseCursor _returnvalue false)
    (Input|SetInputModeGameOnly _returnvalue false)
    (Variables|Default|SetMouseVisibility false)
    (else
      (Variables|/Script/Engine.PlayerController|SetbShowMouseCursor _returnvalue true)
      (Input|SetInputModeGameandUI _returnvalue 0 "DoNotLock" true false)
      (Variables|Default|SetMouseVisibility true))))

(fn DrawPaintParticle
  (bind _sword (Variables|Default|Getsword))
  (Effects|SpawnEmitteratLocation "/Game/Effects/P_PaintSystem.P_PaintSystem" (+ (Transformation|GetSocketLocation _sword (Utilities|Array|Get(acopy) (Transformation|GetAllSocketNames _sword) 1)) (* (Math|Vector|GetForwardVector (Variables|Default|GetFollowCamera)) 1e+02)) (Transformation|GetWorldRotation (Variables|Default|GetFollowCamera))))

(fn SetInteractOutline
  (params (Actor :type Actor%20Object%20Reference) (Visible :type Boolean))
  (bind _returnvalue (Actor|GetComponentbyClass Actor "/Script/Engine.StaticMeshComponent"))
  (Utilities|IsValid _returnvalue
    (:Is%20Valid
      (if (Variables|/Script/Engine.PrimitiveComponent|GetbRenderCustomDepth _returnvalue)
        (if Visible
          (Rendering|SetCustomDepthStencilValue _returnvalue 1)
          (Class|ColorverseCharacter|SetVisibleInteractableOutline true)
          (else
            (Rendering|SetCustomDepthStencilValue _returnvalue 0)
            (Class|ColorverseCharacter|SetVisibleInteractableOutline false)))))))