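; Red slime enemy Blueprint that lunges at player characters, gets knocked back when hit, and drops an item when destroyed.
; It extends parent combat events and sets blackboard flags for attack cooldown and damage, with anim instance delegates triggering the cooldown and clearing the damaged state.
; HitCheck sphere-traces at a mesh socket, damaging each newly hit character using CombatSystem attack power.
; Death plays a montage, while Destroy spawns explosion VFX and the drop.
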(event Custom|CoolTime
  ;[1 1 1] 애님 노티파이 이벤트
  (AI|Components|Blackboard|SetValueasBool (AI|GetBlackboard (Pawn|GetController)) (Variables|Default|GetCoolTimeKey) true)
  (Utilities|FlowControl|Delay (Variables|Default|GetAttackCoolTime))
  (AI|Components|Blackboard|SetValueasBool (AI|GetBlackboard (Pawn|GetController)) (Variables|Default|GetCoolTimeKey) false))

(event Custom|OnEndDamaged_이벤트
  ;[1 1 1] 애님 노티파이 이벤트
  (Variables|Default|SetbIsAttacked false)
  (AI|Components|Blackboard|SetValueasBool (AI|GetBlackboard (Pawn|GetController)) (Variables|Default|GetDamaged) false))

(event Custom|Destroy
  (bind _returnvalue (Transformation|GetActorTransform))
  ;[1 1 1] 죽음
  (Niagara|SpawnSystematLocation "/Game/BloodFX/FX/NS_BloodExplodeBig.NS_BloodExplodeBig" (.location _returnvalue) (.rotation _returnvalue))
  (Utilities|FlowControl|Delay 0.5)
  ;;[1 1 1] 몬스터 부산물 생성
  (Game|SpawnActorfromClass "/Game/Blueprints/BP_DropItem.BP_DropItem_C" (Transformation|GetActorTransform) "AlwaysSpawn" 0 0)
  (Actor|DestroyActor))

(event EventHitCheck
  (bind _mesh (Variables|Character|GetMesh))
  (bind _returnvalue (Transformation|GetSocketLocation _mesh "Bip001"))
  ;[1 1 1] Hit Check
  (bind (_outhits _returnvalue_2) (Collision|MultiSphereTraceForObjects _returnvalue _returnvalue 1e+02 (Variables|Default|GetObject%20Types) false 0 "None"))
  (if _returnvalue_2
    (for _array_element _outhits
      (if (== (Utilities|Array|FindItem (Variables|Default|GetAttackHitResults) (.HitActor (Collision|BreakHitResult _array_element))) -1)
        (Utilities|Array|AddUnique (Variables|Default|GetAttackHitResults) (.HitActor (Collision|BreakHitResult _array_element)))
        (bind _ascolorverse_character (Utilities|Casting|CastToColorverseCharacter (.HitActor (Collision|BreakHitResult _array_element))))
        (bind _returnvalue_3 (Class|CombatSystem|GetCurrentATK (Variables|Default|GetCombatSystem)))
        (Class|ColorverseCharacter|Attacked _ascolorverse_character (Utilities|Struct|MakeDamageMessage self _returnvalue_3 (.ImpactPoint (Collision|BreakHitResult _array_element)) (.ImpactNormal (Collision|BreakHitResult _array_element))))
        (Niagara|SpawnSystematLocation "/Game/Stylized_VFX_StPack/Particles/UPDATE_1_3/P_Web_Hit_01.P_Web_Hit_01" (+ (Transformation|GetActorLocation) (* (Math|Vector|GetForwardVector (Variables|Default|GetFollowCamera)) 2e+02)) (Transformation|GetActorRotation))))))

(event EventAttacked
  (params (damageMessage :type Damage%20Message%20Structure))
  (bind _rootcomponent (Variables|/Script/Engine.Actor|GetRootComponent (.damager damageMessage)))
  (bind _returnvalue (Math|Vector|GetForwardVector _rootcomponent))
  ;[1 1 1] Hit Event
  (|CallParentFunction (Utilities|Struct|MakeDamageMessage (.damager damageMessage) (.damageamount damageMessage) (.hitpoint damageMessage) (.hitnormal damageMessage)))
  (AI|Components|Blackboard|SetValueasBool (AI|GetBlackboard (Pawn|GetController)) (Variables|Default|GetDamaged) true)
  (Class|ColorverseCharacter|SetDisabledAttack)
  (Character|LaunchCharacter (Math|Vector|MakeVector (* (.x _returnvalue) 5e+02) (* (.y _returnvalue) 5e+02) 0.0) true true)
  (Audio|PlaySoundatLocation "/Game/Sounds/Slime_Damaged.Slime_Damaged" (Transformation|GetActorLocation) "0, 0, 0" 1.0 1.0 0.0 0 0 0 0))

(event EventDead
  ;[1 1 1] 죽음
  (|CallParentFunction)
  (Animation|Montage|MontagePlay (Components|SkeletalMesh|GetAnimInstance (Variables|Character|GetMesh)) "/Game/Mannequin/Slime/Animations/Anim_ma060_Die_Montage.Anim_ma060_Die_Montage" 1.0 "MontageLength" 0.0 true))

(event EventAttack
  (bind _capsulecomponent (Variables|Default|GetCapsuleComponent))
  (bind _returnvalue (Math|Vector|GetForwardVector _capsulecomponent))
  ;[1 1 1] 공격
  (|CallParentFunction)
  (Character|LaunchCharacter (Math|Vector|MakeVector (* (.x _returnvalue) 8e+02) (* (.y _returnvalue) 8e+02) 3e+02) true true))

(event EventBeginPlay
  ;[1 1 1] BeginPlay
  (|CallParentFunction)
  ;[1 1 1] 애님 노티파이 이벤트
  (bind _ascolorverse_character_anim_instance (Utilities|Casting|CastToColorverseCharacterAnimInstance (Components|SkeletalMesh|GetAnimInstance (Variables|Character|GetMesh))))
  (Utilities|FlowControl|Sequence
    (:then_0
      (EventDispatchers|BindEventtoOnEndAttack _ascolorverse_character_anim_instance (delegate Custom|CoolTime)))
    (:then_1
      (EventDispatchers|AssignOnEndDamaged _ascolorverse_character_anim_instance (delegate Custom|OnEndDamaged_이벤트)))))

(fn ConstructionScript)