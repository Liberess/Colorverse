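; Puzzle stone that the player paints, summoning a matching golem to destroy it once it holds the right color.
; PaintToStone blends the target color halfway toward each paint, uses the full color from three coats, and resets on Empty paint.
; Tick eases a dynamic material's overlay to the target, then calls GoDestroyStone on golems with matching ID and color.
; Damage from a golem spawns smoke and destroys the stone.
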(event Custom|PaintToStone
  (params (PaintColor :type Linear%20Color%20Structure))
  (bind (_r _g _b) (Utilities|Struct|BreakLinearColor PaintColor))
  ;[1 1 1] Check Painted Color
  (bind _asbp_colorverse_character (Utilities|Casting|CastToBP_ColorverseCharacter (Game|GetPlayerCharacter 0)))
  (Utilities|IsValid _asbp_colorverse_character
    (:Is%20Valid
      (if (Utilities|Enum|Equal(Enum) (Variables|/Script/Colorverse.CombatSystem|GetCurrentPaintColor (Variables|/Script/Colorverse.ColorverseCharacter|GetCombatSystem _asbp_colorverse_character)) (Variables|Stone|GetColorTag))
        (Variables|Stone|SetIsRightColor true)
        (else
          (Variables|Stone|SetIsRightColor false)))
      (if (not (Utilities|Enum|Equal(Enum) (Variables|/Script/Colorverse.CombatSystem|GetCurrentPaintColor (Variables|/Script/Colorverse.ColorverseCharacter|GetCombatSystem _asbp_colorverse_character)) "Empty"))
        ;[1 1 1] Paint Color
        (if (not (Variables|Stone|GetIsDrawComplete))
          (Math|Integer|IncrementInt (Variables|Stone|GetPaintCount)
            (:%20%20
              (bind _currentcolor (CallFunction|GetCurrentOverlayColor))
              (Variables|Stone|SetTargetColor (Utilities|Struct|MakeLinearColor (Math|Float|Lerp (.r _currentcolor) _r 0.5) (Math|Float|Lerp (.g _currentcolor) _g 0.5) (Math|Float|Lerp (.b _currentcolor) _b 0.5) 1.0))
              (Variables|Stone|SetIsColorChanged true)
              (if (>= (Variables|Stone|GetPaintCount) 3)
                (Variables|Stone|SetTargetColor PaintColor)))))
        (else
          ;[1 1 1] Intialize Color
          (Variables|Stone|SetTargetColor "(R=1.000000,G=1.000000,B=1.000000,A=1.000000)")
          (Variables|Stone|SetIsDrawComplete false)
          (Variables|Stone|SetIsColorChanged true)
          (Variables|Stone|SetPaintCount 0))))))

(event EventBeginPlay
  (Utilities|FlowControl|Sequence
    (:then_0
      ;[1 1 1] Instantiate Dynamic Material (PaintingMat, BrushMat)
      (bind _returnvalue (Rendering|Material|CreateDynamicMaterialInstance "/Game/Painter/M_RT_Painting.M_RT_Painting" "PaintingMatInst" "None" :!class /Script/Engine.KismetMaterialLibrary))
      (bind _output_get (Variables|Default|SetPaintingMatInst _returnvalue))
      (Rendering|Material|SetMaterial (Variables|Default|GetStaticMesh) 0 _output_get))
    (:then_1
      (Variables|Stone|SetCurrentColor "(R=0.100000,G=0.100000,B=0.100000,A=1.000000)"))))

(event EventTick
  (params (DeltaSeconds :type Float%20%28single-precision%29))
  ;[1 1 1] Change Color
  (if (and (not (Variables|Stone|GetIsDrawComplete)) (Variables|Stone|GetIsColorChanged))
    (Variables|Stone|SetCurrentColor (Math|Color|Lerp(LinearColor) (Variables|Stone|GetCurrentColor) (Variables|Stone|GetTargetColor) (* DeltaSeconds 2.0)))
    (CallFunction|SetOverlayColor)
    (if (<= (Math|Float|Absolute(Float) (Class|KismetMathLibrary|LinearColorDistance (Variables|Stone|GetCurrentColor) (Variables|Stone|GetTargetColor))) 0.1)
      (Variables|Stone|SetIsColorChanged false)
      (if (>= (Variables|Stone|GetPaintCount) 3)
        (Variables|Stone|SetCurrentColor (Variables|Stone|GetTargetColor))
        (CallFunction|SetOverlayColor)
        (if (Variables|Stone|GetIsRightColor)
          (Variables|Stone|SetIsDrawComplete true)
          (bind _outactors (Actor|GetAllActorsOfClass "/Game/Blueprints/BP_PuzzleGolem.BP_PuzzleGolem_C"))
          (for _array_element _outactors
            (if (and (== (Variables|/Game/Blueprints/BP_PuzzleGolem.BP_PuzzleGolem_C|GetID _array_element) (Variables|Stone|GetID)) (Utilities|Enum|Equal(Enum) (Variables|/Game/Blueprints/BP_PuzzleGolem.BP_PuzzleGolem_C|GetTargetColor _array_element) (Variables|Stone|GetColorTag)))
              (Default|GoDestroyStone _array_element self))))
        (else
          (CallFunction|SetOverlayColor))))))

(event Game|Damage|EventAnyDamage
  (params (Damage :type Float%20%28single-precision%29) (DamageType :type Damage%20Type%20Object%20Reference) (InstigatedBy :type Controller%20Object%20Reference) (DamageCauser :type Actor%20Object%20Reference))
  ;[1 1 1] AnyDamage
  (Utilities|Casting|CastToBP_PuzzleGolem DamageCauser)
  (Effects|SpawnEmitteratLocation "/Game/StarterContent/Particles/P_Smoke.P_Smoke" (Transformation|GetActorLocation))
  (Utilities|FlowControl|Delay 0.1)
  (Actor|DestroyActor))

(fn ConstructionScript)

(fn GetCurrentOverlayColor
  (bind _returnvalue (Rendering|Material|GetVectorParameterValue (Variables|Default|GetPaintingMatInst) "OverlayColor" :!class /Script/Engine.MaterialInstanceDynamic))
  (bind _output_get (Variables|Stone|SetCurrentColor _returnvalue))
  (return _output_get))

(fn SetOverlayColor
  (Rendering|Material|SetVectorParameterValue (Variables|Default|GetPaintingMatInst) "OverlayColor" (Variables|Stone|GetCurrentColor) :!class /Script/Engine.MaterialInstanceDynamic))