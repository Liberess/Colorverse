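; BP_ColorverseGameMode is the game mode that starts up Colorverse's global managers when play begins.
; On BeginPlay it initializes the ColorManager, then the InventoryManager, each only if valid.
; It then creates any missing HUD and inventory widgets, sizing the inventory container to the inventory array, and hands both to the InventoryManager.
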(event EventBeginPlay
  (bind _returnvalue (Subsystems|GetColorManager))
  (bind _returnvalue_2 (Subsystems|GetInventoryManager))
  (Utilities|FlowControl|Sequence
    (:then_0
      (Utilities|IsValid _returnvalue
        (:Is%20Valid
          (Class|ColorManager|InitializeManager _returnvalue))))
    (:then_1
      (Utilities|IsValid _returnvalue_2
        (:Is%20Valid
          (Class|InventoryManager|InitializeManager _returnvalue_2)
          (Utilities|FlowControl|Sequence
            (:then_0
              (bind _returnvalue_3 (Class|InventoryManager|GetHUDWidget _returnvalue_2))
              (Utilities|IsValid _returnvalue_3
                (:Is%20Not%20Valid
                  (bind _returnvalue_4 (UserInterface|CreateWidget "/Game/UI/BP_HUD.BP_HUD_C"))
                  (Class|HUDWidget|InitializedHUD _returnvalue_4)
                  (Variables|/Script/Colorverse.InventoryManager|SetHUDWidget _returnvalue_2 _returnvalue_4))))
            (:then_1
              (Variables|/Script/Colorverse.InventoryManager|GetInventoryWidget _returnvalue_2
                (:then)
                (:else
                  (bind _returnvalue_5 (UserInterface|CreateWidget "/Game/UI/BP_InventoryWidget.BP_InventoryWidget_C"))
                  (Class|ContainerWidget|CreateContainer _returnvalue_5 (Utilities|Array|Length (Variables|/Script/Colorverse.InventoryManager|GetInventoryArray _returnvalue_2)))
                  (Variables|/Script/Colorverse.InventoryManager|SetInventoryWidget _returnvalue_2 _returnvalue_5))))))))))

(fn ConstructionScript)