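; BP_DestructiblePuzzleStone is a breakable puzzle stone that shatters and disappears when activated.
; Active tints the GeometryCollection through its OverlayColor material parameter using StoneColor and applies an upward impulse to it.
; After a short delay, a timeline drives the root component's world scale and destroys the actor when it finishes.
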(event Custom|Active
  (bind _geometrycollection (Variables|Default|GetGeometryCollection))
  (Rendering|Material|SetVectorParameterValueonMaterials _geometrycollection "OverlayColor" (Math|Conversions|ToVector(LinearColor) (Variables|Default|GetStoneColor)))
  (Physics|AddImpulse _geometrycollection "0.000000,0.000000,100.000000" "None" false)
  (Utilities|FlowControl|Delay 3.0)
  (bind _scale (Timeline|타임라인 PlayFromStart)
    (:Update
      (Transformation|SetWorldScale3D (Variables|Default|GetDefaultSceneRoot) (Math|Conversions|ToVector(Float) _scale)))
    (:Finished
      (Actor|DestroyActor))))

(fn ConstructionScript)