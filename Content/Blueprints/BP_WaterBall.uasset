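; BP_WaterBall is a projectile that flies at the player and damages Colorverse characters, expiring after a timed delay.
; The shot event locks direction toward the player's position, then Tick moves it by swept offsets without delta-time scaling.
; Sphere overlaps damage pawns or, on a custom trace channel, attempt a turnaround that changes only rotation, not travel direction.
; Blocking hits destroy it, except against BP_Deer_Blue.
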(event OnComponentBeginOverlap(Sphere)
  (params (OverlappedComponent :type Primitive%20Component%20Object%20Reference) (OtherActor :type Actor%20Object%20Reference) (OtherComp :type Primitive%20Component%20Object%20Reference) (OtherBodyIndex :type Integer) (bFromSweep :type Boolean) (SweepResult :type Hit%20Result%20Structure%20%28by%20ref%29))
  (bind _returnvalue (Collision|GetCollisionObjectType OtherComp))
  (bind _returnvalue_2 (Transformation|GetActorForwardVector))
  (if (Utilities|Enum|Equal(Enum) _returnvalue "ECC_GameTraceChannel6")
    (Transformation|SetWorldRotation (Variables|Default|GetDefaultSceneRoot) (Math|Rotator|FindLookatRotation _returnvalue_2 (* _returnvalue_2 -1.0)) false false)
    (elif (Utilities|Enum|Equal(Enum) _returnvalue "ECC_Pawn")
      (bind _ascolorverse_character (Utilities|Casting|CastToColorverseCharacter OtherActor))
      (Class|ColorverseCharacter|Attacked _ascolorverse_character (Utilities|Struct|MakeDamageMessage self 4e+01 (.impactpoint SweepResult) (.impactnormal SweepResult))))))

(event OnComponentHit(Sphere)
  (params (HitComponent :type Primitive%20Component%20Object%20Reference) (OtherActor :type Actor%20Object%20Reference) (OtherComp :type Primitive%20Component%20Object%20Reference) (NormalImpulse :type Vector :default "0, 0, 0") (Hit :type Hit%20Result%20Structure%20%28by%20ref%29))
  (Utilities|Casting|CastToBP_Deer_Blue OtherActor
    (:CastFailed
      (Actor|DestroyActor))))

(event Custom|shot
  (Variables|Default|Setmove true)
  (Variables|Default|SetDir (Math|Vector|GetUnitDirection(Vector) (Transformation|GetActorLocation) (Transformation|GetActorLocation (Game|Player|GetPlayerPawn 0)))))

(event EventTick
  (params (DeltaSeconds :type Float%20%28single-precision%29))
  (if (Variables|Default|Getmove)
    (Class|SceneComponent|AddWorldTransform (Variables|Default|GetDefaultSceneRoot) (Math|Transform|MakeTransform (* (Variables|Default|GetDir) (Variables|Default|Getspeed)) "0, 0, 0" "1.000000,1.000000,1.000000") true false)))

(event EventBeginPlay
  (Utilities|FlowControl|Delay 1e+01)
  (Actor|DestroyActor))

(fn ConstructionScript)