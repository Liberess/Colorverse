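; BP_PuzzleStone is a paintable puzzle stone that puzzle golems destroy once it has the right color.
; When painting completes, it calls GoDestroyStone on every BP_PuzzleGolem whose puzzle tag matches its own and whose target color tag matches its current color.
; Damage caused by a puzzle golem spawns a smoke effect, then destroys the stone after a brief delay.
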(event Game|Damage|EventAnyDamage
  (params (Damage :type Float%20%28single-precision%29) (DamageType :type Damage%20Type%20Object%20Reference) (InstigatedBy :type Controller%20Object%20Reference) (DamageCauser :type Actor%20Object%20Reference))
  ;[1 1 1] AnyDamage
  (Utilities|Casting|CastToBP_PuzzleGolem DamageCauser)
  (Effects|SpawnEmitteratLocation "/Game/StarterContent/Particles/P_Smoke.P_Smoke" (Transformation|GetActorLocation))
  (Utilities|FlowControl|Delay 0.1)
  (Actor|DestroyActor))

(event EventCompletePainted
  ;[1 1 1] Complete Painted Event
  (bind _outactors (Actor|GetAllActorsOfClass "/Game/Blueprints/Puzzle/BP_PuzzleGolem.BP_PuzzleGolem_C"))
  (for _array_element _outactors
    (if (and (Utilities|Enum|Equal(Enum) (Variables|/Game/Blueprints/Puzzle/BP_PuzzleGolem.BP_PuzzleGolem_C|GetPuzzleTag _array_element) (Variables|Default|GetPuzzleTag)) (Utilities|Enum|Equal(Enum) (Variables|/Game/Blueprints/Puzzle/BP_PuzzleGolem.BP_PuzzleGolem_C|GetTargetColorTag _array_element) (Variables|Default|GetCurrentColorTag)))
      (Default|GoDestroyStone _array_element self))))

(fn ConstructionScript)