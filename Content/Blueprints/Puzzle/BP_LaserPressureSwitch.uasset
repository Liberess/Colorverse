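; Puzzle pressure switch that lowers when stepped on and, for a puzzle golem, activates its linked laser and sets that golem's color on the laser and linked wall.
; Overlap changes and a reset event re-arm a Tick-driven DoOnce check while the Sanctum is locked.
; A match between golem, laser and fully painted wall increases the Sanctum's color count once; losing it decreases the count.
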(event OnComponentBeginOverlap(BoxCol)
  (params (OverlappedComponent :type Primitive%20Component%20Object%20Reference) (OtherActor :type Actor%20Object%20Reference) (OtherComp :type Primitive%20Component%20Object%20Reference) (OtherBodyIndex :type Integer) (bFromSweep :type Boolean) (SweepResult :type Hit%20Result%20Structure%20%28by%20ref%29))
  (bind _linkedlaserwall (Variables|Default|GetLinkedLaserWall))
  (if (not (Variables|Default|GetIsComplete))
    (bind _asbp_puzzle_golem (Utilities|Casting|CastToBP_PuzzleGolem OtherActor)
      (:then
        (Utilities|IsValid (Variables|Default|GetCurrentGolem)
          (:Is%20Not%20Valid
            (Variables|Default|SetCurrentGolem _asbp_puzzle_golem)
            (Utilities|FlowControl|Sequence
              (:then_0
                (CallFunction|SetLaserWall (Variables|/Game/Blueprints/Puzzle/BP_PuzzleGolem.BP_PuzzleGolem_C|GetTargetColorTag _asbp_puzzle_golem) true)
                (if (not (Variables|Default|GetIsAlreadyInteract)) :!label _label
                  (Variables|Default|SetIsAlreadyInteract true)
                  (bind _switchposition (Timeline|SwitchActivate Play)
                    (:Update
                      (Transformation|SetRelativeLocation (Variables|Default|GetSwitch) (Math|Vector|MakeVector 0.0 0.0 _switchposition) false false)))))
              (:then_1
                ;[1 1 1] Check Laser State Event
                (Utilities|FlowControl|DoOnce false) ; enters at Reset
              )))))
      (:CastFailed
        (goto _label)))))

(event OnComponentEndOverlap(BoxCol)
  (params (OverlappedComponent :type Primitive%20Component%20Object%20Reference) (OtherActor :type Actor%20Object%20Reference) (OtherComp :type Primitive%20Component%20Object%20Reference) (OtherBodyIndex :type Integer))
  (bind _linkedlaserwall (Variables|Default|GetLinkedLaserWall))
  (bind _asbp_puzzle_golem (Utilities|Casting|CastToBP_PuzzleGolem OtherActor)
    (:then
      (if (== _asbp_puzzle_golem (Variables|Default|GetCurrentGolem))
        (Variables|Default|SetCurrentGolem 0)
        (Utilities|FlowControl|Sequence
          (:then_0
            (CallFunction|SetLaserWall "Empty" false)
            (if (Variables|Default|GetIsAlreadyInteract) :!label _label
              (Variables|Default|SetIsAlreadyInteract false)
              (bind _switchposition (Timeline|SwitchActivate Reverse)
                (:Update
                  (Transformation|SetRelativeLocation (Variables|Default|GetSwitch) (Math|Vector|MakeVector 0.0 0.0 _switchposition) false false)))))
          (:then_1
            ;[1 1 1] Check Laser State Event
            (Utilities|FlowControl|DoOnce false) ; enters at Reset
          ))
        (else
          (goto _label))))
    (:CastFailed
      (goto _label))))

(event Custom|Reset%20Check%20Laser%20Event
  (bind _currentgolem (Variables|Default|GetCurrentGolem))
  (bind _linkedlaserwall (Variables|Default|GetLinkedLaserWall))
  (bind _targetcolortag (Variables|/Game/Blueprints/Puzzle/BP_PuzzleGolem.BP_PuzzleGolem_C|GetTargetColorTag _currentgolem))
  ;[1 1 1] Check Laser State Event
  (Utilities|FlowControl|DoOnce false) ; enters at Reset
)

(event EventBeginPlay
  (bind _linkedlaserwall (Variables|Default|GetLinkedLaserWall))
  (bind _linkedlaser (Variables|Default|GetLinkedLaser))
  (Utilities|FlowControl|Sequence
    (:then_0
      (Utilities|IsValid _linkedlaser
        (:Is%20Valid
          (Default|SetActiveLaser _linkedlaser false))))
    (:then_1
      (Utilities|IsValid _linkedlaserwall
        (:Is%20Valid
          (Variables|/Game/Blueprints/Puzzle/BP_LaserWall.BP_LaserWall_C|SetLinkedSwitch _linkedlaserwall self))))))

(event EventTick
  (params (DeltaSeconds :type Float%20%28single-precision%29))
  (bind _currentgolem (Variables|Default|GetCurrentGolem))
  (bind _linkedlaserwall (Variables|Default|GetLinkedLaserWall))
  (bind _sanctum (Variables|Default|GetSanctum))
  (bind _targetcolortag (Variables|/Game/Blueprints/Puzzle/BP_PuzzleGolem.BP_PuzzleGolem_C|GetTargetColorTag _currentgolem))
  ;[1 1 1] Check Laser State Event
  (Utilities|IsValid _sanctum
    (:Is%20Valid
      (if (not (Variables|/Script/Colorverse.Sanctum|GetbIsUnlock _sanctum))
        (Utilities|FlowControl|DoOnce false
          (:Completed
            (Utilities|IsValid _currentgolem
              (:Is%20Valid
                (if (and (Utilities|Enum|Equal(Enum) _targetcolortag (Variables|/Game/Blueprints/Puzzle/BP_Laser.BP_Laser_C|GetColorTag (Variables|Default|GetLinkedLaser))) (and (Utilities|Enum|Equal(Enum) _targetcolortag (Variables|/Script/Colorverse.PaintableObject|GetCurrentColorTag _linkedlaserwall)) (Variables|/Script/Colorverse.PaintableObject|GetbIsPaintedComplete _linkedlaserwall)))
                  (if (not (Variables|Default|GetIsComplete))
                    (Class|Sanctum|IncreaseColor (Variables|Default|GetSanctum))
                    (Variables|Default|SetIsComplete true))
                  (else
                    (if (Variables|Default|GetIsComplete) :!label _label
                      (Class|Sanctum|DecreaseColor (Variables|Default|GetSanctum))
                      (Variables|Default|SetIsComplete false)))))
              (:Is%20Not%20Valid
                (goto _label)))))))))

(fn ConstructionScript)

(fn SetLaserWall
  (params (ColorTag :type ECombineColors%20Enum :default "Red") (Active :type Boolean))
  (bind _linkedlaserwall (Variables|Default|GetLinkedLaserWall))
  (bind _linkedlaser (Variables|Default|GetLinkedLaser))
  (Utilities|IsValid _linkedlaserwall
    (:Is%20Valid
      (Variables|/Script/Colorverse.PaintableObject|SetTargetColorTag _linkedlaserwall ColorTag)
      (Default|SetActiveLaser _linkedlaser Active)
      (Variables|/Game/Blueprints/Puzzle/BP_Laser.BP_Laser_C|SetColorTag _linkedlaser ColorTag))))