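; Boss door puzzle actor that removes its lightless barrier once enough completions are counted.
; IncreaseCount and DecreaseCount track progress; reaching the maximum runs a timeline that drives a dynamic material parameter, then destroys the barrier component.
; A separate SetCompleteSwitch path records switches and checks their indices against activation order, marking completion and setting the count to three without starting the fade.
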(event Custom|SetCompleteSwitch
  (params (Switch :type BP%20Multiple%20Laser%20Pressure%20Switch%20Object%20Reference) (IsComplete :type Boolean))
  (bind _switchs (Variables|Default|GetSwitchs))
  ;[1 1 1] Set Complete Switch
  (if (not (Variables|Default|GetIsComplete))
    (if IsComplete
      (if (not (Utilities|Array|ContainsItem (Variables|Default|GetSwitchs) Switch))
        (Utilities|Array|Add _switchs Switch)
        (if (>= (Utilities|Array|Length _switchs) 3)
          (bind (_array_element _array_index) (Utilities|Array|ForEachLoopwithBreak (Variables|Default|GetSwitchs) :!label _label)
            (:LoopBody
              (if (== (Variables|/Game/Blueprints/Puzzle/BP_MultipleLaserPressureSwitch.BP_MultipleLaserPressureSwitch_C|GetIndex _array_element) _array_index)
                (Variables|Default|SetIsWrongOrder false)
                (else
                  (Variables|Default|SetIsWrongOrder true)
                  (goto _label Break))))
            (:Completed
              (if (not (Variables|Default|GetIsWrongOrder))
                (Variables|Default|SetIsComplete true)
                (Variables|Default|SetIsWrongOrder false)
                (Development|PrintString "BossDoor::Complete!!!" true true "(R=0.000000,G=0.660000,B=1.000000,A=1.000000)" 4.0)
                (Variables|Default|SetCompleteCount 3))))))
      (else
        (bind _returnvalue (Utilities|Array|RemoveItem (Variables|Default|GetSwitchs) Switch))
        (if _returnvalue
          (Variables|Default|SetIsWrongOrder false))))))

(event Custom|DecreaseCount
  (if (> (Variables|Default|GetCompleteCount) 0)
    (Math|Integer|DecrementInt (Variables|Default|GetCompleteCount)
      (:%20%20
        (Development|PrintString "BossDoor::Decrease" true true "(R=1.000000,G=0.086219,B=0.000000,A=1.000000)")))))

(event Custom|IncreaseCount
  (if (not (Variables|Default|GetIsComplete))
    (if (< (Variables|Default|GetCompleteCount) (Variables|Default|GetMaxCompleteCount))
      (Math|Integer|IncrementInt (Variables|Default|GetCompleteCount)
        (:%20%20
          (Development|PrintString "BossDoor::Increase")
          (if (>= (Variables|Default|GetCompleteCount) (Variables|Default|GetMaxCompleteCount))
            (Development|PrintString "Open Boss Door" true true "(R=0.187252,G=1.000000,B=0.000000,A=1.000000)")
            (bind _opacity (Timeline|FadeBarrier PlayFromStart)
              (:Update
                (Rendering|Material|SetScalarParameterValue (Variables|Default|GetLightlessBarrierMat) "DeltaTime" _opacity :!class /Script/Engine.MaterialInstanceDynamic))
              (:Finished
                (Components|DestroyComponent (Variables|Default|GetBlackBarrier))))))))))

(event EventBeginPlay
  ;[1 1 1] Set LightlessBarrier MI
  (bind _returnvalue (Rendering|Material|CreateDynamicMaterialInstance (Variables|Default|GetBlackBarrier) 0 "/Game/Materials/M_LightlessBarrier.M_LightlessBarrier" "LightlessBarrier" :!class /Script/Engine.PrimitiveComponent))
  (Variables|Default|SetLightlessBarrierMat _returnvalue))

(fn ConstructionScript)