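; BP_Laser is a puzzle laser that draws a beam in two segments: emitter to LaserWall, then onward in a settable color to a PictureWall or Sanctum.
; On BeginPlay, a forward multi-object trace caches both points by actor tag.
; Auto lasers start lit, while SetActiveLaser toggles the beam, spawning the second segment after a short delay.
; ChangeLaserColor respawns the colored segment, and Tick updates both segments' endpoints.
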(event Custom|ChangeLaserColor
  (params (ResetColor :type Linear%20Color%20Structure))
  ;[1 1 1] Change Laser Color Event
  (Variables|Default|SetLaserColor ResetColor)
  (if (Variables|Default|GetIsThroughLaser)
    (Utilities|IsValid (Variables|Default|GetNextLaserParticle) :!label _label
      (:Is%20Valid
        (Components|DestroyComponent (Variables|Default|GetNextLaserParticle)))
      (:Is%20Not%20Valid
        _))
    (bind _returnvalue (Effects|SpawnEmitterAttached "/Game/Effects/P_Laser.P_Laser" (Variables|Default|GetStaticMesh) "None" (Variables|Default|GetPlaneVec)))
    (bind _output_get (Variables|Default|SetNextLaserParticle _returnvalue))
    (Effects|Components|ParticleSystem|SetColorParameter _output_get "Color" (Variables|Default|GetLaserColor))
    (elif (Variables|Default|GetIsAutoLaser)
      (goto _label))))

(event Custom|SetActiveLaser
  (params (Active :type Boolean))
  (Variables|Default|SetIsThroughLaser Active)
  (Utilities|IsValid (Variables|Default|GetPreviousLaserParticle)
    (:Is%20Valid
      (Components|DestroyComponent (Variables|Default|GetPreviousLaserParticle)))
    (:Is%20Not%20Valid
      _))
  (Utilities|IsValid (Variables|Default|GetNextLaserParticle)
    (:Is%20Valid
      (Components|DestroyComponent (Variables|Default|GetNextLaserParticle)))
    (:Is%20Not%20Valid
      _))
  (if Active
    (bind _returnvalue (Effects|SpawnEmitterAttached "/Game/Effects/P_Laser.P_Laser" (Variables|Default|GetStaticMesh) "None"))
    (Variables|Default|SetPreviousLaserParticle _returnvalue)
    (Utilities|FlowControl|Delay 0.4)
    (bind _returnvalue_2 (Effects|SpawnEmitterAttached "/Game/Effects/P_Laser.P_Laser" (Variables|Default|GetStaticMesh) "None" (Variables|Default|GetPlaneVec)))
    (bind _output_get (Variables|Default|SetNextLaserParticle _returnvalue_2))
    (Effects|Components|ParticleSystem|SetColorParameter _output_get "Color" (Variables|Default|GetLaserColor))))

(event EventTick
  (params (DeltaSeconds :type Float%20%28single-precision%29))
  (bind _previouslaserparticle (Variables|Default|GetPreviousLaserParticle))
  (bind _nextlaserparticle (Variables|Default|GetNextLaserParticle))
  ;[1 1 1] Draw Beam Particle
  (Utilities|FlowControl|Sequence
    (:then_0
      (Utilities|IsValid (Variables|Default|GetPreviousLaserParticle)
        (:Is%20Valid
          (Class|ParticleSystemComponent|SetBeamSourcePoint _previouslaserparticle 0 (Transformation|GetWorldLocation (Variables|Default|GetStaticMesh)))
          (Class|ParticleSystemComponent|SetBeamEndPoint _previouslaserparticle 0 (Variables|Default|GetPlaneVec)))))
    (:then_1
      (Utilities|IsValid (Variables|Default|GetNextLaserParticle)
        (:Is%20Valid
          (Class|ParticleSystemComponent|SetBeamSourcePoint _nextlaserparticle 0 (Variables|Default|GetPlaneVec))
          (Class|ParticleSystemComponent|SetBeamEndPoint _nextlaserparticle 0 (Variables|Default|GetTargetVec))
          (Effects|Components|ParticleSystem|SetColorParameter _nextlaserparticle "Color" (Variables|Default|GetLaserColor)))))))

(event EventBeginPlay
  (bind _staticmesh (Variables|Default|GetStaticMesh))
  (bind _returnvalue (Transformation|GetWorldLocation _staticmesh))
  (Utilities|FlowControl|Sequence
    (:then_0
      ;[1 1 1] Setup Wall & Target
      (bind _outhits (Class|KismetSystemLibrary|LineTraceMultiforObjects _returnvalue (+ _returnvalue (* (Math|Vector|GetForwardVector _staticmesh) 5e+03)) (Utilities|Array|MakeArray "ObjectTypeQuery8" "ObjectTypeQuery9") true 0 "None" true "(R=1.000000,G=0.000000,B=0.000000,A=1.000000)" "(R=0.000000,G=1.000000,B=0.000000,A=1.000000)" 1e+01))
      (for _array_element _outhits
        (if (Actor|ActorHasTag (.HitActor (Collision|BreakHitResult _array_element)) "PictureWall")
          (Variables|Default|SetTargetVec (.Location (Collision|BreakHitResult _array_element)))
          (elif (Actor|ActorHasTag (.HitActor (Collision|BreakHitResult _array_element)) "LaserWall")
            (Variables|Default|SetPlaneVec (.Location (Collision|BreakHitResult _array_element)))
            (elif (Actor|ActorHasTag (.HitActor (Collision|BreakHitResult _array_element)) "Sanctum")
              (Variables|Default|SetTargetVec (.Location (Collision|BreakHitResult _array_element))))))))
    (:then_1
      ;[1 1 1] Spawn Base Beam Particle
      (if (Variables|Default|GetIsAutoLaser)
        (bind _returnvalue_2 (Effects|SpawnEmitterAttached "/Game/Effects/P_Laser.P_Laser" (Variables|Default|GetStaticMesh) "None"))
        (Variables|Default|SetPreviousLaserParticle _returnvalue_2)
        (CallFunction|ChangeLaserColor "(R=1.000000,G=1.000000,B=1.000000,A=1.000000)")))))

(fn ConstructionScript)