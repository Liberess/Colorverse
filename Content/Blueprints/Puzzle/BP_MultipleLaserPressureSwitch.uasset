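; Pressure switch for a color puzzle that toggles its linked lasers and reports completion to the level's BP_SealedStone.
; BeginPlay tints the lasers from ColorTag, turns them off and finds the stone.
; Box overlap animates the plate, toggles the lasers and resets a Tick-fed DoOnce that re-evaluates completion once.
; Completion requires an occupied switch and a linked laser wall fully painted in NeedColorTag.
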(event OnComponentBeginOverlap(BoxCol)
  (params (OverlappedComponent :type Primitive%20Component%20Object%20Reference) (OtherActor :type Actor%20Object%20Reference) (OtherComp :type Primitive%20Component%20Object%20Reference) (OtherBodyIndex :type Integer) (bFromSweep :type Boolean) (SweepResult :type Hit%20Result%20Structure%20%28by%20ref%29))
  (if (Math|Boolean|NANDBoolean (Utilities|IsValid (Variables|Default|GetCurrentActor)) (Variables|Default|GetIsAlreadyInteract))
    (Variables|Default|SetIsAlreadyInteract true)
    (Variables|Default|SetCurrentActor OtherActor)
    (CallFunction|CheckLantern)
    (CallFunction|SetLaserWall true)
    (bind _switchposition (Timeline|SwitchActivate Play)
      (:Update
        (Transformation|SetRelativeLocation (Variables|Default|GetSwitch) (Math|Vector|MakeVector 0.0 0.0 _switchposition) false false)))))

(event OnComponentEndOverlap(BoxCol)
  (params (OverlappedComponent :type Primitive%20Component%20Object%20Reference) (OtherActor :type Actor%20Object%20Reference) (OtherComp :type Primitive%20Component%20Object%20Reference) (OtherBodyIndex :type Integer))
  (if (== OtherActor (Variables|Default|GetCurrentActor))
    (Variables|Default|SetIsAlreadyInteract false)
    (Variables|Default|SetCurrentActor 0)
    (CallFunction|CheckLantern)
    (CallFunction|SetLaserWall false)
    (bind _switchposition (Timeline|SwitchActivate Reverse)
      (:Update
        (Transformation|SetRelativeLocation (Variables|Default|GetSwitch) (Math|Vector|MakeVector 0.0 0.0 _switchposition) false false)))))

(event EventBeginPlay
  (Utilities|FlowControl|Sequence
    (:then_0
      (bind _asbp_colorverse_character (Utilities|Casting|CastToBP_ColorverseCharacter (Game|GetPlayerCharacter 0)))
      (bind _returnvalue (Class|CombatSystem|GetCurrentPaintLinearColorbyEnum (Variables|/Script/Colorverse.ColorverseCharacter|GetCombatSystem _asbp_colorverse_character) (Variables|Default|GetColorTag))))
    (:then_1
      (for _array_element (Variables|Default|GetLinkedLaser)
        (bind _output_get (Variables|/Game/Blueprints/Puzzle/BP_Laser.BP_Laser_C|SetPreviousLaserColor _array_element _returnvalue))
        (Variables|/Game/Blueprints/Puzzle/BP_Laser.BP_Laser_C|SetNextLaserColor _array_element _output_get)
        (Default|SetActiveLaser _array_element false)))
    (:then_2
      (bind _returnvalue_2 (Actor|GetActorOfClass "/Game/Blueprints/Puzzle/BP_SealedStone.BP_SealedStone_C"))
      (Variables|Default|SetSealedStone _returnvalue_2))))

(event EventCheckLantern
  ;[1 1 1] Check Laser State Event
  (Utilities|FlowControl|DoOnce false) ; enters at Reset
)

(event EventTick
  (params (DeltaSeconds :type Float%20%28single-precision%29))
  ;[1 1 1] Check Laser State Event
  (Utilities|FlowControl|DoOnce false
    (:Completed
      (if (Variables|Default|GetIsAlreadyInteract)
        (bind _linkedlaserwall (Variables|Default|GetLinkedLaserWall)
          (:then
            (if (and (Utilities|Enum|Equal(Enum) (Variables|Default|GetNeedColorTag) (Variables|/Script/Colorverse.PaintableObject|GetCurrentColorTag _linkedlaserwall)) (Variables|/Script/Colorverse.PaintableObject|GetbIsPaintedComplete _linkedlaserwall))
              (bind _output_get (Variables|Default|SetIsComplete true))
              (Default|SetCompleteSwitch (Variables|Default|GetSealedStone) self _output_get)))
          (:else))
        (else
          (bind _output_get_2 (Variables|Default|SetIsComplete false))
          (bind _sealedstone (Variables|Default|GetSealedStone)
            (:then
              (Default|SetCompleteSwitch _sealedstone self _output_get_2))
            (:else)))))))

(fn ConstructionScript)

(fn SetLaserWall
  (params (Active :type Boolean))
  (for _array_element (Variables|Default|GetLinkedLaser)
    (Default|SetActiveLaser _array_element Active)))