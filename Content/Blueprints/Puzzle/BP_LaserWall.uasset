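; BP_LaserWall is a paintable puzzle wall that recolors a linked laser, extending its parent's paint logic.
; On BeginPlay it links the first BP_Laser and BP_PictureWall sharing its ID.
; Painting changes the laser to TargetColor and flags the color correct if TargetColorTag is empty.
; When painting completes with an empty CurrentColorTag, it also changes the linked picture and resets LinkedSwitch's laser check.
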(event EventCompletePainted
  (bind _linkedpicturewall (Variables|Default|GetLinkedPictureWall))
  (bind _linkedlaser (Variables|Default|GetLinkedLaser))
  (bind _linkedswitch (Variables|Default|GetLinkedSwitch))
  ;[1 1 1] Complete Painted Event
  (Utilities|IsValid _linkedlaser
    (:Is%20Valid
      (Variables|/Game/Blueprints/Puzzle/BP_Laser.BP_Laser_C|SetLaserColor _linkedlaser (Variables|Default|GetTargetColor))
      (if (Utilities|Enum|Equal(Enum) (Variables|Default|GetCurrentColorTag) "Empty")
        (Utilities|FlowControl|Sequence
          (:then_0
            (Utilities|IsValid _linkedpicturewall
              (:Is%20Valid
                (Default|ChangePicture _linkedpicturewall))))
          (:then_1
            (Utilities|IsValid _linkedswitch
              (:Is%20Valid
                (Default|ResetCheckLaserEvent _linkedswitch)
                (Development|PrintString "ggggggg" true true "(R=0.133145,G=1.000000,B=0.000000,A=1.000000)" 1e+01)))))))))

(event EventPainttoObject
  (params (_PaintColor :type Linear%20Color%20Structure) (_CurrentColorTag :type ECombineColors%20Enum :default "Red"))
  (bind _linkedlaser (Variables|Default|GetLinkedLaser))
  ;[1 1 1] Paint To Object Event
  (|CallParentFunction _PaintColor _CurrentColorTag)
  (if (Utilities|Enum|Equal(Enum) (Variables|Default|GetTargetColorTag) "Empty")
    (Variables|Default|SetbIsRightColor true))
  (Utilities|IsValid _linkedlaser
    (:Is%20Valid
      (Default|ChangeLaserColor _linkedlaser (Variables|Default|GetTargetColor)))))

(event EventBeginPlay
  (|CallParentFunction)
  (Utilities|FlowControl|Sequence
    (:then_0
      (bind _outactors (Actor|GetAllActorsOfClass "/Game/Blueprints/Puzzle/BP_Laser.BP_Laser_C"))
      (bind _array_element (Utilities|Array|ForEachLoopwithBreak _outactors :!label _label)
        (:LoopBody
          (if (== (Variables|/Game/Blueprints/Puzzle/BP_Laser.BP_Laser_C|GetID _array_element) (Variables|Default|GetID))
            (Variables|Default|SetLinkedLaser _array_element)
            (goto _label Break)))))
    (:then_1
      (bind _outactors_2 (Actor|GetAllActorsOfClass "/Game/Blueprints/Puzzle/BP_PictureWall.BP_PictureWall_C"))
      (bind _array_element_2 (Utilities|Array|ForEachLoopwithBreak _outactors_2 :!label _label_2)
        (:LoopBody
          (if (== (Variables|/Game/Blueprints/Puzzle/BP_PictureWall.BP_PictureWall_C|GetID _array_element_2) (Variables|Default|GetID))
            (Variables|Default|SetLinkedPictureWall _array_element_2)
            (goto _label_2 Break)))))))

(fn ConstructionScript)