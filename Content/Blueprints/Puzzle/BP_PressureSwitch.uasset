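; BP_PressureSwitch is a puzzle pressure plate that adds to a matching boss door's count while an actor stands on it.
; On BeginPlay it finds the BP_BossDoor sharing its PuzzleTag.
; Capsule overlaps track one occupant, adjusting the count and playing or reversing a timeline that moves the switch vertically, with a sound on press.
; Once the door completes, the switch stops responding; without a door it still animates.
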(event OnComponentBeginOverlap(CapsuleCol)
  (params (OverlappedComponent :type Primitive%20Component%20Object%20Reference) (OtherActor :type Actor%20Object%20Reference) (OtherComp :type Primitive%20Component%20Object%20Reference) (OtherBodyIndex :type Integer) (bFromSweep :type Boolean) (SweepResult :type Hit%20Result%20Structure%20%28by%20ref%29))
  (Variables|Default|GetCurrentActor
    (:then)
    (:else
      (Variables|Default|SetCurrentActor OtherActor)
      (if (not (Variables|Default|GetIsAlreadyInteract))
        (Variables|Default|SetIsAlreadyInteract true)
        (bind _bossdoor (Variables|Default|GetBossDoor)
          (:then
            (if (not (Variables|/Game/Blueprints/Puzzle/BP_BossDoor.BP_BossDoor_C|GetIsComplete _bossdoor))
              (Default|IncreaseCount _bossdoor)
              (Audio|SpawnSoundatLocation (Variables|Default|GetPressSound) (Transformation|GetActorLocation) "0, 0, 0" 1.0 1.0 0.0 0 0 :!label _label)
              (bind _switchposition (Timeline|SwitchActivate Play)
                (:Update
                  (Transformation|SetRelativeLocation (Variables|Default|GetSwitch) (Math|Vector|MakeVector 0.0 0.0 _switchposition) false false)))))
          (:else
            (goto _label)))))))

(event OnComponentEndOverlap(CapsuleCol)
  (params (OverlappedComponent :type Primitive%20Component%20Object%20Reference) (OtherActor :type Actor%20Object%20Reference) (OtherComp :type Primitive%20Component%20Object%20Reference) (OtherBodyIndex :type Integer))
  (bind _currentactor (Variables|Default|GetCurrentActor)
    (:then
      (if (== _currentactor OtherActor)
        (Variables|Default|SetCurrentActor 0)
        (if (Variables|Default|GetIsAlreadyInteract)
          (Variables|Default|SetIsAlreadyInteract false)
          (bind _bossdoor (Variables|Default|GetBossDoor)
            (:then
              (if (not (Variables|/Game/Blueprints/Puzzle/BP_BossDoor.BP_BossDoor_C|GetIsComplete _bossdoor))
                (Default|DecreaseCount _bossdoor)
                (bind _switchposition (Timeline|SwitchActivate Reverse)
                  (:Update
                    (Transformation|SetRelativeLocation (Variables|Default|GetSwitch) (Math|Vector|MakeVector 0.0 0.0 _switchposition) false false)))))
            (:else
              (Timeline|SwitchActivate Reverse))))))
    (:else)))

(event EventBeginPlay
  (bind _outactors (Actor|GetAllActorsOfClass "/Game/Blueprints/Puzzle/BP_BossDoor.BP_BossDoor_C"))
  (bind _array_element (Utilities|Array|ForEachLoopwithBreak _outactors :!label _label)
    (:LoopBody
      (if (Utilities|Enum|Equal(Enum) (Variables|/Game/Blueprints/Puzzle/BP_BossDoor.BP_BossDoor_C|GetPuzzleTag _array_element) (Variables|Default|GetPuzzleTag))
        (Variables|Default|SetBossDoor _array_element)
        (goto _label Break)))))

(fn ConstructionScript)