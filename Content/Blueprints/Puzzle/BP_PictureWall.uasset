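; BP_PictureWall is a puzzle wall actor whose displayed picture can be switched by index.
; On BeginPlay it creates a dynamic material instance from M_Rock5 on its static mesh and stores it.
; The ChangePicture event uses the index to pick from paired base and normal texture arrays and sets both as texture parameters on that instance.
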(event Custom|ChangePicture
  (params (Index :type Integer))
  (bind _mi (Variables|Default|GetMI)
    (:then
      (Rendering|Material|SetTextureParameterValue _mi "BaseTexture" (Utilities|Array|Get(acopy) (Variables|Default|GetBaseTextures) Index))
      (Rendering|Material|SetTextureParameterValue _mi "Normal" (Utilities|Array|Get(acopy) (Variables|Default|GetNormalTextures) Index)))
    (:else)))

(event EventBeginPlay
  (bind _returnvalue (Rendering|Material|CreateDynamicMaterialInstance (Variables|Default|GetStaticMesh) 0 "/Game/Meshes/Sealed_Stone/Material/M_Rocks/M_Rock5.M_Rock5" "None" :!class /Script/Engine.PrimitiveComponent))
  (Variables|Default|SetMI _returnvalue))

(fn ConstructionScript)