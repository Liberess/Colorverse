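; Sealed stone puzzle actor that gates a boss door behind three lit crystals and an ordered switch puzzle.
; Dynamic materials fade crystal emissive colors via timelines, and the third completed fade activates the stone and lights the main crystal white.
; Registered switches are checked against their indices in activation order.
; A correct order plays a sequence, fades the door barrier, hides the HUD and stops player BGM.
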(event Custom|SetCompleteSwitch
  (params (Switch :type BP%20Multiple%20Laser%20Pressure%20Switch%20Object%20Reference) (IsComplete :type Boolean))
  ;[1 1 1] Set Complete Switch
  (if (not (Variables|Default|GetIsComplete))
    (if IsComplete
      (if (not (Utilities|Array|ContainsItem (Variables|Default|GetSwitchs) Switch))
        (Utilities|Array|Add (Variables|Default|GetSwitchs) Switch)
        (CallFunction|CheckSwitchState))
      (else
        (bind _returnvalue (Utilities|Array|RemoveItem (Variables|Default|GetSwitchs) Switch))
        (if _returnvalue
          (Variables|Default|SetIsWrongOrder false))))))

(event Custom|ChangeCrystalColor
  (params (Index :type Integer) (Color :type Linear%20Color%20Structure) (IsMain :type Boolean))
  (bind _maincrystalmi (Variables|Default|GetMainCrystalMI))
  ;[1 1 1] Change Crystal Color
  (if IsMain
    (bind _time (Timeline|ChangeColor PlayFromStart)
      (:Update
        (bind _returnvalue (Rendering|Material|GetVectorParameterValue _maincrystalmi "EmissiveColor" :!class /Script/Engine.MaterialInstanceDynamic))
        (Rendering|Material|SetVectorParameterValue _maincrystalmi "EmissiveColor" (Math|Color|Lerp(LinearColor) _returnvalue Color _time) :!class /Script/Engine.MaterialInstanceDynamic)))
    (else
      (bind _time_2 (Timeline|타임라인 PlayFromStart)
        (:Update
          (Rendering|Material|SetVectorParameterValue (Utilities|Array|Get(acopy) (Variables|Default|GetCrystalMIs) Index) "EmissiveColor" (Math|Color|Lerp(LinearColor) :B Color :Alpha _time_2) :!class /Script/Engine.MaterialInstanceDynamic))
        (:Finished
          (bind _result (Math|Integer|IncrementInt (Variables|Default|GetUnlockSanctumCount))
            (:%20%20
              (if (>= _result 3)
                (Variables|Default|SetIsActive true)
                (CallFunction|CheckSwitchState)
                (CallFunction|ChangeCrystalColor 0 "(R=1.000000,G=1.000000,B=1.000000,A=1.000000)" true)))))))))

(event EventBeginPlay
  ;[1 1 1] BeginPlay :: Set MI
  (Utilities|Array|Clear (Variables|Default|GetCrystalMIs))
  (for _index (range 0 2)
    (bind _returnvalue (Rendering|Material|CreateDynamicMaterialInstance (Variables|Default|GetStaticMesh) _index (Variables|Default|GetCrystalMat) "None" :!class /Script/Engine.PrimitiveComponent))
    (Utilities|Array|Add (Variables|Default|GetCrystalMIs) _returnvalue)
    (Rendering|Material|SetVectorParameterValue _returnvalue "EmissiveColor" "(R=0.000000,G=0.000000,B=0.000000,A=0.500000)" :!class /Script/Engine.MaterialInstanceDynamic))
  (bind _returnvalue_2 (Rendering|Material|CreateDynamicMaterialInstance (Variables|Default|GetStaticMesh) 4 (Variables|Default|GetCrystalMat) "None" :!class /Script/Engine.PrimitiveComponent))
  (bind _output_get (Variables|Default|SetMainCrystalMI _returnvalue_2))
  (Rendering|Material|SetVectorParameterValue _output_get "EmissiveColor" "(R=0.000000,G=0.000000,B=0.000000,A=0.500000)" :!class /Script/Engine.MaterialInstanceDynamic))

(fn ConstructionScript)

(fn CheckSwitchState
  (if (Variables|Default|GetIsActive)
    (if (>= (Utilities|Array|Length (Variables|Default|GetSwitchs)) 3)
      (bind (_array_element _array_index) (Utilities|Array|ForEachLoopwithBreak (Variables|Default|GetSwitchs) :!label _label)
        (:LoopBody
          (if (== (Variables|/Game/Blueprints/Puzzle/BP_MultipleLaserPressureSwitch.BP_MultipleLaserPressureSwitch_C|GetIndex _array_element) _array_index)
            (Variables|Default|SetIsWrongOrder false)
            (else
              (Variables|Default|SetIsWrongOrder true)
              (goto _label Break))))
        (:Completed
          (if (not (Variables|Default|GetIsWrongOrder))
            (Variables|Default|SetIsComplete true)
            (Sequencer|Player|Play (Variables|/Script/LevelSequence.LevelSequenceActor|GetSequencePlayer (Variables|Default|GetSequence)) :!class /Script/MovieScene.MovieSceneSequencePlayer)
            (Default|FadeBarrierEvent (Variables|Default|GetBossDore))
            (Class|InventoryManager|SetVisibleHUDWidget (Subsystems|GetInventoryManager) false)
            (bind _asbp_colorverse_character (Utilities|Casting|CastToBP_ColorverseCharacter (Game|GetPlayerCharacter 0)))
            (Default|StopBGM _asbp_colorverse_character))))
      (else
        (return)))))