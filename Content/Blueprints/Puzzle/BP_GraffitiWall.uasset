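; BP_GraffitiWall is a puzzle wall that advances the color of a linked Sanctum once it has been painted.
; At BeginPlay, after the parent's logic, it searches all BP_Sanctum actors and caches the first whose StatueColor, as an integer, matches the wall's ID.
; The CompletePainted event disables interaction on the wall and calls IncreaseColor on that Sanctum if one is valid.
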(event EventCompletePainted
  (bind _sanctum (Variables|Default|GetSanctum))
  (Variables|Default|SetbIsInteractable false)
  (Utilities|IsValid _sanctum
    (:Is%20Valid
      (Class|Sanctum|IncreaseColor _sanctum))))

(event EventBeginPlay
  (|CallParentFunction)
  (bind _outactors (Actor|GetAllActorsOfClass "/Game/Blueprints/BP_Sanctum.BP_Sanctum_C"))
  (bind _array_element (Utilities|Array|ForEachLoopwithBreak _outactors :!label _label)
    (:LoopBody
      (if (== (Math|Conversions|ToInteger(Byte) (Variables|/Script/Colorverse.Sanctum|GetStatueColor _array_element)) (Variables|Default|GetID))
        (Variables|Default|SetSanctum _array_element)
        (goto _label Break)))))

(fn ConstructionScript)