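; Puzzle golem AI enemy that chases and melee-attacks the player while their paint color matches its target color.
; PawnSensing sight and hearing feed FollowTarget, an AIMoveTo chase behind a DoOnce that a looping timer re-arms.
; Noise sets a stone-follow flag that suppresses sight reactions and attacks; GoDestroyStone also sets it, then strikes the stone and restores sight.
; BeginPlay tints body and eyes to the target color through a dynamic material.
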(event OnHearNoise(PawnSensing)
  (params (Instigator :type Pawn%20Object%20Reference) (Location :type Vector%20%28by%20ref%29 :default "0, 0, 0") (Volume :type Float%20%28single-precision%29))
  ;[1 1 1] Hear Noise
  (Variables|Golem|SetIsFollowStone true)
  (Variables|Golem|SetIsSeeingTarget true)
  (Class|PawnSensingComponent|SetSensingInterval (Variables|Default|GetPawnSensing) 0.0)
  (CallFunction|FollowTarget Instigator))

(event OnSeePawn(PawnSensing)
  (params (Pawn :type Pawn%20Object%20Reference))
  ;[1 1 1] Scan Target
  (if (not (Variables|Golem|GetIsFollowStone))
    (bind _asbp_colorverse_character (Utilities|Casting|CastToBP_ColorverseCharacter Pawn))
    (if (Utilities|Enum|Equal(Enum) (Variables|/Script/Colorverse.CombatSystem|GetCurrentPaintColor (Variables|/Script/Colorverse.ColorverseCharacter|GetCombatSystem _asbp_colorverse_character)) (Variables|Golem|GetTargetColor))
      (Variables|Golem|SetIsSeeingTarget true)
      (CallFunction|FollowTarget _asbp_colorverse_character)
      (else
        (Components|Movement|StopMovementImmediately (Variables|Character|GetCharacterMovement))
        (CallFunction|ResetFollowTarget)))))

(event Custom|FollowTarget
  (params (Target :type Actor%20Object%20Reference))
  ;[1 1 1] Follow Target
  (Utilities|FlowControl|DoOnce false
    (:Completed
      (Variables|Golem|SetCanAttack true)
      (if (Variables|Golem|GetIsSeeingTarget)
        (AI|AIMoveTo self "0, 0, 0" Target 5e+01 true :!label _label
          (:OnSuccess
            (if (<= (Transformation|GetDistanceTo self Target) 1e+02)
              (if (and (Variables|Golem|GetCanAttack) (not (Variables|Golem|GetIsFollowStone)))
                (Variables|Golem|SetCanAttack false)
                (bind _returnvalue (Animation|PlayAnimMontage "/Game/Animations/Golem/Golem_Hit2_Montage.Golem_Hit2_Montage" 1.0 "None"))
                (Utilities|FlowControl|Delay _returnvalue)
                (Variables|Golem|SetCanAttack true)
                (Game|Damage|ApplyDamage Target 1e+01 0 0))
              (else
                (goto _label)))))))))

(event Custom|GoDestroyStone
  (params (Stone :type Actor%20Object%20Reference))
  ;[1 1 1] Go Destroy Stone
  (Variables|Golem|SetIsFollowStone true)
  (Variables|Golem|SetIsSeeingTarget true)
  (Variables|/Script/AIModule.PawnSensingComponent|SetbSeePawns (Variables|Default|GetPawnSensing) false)
  (AI|AIMoveTo self "0, 0, 0" Stone 5e+01 true
    (:then
      (Transformation|SetActorRotation (Math|Rotator|MakeRotator 0.0 0.0 (.yaw (Math|Interpolation|RInterpTo (Transformation|GetActorRotation) (Math|Rotator|FindLookatRotation (Transformation|GetActorLocation) (Transformation|GetActorLocation Stone)) (Utilities|Time|GetWorldDeltaSeconds) 1e+01)))))
    (:OnSuccess
      (Animation|PlayAnimMontage "/Game/Animations/Golem/Golem_Hit2_Montage.Golem_Hit2_Montage" 1.0 "None")
      (Game|Damage|ApplyDamage Stone 1e+01 0 self)
      (Variables|/Script/AIModule.PawnSensingComponent|SetbSeePawns (Variables|Default|GetPawnSensing) true)
      (Variables|Golem|SetIsFollowStone false)
      (CallFunction|ResetFollowTarget))))

(event Custom|ResetFollowTarget
  ;[1 1 1] Follow Target
  (Utilities|FlowControl|DoOnce false) ; enters at Reset
)

(event EventBeginPlay
  (Utilities|FlowControl|Sequence
    (:then_0
      (Utilities|Time|SetTimerbyEvent (delegate Custom|ResetFollowTarget) 0.5 true))
    (:then_1
      (bind _returnvalue (Rendering|Material|CreateDynamicMaterialInstance "/Game/Materials/m_stoneGolem_skin1.m_stoneGolem_skin1" "GolemMatInst" "None" :!class /Script/Engine.KismetMaterialLibrary))
      (bind _output_get (Variables|Default|SetGolemMatInst _returnvalue))
      (Rendering|Material|SetMaterial (Variables|Character|GetMesh) 0 _output_get))
    (:then_2
      (bind _asbp_colorverse_character (Utilities|Casting|CastToBP_ColorverseCharacter (Game|GetPlayerCharacter 0)))
      (bind _returnvalue_2 (Class|CombatSystem|GetCurrentPaintLinearColorbyEnum (Variables|/Script/Colorverse.ColorverseCharacter|GetCombatSystem _asbp_colorverse_character) (Variables|Golem|GetTargetColor))))
    (:then_3
      (Rendering|Material|SetVectorParameterValue (Variables|Default|GetGolemMatInst) "BodyColor" _returnvalue_2 :!class /Script/Engine.MaterialInstanceDynamic)
      (Rendering|Material|SetVectorParameterValue (Variables|Default|GetGolemMatInst) "EyesColor" _returnvalue_2 :!class /Script/Engine.MaterialInstanceDynamic))))

(fn ConstructionScript)